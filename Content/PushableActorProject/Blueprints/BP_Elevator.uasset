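; BP_Elevator is a moving platform actor that travels along a set path and can spin as it moves.
; The construction script converts each MovementPoints entry from actor-local to world space and feeds the results to InterpToMovement as control points, with ElevatorTime as the duration.
; On Tick, the mesh yaws locally at RotationRate whenever that rate is positive.
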(event `self.ReceiveTick`
  (params (DeltaSeconds :type "Float (single-precision)"))
  (bind _rotationrate (`self.RotationRate`))
  (if (> _rotationrate 0.0)
    (`SceneComponent.K2_AddLocalRotation` (`self.Mesh`) (`KismetMathLibrary.MakeRotator` 0.0 0.0 (* DeltaSeconds _rotationrate)) false false)))

(fn `UserConstructionScript`
  (locals (MovementList :type "Array of InterpControlPoint Structure"))
  (set `InterpToMovementComponent.Duration` (`self.ElevatorTime`) (`self.InterpToMovement`))
  (for _array_element (`self.MovementPoints`)
    (`KismetArrayLibrary.Array_Add` (`local.MovementList`) (make `InterpControlPoint` (`KismetMathLibrary.TransformLocation` (`self.GetTransform`) _array_element) false)))
  (set `InterpToMovementComponent.ControlPoints` (`local.MovementList`) (`self.InterpToMovement`)))