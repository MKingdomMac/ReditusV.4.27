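; BP_PushPawn_Slide is a pushable pawn variant that slides after being pushed until it hits a wall.
; Once pushed past a start speed, it locks its horizontal velocity direction and keeps applying movement input along it.
; When speed passes a ratio of push speed, it forces the character's AC_PushCharacter to let go.
; The parent's wall check ends the slide, and the pawn cannot be pushed while sliding.
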(fn `CanBePushed`
  (returns (bPushable :type Boolean))
  ;[1 1 1] CAN BE PUSHED - Can't push while the box is sliding
  (return (and (`parent.CanBePushed`) (not (`self.bSlidingActive`)))) ; Cannot grab and push while moving
)

(fn `CheckWall`
  (params (Hit :type "HitResult Structure"))
  (returns (bHitWall :type Boolean))
  (bind _bhitwall (`parent.CheckWall` Hit))
  (if _bhitwall
    (set `self.bSlidingActive` false)
    (return true)
    (else
      (return false))))

(fn `UpdatePushActor`
  (params (Delta :type "Float (double-precision)"))
  ;[1 1 1] UPDATE PUSH ACTOR - Quick sliding implementation - On movement begin slide and continue until hitting a wall
  (`parent.UpdatePushActor` Delta)
  (if (`self.bSlidingActive`)
    (`self.AddMovementInput` (`self.SlideDirection`)) ; Move until we hit something
    (bind _pushcharacter (`self.PushCharacter`)
      (:`then`
        (if (> (`KismetMathLibrary.VSizeXYSquared` (`MovementComponent.Velocity` (`self.FloatingPawnMovement`))) (`KismetMathLibrary.Square` (* (`self.PushSpeed`) (`self.SlideReleaseRatio`))))
          (bind _returnvalue (`self.GetComponentByClass` _pushcharacter "/Game/PushableActorProject/Blueprints/BasicPush/AC_PushCharacter.AC_PushCharacter_C"))
          (`/Engine/EditorBlueprintResources/StandardMacros.IsValid` _returnvalue
            (:`Is Valid`
              (`/Game/PushableActorProject/Blueprints/BasicPush/AC_PushCharacter.TogglePush` _returnvalue false 1.0) ; Pushed in direction\nForce let go
            ))))
      (:`else`))
    (elif (and (`KismetSystemLibrary.IsValid` (`self.PushCharacter`)) (> (`KismetMathLibrary.VSizeXYSquared` (`MovementComponent.Velocity` (`self.FloatingPawnMovement`))) (`self.SlideStartSpeedSq`)))
      (bind _output_get (set `self.SlideDirection` (`KismetMathLibrary.Vector_Normal2D` (`MovementComponent.Velocity` (`self.FloatingPawnMovement`)))))
      (if (not (`KismetMathLibrary.Vector_IsZero` _output_get))
        (set `self.bSlidingActive` true)))))

(fn `UserConstructionScript`
  (`parent.UserConstructionScript`))