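; Pushable sphere pawn that visually rolls its mesh as it moves.
; A PhysWalking override runs the parent logic, then derives speed from the actual change in location, avoiding issues when hitting objects.
; It rotates the mesh around the horizontal axis perpendicular to velocity, using a fixed speed-to-angle scale.
; The construction script caches the start location and the sphere's circumference, though the roll calculation ignores the latter.
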(fn `PhysWalking`
  (params (Delta :type "Float (double-precision)"))
  (locals (LinearSpeed :type "Float (double-precision)" :default 0.0) (AngularVelocity :type "Float (double-precision)" :default 0.0))
  (`parent.PhysWalking` Delta)
  (set `local.LinearSpeed` (/ (`KismetMathLibrary.VSize` (- (`self.LocationPrevious`) (`self.K2_GetActorLocation`))) (`local.Delta`))) ; Calculating out by movement\nAvoids issues with hitting objects
  (set `local.AngularVelocity` (/ (* (`local.LinearSpeed`) 100.0) (`KismetMathLibrary.Square` 100.0)))
  (`SceneComponent.K2_AddWorldRotation` (`self.Mesh`) (`KismetMathLibrary.RotatorFromAxisAndAngle` (`KismetMathLibrary.Vector_Normal2D` (`KismetMathLibrary.Cross_VectorVector` (0.0 0.0 1.0) (`self.GetVelocity`))) (`local.AngularVelocity`)) false false)
  (set `self.LocationPrevious` (`self.K2_GetActorLocation`)))

(fn `UserConstructionScript`
  (`parent.UserConstructionScript`)
  (set `self.SphereCircumference ` (* 2.0 (`.SphereRadius` (`KismetSystemLibrary.GetComponentBounds` (`self.Mesh`))) (`KismetMathLibrary.GetPI`)))
  (set `self.LocationPrevious` (`self.K2_GetActorLocation`)))