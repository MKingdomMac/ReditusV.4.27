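; BP_PushPawnPickup is a pushable pawn variant that the player lifts and puts down.
; BeginPush and EndPush toggle the lifting flags on BP_JRPGPlayerController and switch movement mode to Flying and Falling respectively.
; Entering either mode detaches PlayerLocation, records the pickup start transform and zeroes movement speed as a hack to lock movement; Flying also snaps PlayerLocation to the pushing character.
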(event `Delay`
  (`KismetSystemLibrary.Delay` 50.0))

(fn `BeginPush`
  (params (Character :type "Character Object Reference") (`Push Side` :type "/Game/PushableActorProject/Blueprints/BasicPush/Struct_PushOptions Structure") (Trigger :type "BoxComponent Object Reference") (Pushing :type Boolean) (`player controller` :type "/Game/TurnBasedJRPGTemplate/Blueprints/Controllers/BP_JRPGPlayerController Object Reference"))
  (`parent.BeginPush` Character `Push Side` Trigger false null)
  (bind _asbp_jrpgplayer_controller (cast `/Game/TurnBasedJRPGTemplate/Blueprints/Controllers/BP_JRPGPlayerController` (`GameplayStatics.GetPlayerController` 0)))
  (set `self.JrpgController` _asbp_jrpgplayer_controller)
  (set `/Game/TurnBasedJRPGTemplate/Blueprints/Controllers/BP_JRPGPlayerController.IsLifting` true _asbp_jrpgplayer_controller)
  (set `/Game/TurnBasedJRPGTemplate/Blueprints/Controllers/BP_JRPGPlayerController.IsLiftingState` true _asbp_jrpgplayer_controller)
  (`self.SetMovementMode` "MOVE_Flying"))

(fn `EndPush`
  (`parent.EndPush`)
  (bind _asbp_jrpgplayer_controller (cast `/Game/TurnBasedJRPGTemplate/Blueprints/Controllers/BP_JRPGPlayerController` (`GameplayStatics.GetPlayerController` 0)))
  (set `/Game/TurnBasedJRPGTemplate/Blueprints/Controllers/BP_JRPGPlayerController.IsLiftingState` false _asbp_jrpgplayer_controller)
  (set `/Game/TurnBasedJRPGTemplate/Blueprints/Controllers/BP_JRPGPlayerController.IsLifting` false _asbp_jrpgplayer_controller)
  (`self.SetMovementMode` "MOVE_Falling"))

(fn `EnterFallingMode`
  (bind _floatingpawnmovement (`self.FloatingPawnMovement`))
  (`parent.EnterFallingMode`)
  (`SceneComponent.K2_DetachFromComponent` (`self.PlayerLocation`) "KeepWorld" "KeepWorld" "KeepWorld" true)
  (set `self.PickupTransformStart` (`self.GetTransform`))
  (`MovementComponent.StopMovementImmediately` _floatingpawnmovement) ; Quick hack to make sure we cannot move during the pickup action
  (set `FloatingPawnMovement.MaxSpeed` 0.0 _floatingpawnmovement))

(fn `EnterFlyingMode`
  (bind _floatingpawnmovement (`self.FloatingPawnMovement`))
  (`parent.EnterFlyingMode`)
  (`SceneComponent.K2_DetachFromComponent` (`self.PlayerLocation`) "KeepWorld" "KeepWorld" "KeepWorld" true)
  (`SceneComponent.K2_SetWorldTransform` (`self.PlayerLocation`) (`self.GetTransform` (`self.PushCharacter`)) false false)
  (set `self.PickupTransformStart` (`self.GetTransform`))
  (`MovementComponent.StopMovementImmediately` _floatingpawnmovement) ; Quick hack to make sure we cannot move during the pickup action
  (set `FloatingPawnMovement.MaxSpeed` 0.0 _floatingpawnmovement))

(fn `UserConstructionScript`
  (`parent.UserConstructionScript`))