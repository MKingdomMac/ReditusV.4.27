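; Pickup variant of the pushable pawn that the JRPG character lifts overhead, carries and sets down.
; BeginPush flags the controller as lifting and enters flying mode, where a timeline lerps the pawn above the character, with movement zeroed until it finishes.
; Release requires standing still and a clear box trace in the facing direction, whose end becomes the drop timeline's target before falling resumes.
; A rotational pickup is included, but its call is disconnected.
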(event `PlayPickupAction`
  ;[1 1 1] PICKUP MOVEMENT
  (set `/Game/TurnBasedJRPGTemplate/Blueprints/Controllers/BP_JRPGPlayerController.CanJump` false (`self.JrpgController`))
  (set `self.bInPickup` true)
  (`TimelineComponent.SetPlayRate` (`self.Timeline_Pickup`) (/ 1.0 (`self.PickupTime_0`)))
  (bind (_direction _alpha) (`Timeline|Timeline_Pickup` :!via `PlayFromStart`)
    (:`Update`
      (`self.K2_SetActorTransform` (`KismetMathLibrary.TLerp` (`self.PickupTransformStart_0`) (`.ReturnValue` (`self.GetPickupEndTransform`)) _alpha)))
    (:`Finished`
      (set `self.bInPickup` false)
      (set `FloatingPawnMovement.MaxSpeed` (`self.PushSpeed`) (`self.FloatingPawnMovement`))
      (`SceneComponent.K2_AttachToComponent` (`self.PlayerLocation`) (`self.PushCollision`) "None" "KeepWorld" "KeepWorld" "KeepWorld" true))))

(event `PlayDropAction`
  ;[1 1 1] DROP MOVEMENT
  (`self.DisableInput` (`self.JrpgController`) null)
  (`TimelineComponent.SetPlayRate` (`self.Timeline_DropMovement`) 2.0)
  (set `self.DropActionLocationStart` (`self.K2_GetActorLocation`))
  (bind (_direction _locationalpha) (`Timeline|Timeline_DropMovement` :!via `PlayFromStart`)
    (:`Update`
      (`self.K2_SetActorLocation` (`KismetMathLibrary.VLerp` (`self.DropActionLocationStart`) (`self.DropActionLocationEnd`) _locationalpha))
      (`KismetSystemLibrary.Delay` 1.0)
      (set `/Game/TurnBasedJRPGTemplate/Blueprints/Controllers/BP_JRPGPlayerController.CanJump` true (`self.JrpgController`))
      (`self.EnableInput` (`self.JrpgController`) null))
    (:`Finished`
      (`parent.EndPush`)
      (`self.SetMovementMode` "MOVE_Falling"))))

(event `PlayRotationalPickupAction`
  (bind _location (`self.GetPickupEndTransform`))
  (bind (_returnvalue_x _returnvalue_y _returnvalue_z) (`KismetMathLibrary.BreakVector` (* (`self.PushActorScale`) (`self.DefaultBoxExtents`))))
  (bind (_returnvalue_x_2 _returnvalue_y_2) (`KismetMathLibrary.BreakVector` (`KismetMathLibrary.NegateVector` (`self.ReturnPushDirections`))))
  ;[0.6623 1 0.5368] Rotational Pickup Movement
  (set `self.bInPickup` true)
  (`self.SetupDropAttachment` (`KismetMathLibrary.MakeVector` (* _returnvalue_x_2 _returnvalue_x) (* _returnvalue_y_2 _returnvalue_y) _returnvalue_z)) ; Attach mesh to target
  (`TimelineComponent.SetPlayRate` (`self.RotationalDrop`) (`self.PickupTime_0`)) ; Set play rate - Based on 1 second
  (bind (_direction _rotationalpha _locationalpha) (`Timeline|Timeline_PickupRotation` :!via `PlayFromStart`)
    (:`Update`
      (`SceneComponent.K2_SetWorldRotation` (`self.Rotator`) (`KismetMathLibrary.RLerp` (`self.DropRotationStart`) (`self.DropRotationEnd`) _rotationalpha true) false false)
      (`self.K2_SetActorLocation` (`KismetMathLibrary.VLerp` (`self.DropStart`) _location _locationalpha)) ; Simply move the push actor through the floor to\nthe new location.
      (`/Engine/EditorBlueprintResources/StandardMacros.Gate` true :!label _label
        (:`Exit`
          (`SceneComponent.K2_SetWorldLocation` (`self.Mesh`) (`KismetMathLibrary.VLerp` (`self.MeshLocationRotationStart`) _location _locationalpha) false false) ; Bit hacky to get correct movement :\\
        )))
    (:`Finished`
      (`SceneComponent.K2_AttachToComponent` (`self.Mesh`) (`self.PushCollision`) "None" "KeepWorld" "KeepWorld" "KeepWorld" true) ; Reattach box mesh to our pawn actor
      (`SceneComponent.K2_AttachToComponent` (`self.PlayerLocation`) (`self.PushCollision`) "None" "KeepWorld" "KeepWorld" "KeepWorld" true)
      (set `FloatingPawnMovement.MaxSpeed` (`self.PushSpeed`) (`self.FloatingPawnMovement`))
      (set `self.bInPickup` false)
      (goto _label :!via `Close`))
    (:`SetLocation`
      (set `self.MeshLocationRotationStart` (`SceneComponent.K2_GetComponentLocation` (`self.Mesh`)))
      (goto _label :!via `Open`))))

(fn `BeginPush`
  (params (Character :type "Character Object Reference") (`Push Side` :type "/Game/PushableActorProject/Blueprints/BasicPush/Struct_PushOptions Structure") (Trigger :type "BoxComponent Object Reference") (Pushing :type Boolean) (`player controller` :type "/Game/TurnBasedJRPGTemplate/Blueprints/Controllers/BP_JRPGPlayerController Object Reference"))
  (`parent.BeginPush` Character `Push Side` Trigger false `player controller`)
  (bind _asbp_jrpgplayer_controller (cast `/Game/TurnBasedJRPGTemplate/Blueprints/Controllers/BP_JRPGPlayerController` (`GameplayStatics.GetPlayerController` 0)))
  (set `self.JrpgController` _asbp_jrpgplayer_controller)
  (`/Game/TurnBasedJRPGTemplate/Blueprints/Controllers/BP_JRPGPlayerController.LIfting` _asbp_jrpgplayer_controller)
  (set `/Game/TurnBasedJRPGTemplate/Blueprints/Controllers/BP_JRPGPlayerController.IsLiftingState` true _asbp_jrpgplayer_controller)
  (`self.SetMovementMode` "MOVE_Flying"))

(fn `CanReleasePushActor`
  (returns (bCanRelease :type Boolean))
  (bind _returnvalue (`self.K2_GetActorLocation`))
  (bind _outhit (`KismetSystemLibrary.BoxTraceSingle` _returnvalue (+ _returnvalue (* (* (`BoxComponent.GetScaledBoxExtent` (`self.PushCollision`)) (select `byte` (`/Game/TurnBasedJRPGTemplate/Blueprints/PlayerPawns/BP_JRPGCharacterBase.E_PlayerDirection` (cast `/Game/TurnBasedJRPGTemplate/Blueprints/PlayerPawns/BP_JRPGCharacterBase` (`self.PushCharacter`) :!pure true)) :`0` (0.0 -1.0 0.0) :`1` (0.0 1.0 0.0) :`2` (-1.0 0.0 0.0) :`3` (1.0 0.0 0.0) :!type "Vector Structure")) 2.0)) (- (`BoxComponent.GetScaledBoxExtent` (`self.PushCollision`)) 10.0) (`self.K2_GetActorRotation`) "TraceTypeQuery1"))
  (bind (_bblockinghit _binitialoverlap _time _distance _location _impactpoint _normal _impactnormal _physmat _hitactor _hitcomponent _hitbonename _hititem _elementindex _faceindex _tracestart _traceend) (`GameplayStatics.BreakHitResult` _outhit))
  (set `self.DropActionLocationEnd` _traceend)
  (return (and (not _bblockinghit) (not (`self.bInPickup`)) (`KismetMathLibrary.EqualExactly_VectorVector` (`self.GetVelocity`)))))

(fn `EndPush`
  (bind _jrpgcontroller (`self.JrpgController`))
  (set `/Game/TurnBasedJRPGTemplate/Blueprints/Controllers/BP_JRPGPlayerController.IsLifting` false _jrpgcontroller)
  (set `/Game/TurnBasedJRPGTemplate/Blueprints/Controllers/BP_JRPGPlayerController.IsLiftingState` false _jrpgcontroller)
  (`self.PlayDropAction`))

(fn `EnterFlyingMode`
  (bind _returnvalue (`self.K2_GetActorRotation`))
  (bind _floatingpawnmovement (`self.FloatingPawnMovement`))
  (`parent.EnterFlyingMode`)
  (`SceneComponent.K2_DetachFromComponent` (`self.PlayerLocation`) "KeepWorld" "KeepWorld" "KeepWorld" true)
  (`SceneComponent.K2_SetWorldTransform` (`self.PlayerLocation`) (`self.GetTransform` (`self.PushCharacter`)) false false)
  (set `self.PickupTransformStart_0` (`self.GetTransform`))
  (set `self.DropStart` (`self.K2_GetActorLocation`))
  (set `self.DropEnd` (`self.GetPickupEndTransform`))
  (set `self.DropRotationStart` _returnvalue)
  (set `self.DropRotationEnd` (`KismetMathLibrary.ComposeRotators` _returnvalue (`KismetMathLibrary.RotatorFromAxisAndAngle` (`KismetMathLibrary.NegateVector` (`.Right` (`self.ReturnPushDirections`))) 90.0)))
  (`MovementComponent.StopMovementImmediately` _floatingpawnmovement) ; Quick hack to make sure we cannot move during the pickup action
  (set `FloatingPawnMovement.MaxSpeed` 0.0 _floatingpawnmovement)
  (`self.PlayPickupAction`))

(fn `GetPickupEndTransform`
  (returns (Location :type "Vector Structure") (ReturnValue :type "Transform Structure"))
  (bind (_pickuptransformstart_0_location _pickuptransformstart_0_rotation _pickuptransformstart_0_scale) (`KismetMathLibrary.BreakTransform` (`self.PickupTransformStart_0`)))
  (bind _returnvalue_location (`KismetMathLibrary.BreakTransform` (`self.GetTransform` (`self.PushCharacter`))))
  (bind (_boxextent_x _boxextent_y _boxextent_z) (`KismetMathLibrary.BreakVector` (`BoxComponent.BoxExtent` (`self.PushCollision`))))
  (bind _pushcharacter (`self.PushCharacter`)
    (:`then`
      (bind _returnvalue (+ _returnvalue_location (`KismetMathLibrary.MakeVector` 0.0 0.0 (+ _boxextent_z (`CapsuleComponent.GetScaledCapsuleHalfHeight` (`Character.CapsuleComponent` _pushcharacter))))))
      (return _returnvalue (`KismetMathLibrary.MakeTransform` _returnvalue _pickuptransformstart_0_rotation _pickuptransformstart_0_scale)))
    (:`else`
      (`TimelineComponent.Stop` (`self.Timeline_PickupRotation`))
      (`TimelineComponent.Stop` (`self.Timeline_Pickup`))
      (`self.SetMovementMode` "MOVE_Falling"))))

(fn `UserConstructionScript`
  (`parent.UserConstructionScript`))