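; Pushable pawn that constrains its movement to a spline path, running the conform step before the parent's push update.
; While moving, it projects velocity onto the nearest spline direction and pulls itself toward the path at a speed that increases with squared distance.
; Blocked swept moves slide the remaining motion along the hit surface.
; Optional yaw interpolation aligns the pawn with the spline direction.
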(fn `ConformToSpline`
  (params (Delta :type "Float (double-precision)"))
  (locals (StartVelocity :type "Vector Structure" :default (0.0 0.0 0.0)) (WorldSplineLocation :type "Vector Structure" :default (0.0 0.0 0.0)) (WorldSplineDirection :type "Vector Structure" :default (0.0 0.0 0.0)) (ToSplineDirection :type "Vector Structure" :default (0.0 0.0 0.0)) (ToSplineDistanceSq :type "Float (double-precision)" :default 0.0) (DesiredSplineLocation :type "Vector Structure" :default (0.0 0.0 0.0)) (StartRotation :type "Rotator Structure" :default (struct)))
  (bind _returnvalue (`self.K2_GetActorLocation`))
  (bind _returnvalue_2 (`self.K2_GetActorRotation`))
  (bind _worldsplinelocation (`local.WorldSplineLocation`))
  (bind (_returnvalue_roll _returnvalue_pitch _returnvalue_yaw) (`KismetMathLibrary.BreakRotator` (`KismetMathLibrary.MakeRotFromX` (`local.WorldSplineDirection`))))
  (bind _velocity (`MovementComponent.Velocity` (`self.FloatingPawnMovement`)))
  (set `local.StartVelocity` _velocity)
  (if (> (`KismetMathLibrary.VSizeSquared` _velocity) 0.0)
    (bind _currentsplinepath (`self.CurrentSplinePath`)
      (:`then`
        (bind _splinepath (`/Game/PushableActorProject/Blueprints/BasicPush/BP_PushSplinePath.SplinePath` _currentsplinepath)
          (:`then`
            (set `local.WorldSplineLocation` (`SplineComponent.FindLocationClosestToWorldLocation` _splinepath (`self.K2_GetActorLocation`) "World"))
            (set `local.WorldSplineDirection` (`SplineComponent.FindDirectionClosestToWorldLocation` _splinepath (`local.WorldSplineLocation`) "World"))
            (set `MovementComponent.Velocity` (`KismetMathLibrary.ProjectVectorOnToVector` (`MovementComponent.Velocity` (`self.FloatingPawnMovement`)) (`local.WorldSplineDirection`)) (`self.FloatingPawnMovement`))
            (`|ExecutionSequence`
              (:`then_0`
                (set `local.ToSplineDirection` (`KismetMathLibrary.GetDirectionUnitVector` _returnvalue _worldsplinelocation))
                (set `local.ToSplineDistanceSq` (`KismetMathLibrary.Vector_DistanceSquared` _returnvalue _worldsplinelocation))
                (bind _output_get (set `local.DesiredSplineLocation` (`KismetMathLibrary.VInterpTo_Constant` (`self.K2_GetActorLocation`) (`local.WorldSplineLocation`) (`local.Delta`) (`KismetMathLibrary.MapRangeClamped` (`local.ToSplineDistanceSq`) 0.0 10000.0 10.0 (`self.SnapToSplineSpeedMax`)))))
                (bind _sweephitresult (`self.K2_SetActorLocation` _output_get true)) ; Move to Spline
                (bind (_bblockinghit _binitialoverlap _time _distance _location _impactpoint _normal _impactnormal _physmat _hitactor _hitcomponent _hitbonename _hititem _elementindex _faceindex _tracestart _traceend) (`GameplayStatics.BreakHitResult` _sweephitresult))
                (if _bblockinghit
                  (`self.K2_SetActorLocation` (+ (`self.K2_GetActorLocation`) (* (`KismetMathLibrary.ProjectVectorOnToPlane` (- _traceend _tracestart) _normal) (- 1.0 _time))) true) ; Slide Along Surface
                ))
              (:`then_1`
                (if (`self.bRotateToSpline`)
                  (set `local.StartRotation` _returnvalue_2)
                  (`self.K2_SetActorRotation` (`KismetMathLibrary.RInterpTo` _returnvalue_2 (`KismetMathLibrary.MakeRotator` 0.0 0.0 _returnvalue_yaw) (`local.Delta`) 4.0))))))
          (:`else`)))
      (:`else`))))

(fn `UpdatePushActor`
  (params (Delta :type "Float (double-precision)"))
  (if (> Delta 0.0)
    (`self.ConformToSpline` (`local.Delta`))
    (`parent.UpdatePushActor` (`local.Delta`))))

(fn `UserConstructionScript`
  (`parent.UserConstructionScript`))