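; Liftable physical prop that registers itself with an overlapping character's AC_PushCharacter as a lift option, using a side trigger box.
; CanBeLifted gates availability on walking mode, no current lifter and no rotation drop.
; Walking updates follow moving bases via transform deltas with slide-on-hit, snap to floor and tilt toward averaged normals from a 5x5 trace grid.
; Sleep mode disables ticking once idle on a static base.
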(event `self.Box1.OnComponentBeginOverlap`
  (params (OverlappedComponent :type "PrimitiveComponent Object Reference") (OtherActor :type "Actor Object Reference") (OtherComp :type "PrimitiveComponent Object Reference") (OtherBodyIndex :type Integer) (bFromSweep :type Boolean) (SweepResult :type "HitResult Structure (by ref)"))
  (`KismetSystemLibrary.PrintString` "Hello")
  (`self.BeginTriggerOverlap` OtherActor (`self.LiftSideA`) (`self.Box`)))

(fn `BeginTriggerOverlap`
  (params (Actor :type "Actor Object Reference") (SideOptions :type "/Game/PushableActorProject/Blueprints/BasicPush/Struct_PushOptions Structure") (Trigger :type "BoxComponent Object Reference"))
  ;[0.7529 1 0.7529] Add Push actor to Player Character List
  (bind _ascharacter (cast `Character` Actor)
    (:`then`
      (message `/Game/PushableActorProject/Blueprints/BasicPush/BPI_PushActor.AddLiftActor` (`self.GetComponentByClass` _ascharacter "/Game/PushableActorProject/Blueprints/BasicPush/AC_PushCharacter.AC_PushCharacter_C") (make `/Game/PushableActorProject/Blueprints/BasicPush/Struct_LiftActor` self SideOptions Trigger)))
    (:`CastFailed`
      (`KismetSystemLibrary.PrintString` "overlap failed"))))

(fn `CanBeLifted`
  (returns (bLiftable :type Boolean))
  ;[1 1 1] CAN BE PUSHED - Called from the AC_PushCharacter to see if this actor is avaiable to be pushed - If false the prompt / UI won't be showed even if the player is in range of the action - Modify this to allow for more or less options to start pusing
  (return (and (`|EnumEquality` (`self.MovementModeCurrent`) "MOVE_Walking") (not (`KismetSystemLibrary.IsValid` (`self.LiftCharacter`))) (not (`self.bPlayingRotationDrop`)))))

(fn `CheckSleepMode`
  (params (DeltaTime :type "Float (double-precision)"))
  (bind _basecomponent (`self.BaseComponent`))
  ;[1 1 1] CHECK SLEEP MODE
  (if (not (`KismetSystemLibrary.IsValid` (`self.PushCharacter`)))
    (`/Engine/EditorBlueprintResources/StandardMacros.IsValid` _basecomponent ; 2. On a static / Non-moving\ncomponent - Keep tick if on an elevator
      (:`Is Valid`
        (switch `EComponentMobility` (`SceneComponent.Mobility` _basecomponent)
          (:`Static`
            (if (`KismetMathLibrary.Vector_IsNearlyZero` (`self.GetVelocity`))
              (bind _output_get (set `self.SleepTimeCurrent` (+ (`self.SleepTimeCurrent`) (`self.DeltaTime`)))) ; Apply delay to make sure we don't\nstart moving again
              (if (>= _output_get (`self.SleepTimeMax`))
                ;;[1 1 1] Enter sleep
                (`self.EnterSleepMode`)))))))))

(fn `ConformToFloor`
  (params (Delta :type "Float (double-precision)"))
  (locals (Normals :type "Array of Vector Structure") (X :type Integer) (Y :type Integer) (StartLocation :type "Vector Structure" :default (0.0 0.0 0.0)) (StartRotation :type "Rotator Structure" :default (struct)) (SlopeRotation :type "Rotator Structure" :default (struct)))
  (bind _returnvalue (`self.K2_GetActorLocation`))
  (bind (_startrotation_roll _startrotation_pitch _startrotation_yaw) (`KismetMathLibrary.BreakRotator` (`local.StartRotation`)))
  (bind (_bblockinghit _binitialoverlap _time _distance _location _impactpoint _normal) (`GameplayStatics.BreakHitResult` (`self.CurrentFloorHit`)))
  (bind (_origin _boxextent) (`KismetSystemLibrary.GetComponentBounds` (`self.StaticMesh`)))
  (bind (_returnvalue_roll _returnvalue_pitch) (`KismetMathLibrary.BreakRotator` (`KismetMathLibrary.MakeRotFromZX` (`KismetMathLibrary.Normal` (`KismetMathLibrary.GetVectorArrayAverage` (`local.Normals`))) (`self.GetActorForwardVector`))))
  (bind _returnvalue_2 (`KismetMathLibrary.TransformLocation` (`self.GetTransform`) (+ (* (`KismetMathLibrary.MakeVector` (`KismetMathLibrary.Conv_IntToDouble` (`local.X`)) (`KismetMathLibrary.Conv_IntToDouble` (`local.Y`))) (* (/ _boxextent 5.0) 2.0)) (`KismetMathLibrary.MakeVector` 0.0 0.0 (* (.z _boxextent) -1.0)))))
  ;[1 0.498 0.498] CONFORM TO FLOOR - Moves actor down to floor to avoid any small gaps - Moves with current base (Elevators / Moving Platforms) - Rotate to match floor (WIP)
  (if (`GameplayStatics.BreakHitResult` (`self.CurrentFloorHit`))
    (`self.UpdateBasedMovement` (`self.Delta`)) ; Add elevator movement / moving platform movement
    (`self.K2_SetActorLocation` (`KismetMathLibrary.VInterpTo_Constant` (`self.K2_GetActorLocation`) (+ _location _normal) (`self.Delta`) 200.0) true) ; Move to ground - Keep us about a unit away
    (`|ExecutionSequence`
      (:`then_0`
        (for _index (range -2 3)
          (set `local.X` _index)
          (for _index_2 (range -2 3)
            (set `local.Y` _index_2)
            (bind (_outhit _returnvalue_3) (`KismetSystemLibrary.LineTraceSingle` _returnvalue_2 (- _returnvalue_2 (0.0 0.0 50.0)) "TraceTypeQuery1")) ; Create Grid along X & Y axis\nThen transform to world space\nTrace down to find floor under push actor
            (if _returnvalue_3
              (`KismetArrayLibrary.Array_Add` (`local.Normals`) (`.Normal` (`GameplayStatics.BreakHitResult` _outhit))) ; Add to list for later use
            ))))
      (:`then_1`
        (set `local.StartLocation` _returnvalue)
        (set `local.StartRotation` (`self.K2_GetActorRotation`))
        (`self.K2_SetActorLocation` (+ _returnvalue (0.0 0.0 5.0)) true true) ; Move Push Actor up 50 units before rotating
        (set `local.SlopeRotation` (`KismetMathLibrary.MakeRotator` _returnvalue_roll _returnvalue_pitch _startrotation_yaw))
        (`self.K2_SetActorRotation` (`KismetMathLibrary.RInterpTo_Constant` (`local.StartRotation`) (`local.SlopeRotation`) (`self.Delta`) (`KismetMathLibrary.MapRangeClamped` (+ (`KismetMathLibrary.Abs` (.roll (`KismetMathLibrary.NormalizedDeltaRotator` (`local.StartRotation`) (`local.SlopeRotation`)))) (`KismetMathLibrary.Abs` (.pitch (`KismetMathLibrary.NormalizedDeltaRotator` (`local.StartRotation`) (`local.SlopeRotation`))))) 0.0 60.0 (`self.RotateToSlopeSpeedMin`) (`self.RotateToSlopeSpeedMax`)))) ; Set Rotation
        (`self.K2_SetActorLocation` (`local.StartLocation`) true true) ; Move Push Actor back down to the Floor\nafter updating its rotation
      ))))

(fn `EnterSleepMode`
  ;[1 1 1] ENTER SLEEP - Turn off tick on actor and move comp - Reset sleep cooldown - Set Sleeping Bool
  (set `self.bSleeping` true)
  (set `self.SleepTimeCurrent` 0.0)
  (`self.SetActorTickEnabled` false)
  (`ActorComponent.SetComponentTickEnabled` (`self.FloatingPawnMovement`) false))

(fn `EnterWalkingMode`
  (bind (_velocity_x _velocity_y) (`KismetMathLibrary.BreakVector` (`MovementComponent.Velocity` (`self.FloatingPawnMovement`))))
  ;[1 1 1] ON ENTER WALKING - Zero out Z velocity as we are on the ground now
  (set `MovementComponent.Velocity` (`KismetMathLibrary.MakeVector` _velocity_x _velocity_y) (`self.FloatingPawnMovement`)) ; Zero out the Z velocity
)

(fn `ExitSleepMode`
  ;[1 1 1] EXIT SLEEP
  (set `self.bSleeping` false)
  (set `self.SleepTimeCurrent` 0.0)
  (`self.SetActorTickEnabled` true)
  (`ActorComponent.SetComponentTickEnabled` (`self.FloatingPawnMovement`) true))

(fn `FloorTrace`
  (returns (Hit :type "HitResult Structure"))
  (bind _returnvalue (`self.K2_GetActorLocation`))
  ;[1 0.498 0.498] Trace for the ground below our push actor - Checking to see if we are hitting anything or not
  (bind _outhit (`KismetSystemLibrary.BoxTraceSingle` (+ _returnvalue (`KismetMathLibrary.MakeVector` 0.0 0.0 (`self.MinFloorDist`))) (- _returnvalue (`KismetMathLibrary.MakeVector` 0.0 0.0 (`self.MaxFloorDist`))) (- (`.BoxExtent` (`KismetSystemLibrary.GetComponentBounds` (`self.StaticMesh`))) (`self.MinFloorDist`)) (`self.K2_GetActorRotation`) "TraceTypeQuery1" false (`|MakeArray` (`self.PushCharacter`) :!type "Actor Object Reference"))) ; Trace one unit down with same size as Push Collision
  (bind _output_get (set `self.CurrentFloorHit` _outhit))
  (return _output_get))

(fn `PhysWalking`
  (params (Delta :type "Float (double-precision)"))
  ;[1 1 1] WALKING - Moving across the ground / being pushed
  (`self.ConformToFloor` (`self.Delta`)) ; Move Actor to floor\nOnly if we are already on the ground
  (`self.CheckSleepMode` (`local.Delta`)))

(fn `UpdateBasedMovement`
  (params (Delta :type "Float (double-precision)"))
  (locals (bRotationChanged :type Boolean :default false) (LocalBaseLocation :type "Vector Structure") (NewBaseLocation :type "Vector Structure") (DeltaLocation :type "Vector Structure") (DeltaRotation :type "Rotator Structure" :default (struct)))
  ;[1 1 1] UPDATE BASED MOVEMENT - Updated version that uses change in actor location / base component location instead of velocity - Some actors depending on setup would not have a velcoity - This mirrors EPIC's internal code for character based movement updates
  (bind _basecomponent (`self.BaseComponent`) ; Get Current Base Component\nThe component we are on top of
    (:`then`
      (set `self.BaseLocationPrevious` (`self.BaseLocationCurrent`)) ; TEMP - Need to setup functions for setting and releasing our base actor\nThis could cause issues when moving between  base components
      (set `self.BaseLocationCurrent` (`SceneComponent.K2_GetComponentLocation` _basecomponent))
      (set `self.BaseRotationPrevious` (`self.BaseRotationCurrent`))
      (set `self.BaseRotationCurrent` (`SceneComponent.K2_GetComponentRotation` _basecomponent))
      (if (or (!= (`self.BaseLocationCurrent`) (`self.BaseLocationPrevious`)) (!= (`self.BaseRotationPrevious`) (`self.BaseRotationCurrent`)))
        (set `local.DeltaRotation` (`KismetMathLibrary.NormalizedDeltaRotator` (`self.BaseRotationCurrent`) (`self.BaseRotationPrevious`))) ; Get Delta Rotation
        (bind _output_get (set `self.ForwardDirection` (`KismetMathLibrary.GreaterGreater_VectorRotator` (`self.ForwardDirection`) (`local.DeltaRotation`)))) ; Set new forward direction as we rotate
        (set `self.RightDirection` (`KismetMathLibrary.Cross_VectorVector` (0.0 0.0 1.0) _output_get)) ; Set Right Direction based on current side\nWorld based
        (set `local.LocalBaseLocation` (`KismetMathLibrary.InverseTransformLocation` (`KismetMathLibrary.MakeTransform` (`self.BaseLocationPrevious`) (`self.BaseRotationPrevious`)) (- (`self.K2_GetActorLocation`) (`KismetMathLibrary.MakeVector` 0.0 0.0 (.z (`.BoxExtent` (`KismetSystemLibrary.GetComponentBounds` (`self.StaticMesh`)))))))) ; Local Box Location on Base
        (set `local.NewBaseLocation` (+ (`KismetMathLibrary.TransformLocation` (`KismetMathLibrary.MakeTransform` (`self.BaseLocationCurrent`) (`self.BaseRotationCurrent`)) (`local.LocalBaseLocation`)) (`KismetMathLibrary.MakeVector` 0.0 0.0 (.z (`.BoxExtent` (`KismetSystemLibrary.GetComponentBounds` (`self.StaticMesh`))))))) ; Add back in height
        (set `local.DeltaLocation` (- (`local.NewBaseLocation`) (`self.K2_GetActorLocation`))) ; Get Delta Location between current and desired
        (bind _sweephitresult (`self.K2_SetActorLocationAndRotation` (+ (`self.K2_GetActorLocation`) (`local.DeltaLocation`)) (`KismetMathLibrary.ComposeRotators` (`self.K2_GetActorRotation`) (`local.DeltaRotation`)) true)) ; Add Delta Location and Rotation
        (bind (_bblockinghit _binitialoverlap _time _distance _location _impactpoint _normal _impactnormal _physmat _hitactor _hitcomponent _hitbonename _hititem _faceindex _tracestart _traceend) (`GameplayStatics.BreakHitResult` _sweephitresult))
        (if _bblockinghit
          (`self.K2_SetActorLocation` (+ (`self.K2_GetActorLocation`) _normal) true) ; Move slightly away from surface if hitting
          (`self.K2_SetActorLocation` (+ (`self.K2_GetActorLocation`) (* (`KismetMathLibrary.ProjectVectorOnToPlane` (- _traceend _tracestart) _normal) (- 1.0 _time))) true) ; Slide along surface
        )))
    (:`else`)))

(fn `UpdatePushActor`
  (params (Delta :type "Float (double-precision)"))
  ;[0.75 0.75 1] Update Push Actor - Container for the Tick Update
  (if (> Delta 0.0)
    (`|ExecutionSequence`
      (:`then_0`
        (switch `EMovementMode` (`self.MovementModeCurrent`)
          (:`MOVE_Walking`
            (`self.PhysWalking` (`self.Delta`)))
          (:`MOVE_Falling`)))
      (:`then_1`
        (set `self.InputForward` 0.0) ; Clear input after each frame
        (set `self.InputRight` 0.0)))))

(fn `UserConstructionScript`)