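; Ability item for a 2D pixel game that, when used, triggers a default area-damage explosion around its user.
; OnUsed checks the user's energy component against EnergyCost, then calls DecreaseEnergy with a zero amount and runs AbilityEffect.
; AbilityEffect sphere-traces around the user, spawns a one-shot explosion flipbook with sound, and damages hits through DamageOnTouchComponent.
; After the flipbook ends, it destroys that component and expires via a short lifespan.
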(event `self.On Used`
  (params (OwningActor :type "Actor Object Reference"))
  (bind _returnvalue (`self.GetComponentByClass` OwningActor "/Game/Pixel2D/Blueprints/Components/BP_EnergyComponent.BP_EnergyComponent_C"))
  ;[1 1 1] Checks if Player has enough energy. If he does then the ability is used and the energy is consumed
  (set `self.owningActor` OwningActor)
  (`/Engine/EditorBlueprintResources/StandardMacros.IsValid` _returnvalue
    (:`Is Valid`
      (if (< (`/Game/Pixel2D/Blueprints/Components/BP_EnergyComponent.GetCurrentEnergy` _returnvalue) (`self.energyCost`))
        (`KismetSystemLibrary.PrintString` "not enough energy")
        (else
          (`/Game/Pixel2D/Blueprints/Components/BP_EnergyComponent.DecreaseEnergy` _returnvalue 0 OwningActor)
          (`self.AbilityEffect`))))))

(event `AbilityEffect`
  (bind _owningactor (`self.owningActor`))
  (bind _returnvalue (`self.K2_GetActorLocation` _owningactor))
  ;[0.5571 0.6397 1] Default ability creates an area of damage around the user
  (bind _outhits (`KismetSystemLibrary.SphereTraceMulti` _returnvalue (`self.K2_GetActorLocation` _owningactor) 55.0 "TraceTypeQuery2" false (`|MakeArray` _owningactor)))
  (bind _returnvalue_2 (`AddComponent|NODE_AddPaperFlipbookComponent-1` :`bManualAttachment` true :`RelativeTransform` (`KismetMathLibrary.MakeTransform` _returnvalue (struct) (4.0 4.0 4.0))))
  (`PaperFlipbookComponent.SetFlipbook` _returnvalue_2 "/Game/Pixel2D/FlipBooks/Final/FB_explosion-1.FB_explosion-1")
  (`PaperFlipbookComponent.SetLooping` _returnvalue_2 false)
  (`|ExecutionSequence`
    (:`then_0`
      (`KismetSystemLibrary.Delay` (`PaperFlipbookComponent.GetFlipbookLength` _returnvalue_2))
      (`ActorComponent.K2_DestroyComponent` _returnvalue_2)
      (`self.SetLifeSpan` 0.2))
    (:`then_1`
      (`GameplayStatics.PlaySound2D` (`self.AbilitySound`) 1.0 1.0 0.0 null null)
      (for _array_element _outhits
        (bind (_bblockinghit _binitialoverlap _time _distance _location _impactpoint _normal _impactnormal _physmat _hitactor) (`GameplayStatics.BreakHitResult` _array_element))
        (`KismetSystemLibrary.PrintString` (`KismetSystemLibrary.GetDisplayName` _hitactor))
        (`/Game/Pixel2D/Blueprints/Components/BP_DamageOnTouchComponent.DealDamage` (`self.DamageOnTouchComponent`) _hitactor (0.0 0.0 0.0))))))

(fn `UserConstructionScript`
  (`parent.UserConstructionScript`))