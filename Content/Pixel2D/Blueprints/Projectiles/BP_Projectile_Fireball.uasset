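; Fireball projectile for a 2D game that turns into a brief explosion when it hits an enemy or static world geometry.
; Both hit events share one path that swaps the Paper2D flipbook to an explosion animation, rescales it and sets a short lifespan so the actor soon destroys itself.
; Movement, collision detection and damage are not defined in this graph, which only handles the impact visuals and cleanup.
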(event `self.onHitEnemy`
  (`PaperFlipbookComponent.SetFlipbook` (`self.PaperFlipbook`) "/Game/Pixel2D/FlipBooks/Final/FB_explosion-1.FB_explosion-1" :!label _label)
  (`SceneComponent.SetWorldScale3D` (`self.PaperFlipbook`) (0.45 0.45 0.45))
  (`self.SetLifeSpan` 0.2))

(event `self.onHitWorldStatic`
  (goto _label))

(fn `UserConstructionScript`
  (`parent.UserConstructionScript`))