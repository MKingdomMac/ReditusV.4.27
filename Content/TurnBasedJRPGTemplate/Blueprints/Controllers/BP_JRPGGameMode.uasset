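; JRPG game mode that picks where the player spawns in a level, based on the door ID held by the game instance.
; The ChoosePlayerStart override searches all PlayerStart actors for a tag matching that DoorID, falling back to the first one found.
; BeginPlay and Tick are empty, and a leftover SaveGame call in the event graph is never executed.
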(event `self.ReceiveBeginPlay`)

(fn `ChoosePlayerStart`
  (params (Player :type "Controller Object Reference"))
  (returns (ReturnValue :type "Actor Object Reference"))
  (bind _asbp_jrpggame_instance (cast `/Game/TurnBasedJRPGTemplate/Blueprints/Controllers/BP_JRPGGameInstance` (`GameplayStatics.GetGameInstance`)))
  (set `self.JrpgGameInstance` _asbp_jrpggame_instance)
  (bind _outactors (`GameplayStatics.GetAllActorsOfClass` "/Script/Engine.PlayerStart"))
  (for _array_element _outactors
    (bind _asplayer_start (cast `PlayerStart` _array_element))
    (if (== (`PlayerStart.PlayerStartTag` _asplayer_start) (`/Game/TurnBasedJRPGTemplate/Blueprints/Controllers/BP_JRPGGameInstance. Door ID` (`self.JrpgGameInstance`)))
      (return _asplayer_start)))
  (return (`|GetArrayItem` _outactors)))

(fn `UserConstructionScript`)