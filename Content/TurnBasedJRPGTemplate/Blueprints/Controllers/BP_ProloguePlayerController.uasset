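; Player controller for the JRPG prologue that drives the prologue character and initializes unit starting stats and party members on BeginPlay.
; Movement axes, gated by input-block and sequence flags, move the pawn and set its 2D Directionality via the MoveRight and MoveUp helpers.
; Custom events spawn an attached Niagara rain effect after a short delay and deactivate it.
; Both axis handlers still contain debug prints.
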(event `spawn rain`
  (`KismetSystemLibrary.Delay` 0.2)
  (bind _returnvalue (`NiagaraFunctionLibrary.SpawnSystemAttached` "/Game/Particles/NS_RAINING.NS_RAINING" null "None" (0.0 0.0 500.0) (struct) "KeepRelativeOffset"))
  (set `self.RAIN_0` _returnvalue))

(event `self.ReceiveBeginPlay`
  (set `self.As BP Prologue Pawn` (cast `/Game/TurnBasedJRPGTemplate/Blueprints/PlayerPawns/BP_JRPGPrologueCharacter` (`GameplayStatics.GetPlayerPawn` 0) :!pure true))
  (set `self.bShowMouseCursor` false)
  (set `self.battleController` (`self.GetBattleController`))
  (`self.SetUnitsStartingStats`)
  (`self.SetPartyMembers`))

(event `DeactivateRain`
  (`ActorComponent.Deactivate` (`self.RAIN_0`)))

(event `InputAxis|MoveRight`
  (params (AxisValue :type "Float (single-precision)"))
  (bind _as_bp_prologue_pawn (`self.As BP Prologue Pawn`))
  (`self.HasInput`
    (:`hasInput`
      (if (not (`self.IsSequence`))
        (`KismetSystemLibrary.PrintString` "Hello")
        (bind (_ismovingleft _ismovingright) (`self.MoveRight` AxisValue _as_bp_prologue_pawn))
        (`|ExecutionSequence`
          (:`then_0`
            (if _ismovingleft
              (set `/Game/TurnBasedJRPGTemplate/Blueprints/PlayerPawns/BP_JRPGPrologueCharacter.Directionality` (-1.0 0.0) _as_bp_prologue_pawn)))
          (:`then_1`
            (if _ismovingright
              (set `/Game/TurnBasedJRPGTemplate/Blueprints/PlayerPawns/BP_JRPGPrologueCharacter.Directionality` (1.0 0.0) _as_bp_prologue_pawn))))))))

(event `InputAxis|MoveDown`
  (params (AxisValue :type "Float (single-precision)"))
  (bind _as_bp_prologue_pawn (`self.As BP Prologue Pawn`))
  (`self.HasInput`
    (:`hasInput`
      (if (not (`self.IsSequence`))
        (`KismetSystemLibrary.PrintString` (`KismetStringLibrary.Conv_Vector2dToString` (stale _output_get)))
        (bind (_ispressingup_ _ispressingdown_) (`self.MoveUp` AxisValue))
        (`|ExecutionSequence`
          (:`then_0`
            (`Pawn.AddMovementInput` _as_bp_prologue_pawn (0.0 -1.0 0.0) AxisValue false))
          (:`then_1`
            (if _ispressingup_
              (bind _output_get (set `/Game/TurnBasedJRPGTemplate/Blueprints/PlayerPawns/BP_JRPGPrologueCharacter.Directionality` (0.0 1.0) _as_bp_prologue_pawn))))
          (:`then_2`
            (if _ispressingdown_
              (set `/Game/TurnBasedJRPGTemplate/Blueprints/PlayerPawns/BP_JRPGPrologueCharacter.Directionality` (0.0 -1.0) _as_bp_prologue_pawn))))))))

(fn `MoveRight`
  (params (Input :type "Float (double-precision)") (Pawn :type "/Game/TurnBasedJRPGTemplate/Blueprints/PlayerPawns/BP_JRPGPrologueCharacter Object Reference"))
  (returns (isMovingLeft :type Boolean) (isMovingRight :type Boolean) (IsNotMoving :type Boolean))
  (`/Engine/EditorBlueprintResources/StandardMacros.CompareFloat` Input
    (:`>`
      (`Pawn.AddMovementInput` Pawn (1.0 0.0 0.0) Input false)
      (return false true false))
    (:`==`
      (bind _output_get (set `self.local_isMoving` false))
      (return _output_get _output_get false))
    (:`<`
      (`Pawn.AddMovementInput` Pawn (1.0 0.0 0.0) Input false)
      (return true false false))))

(fn `MoveUp`
  (params (Input :type "Float (double-precision)"))
  (returns (`isPressingUp?` :type Boolean) (`isPressingDown?` :type Boolean))
  (locals (local_pressUp :type Boolean) (local_pressDown :type Boolean))
  (if (> Input 0.0)
    (set `local.local_pressUp` true)
    (set `local.local_pressDown` false)
    (elif (> 0.0 Input)
      (set `local.local_pressUp` false)
      (set `local.local_pressDown` true)
      (else
        (set `local.local_pressUp` false)
        (set `local.local_pressDown` false))))
  (return (`local.local_pressUp`) (`local.local_pressDown`)))

(fn `UserConstructionScript`)