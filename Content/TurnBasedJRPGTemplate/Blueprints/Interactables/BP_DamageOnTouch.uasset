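; Interactable JRPG hazard that sends a touching character back to its stored spawn location and damages every player unit.
; On overlap it halts movement, teleports the character, then subtracts a tenth of each unit's max HP, never dropping below 1.
; Updated unit data is written back to the player controller's map, with a particle on the character per damaged unit.
; The floating damage text spawn is disconnected.
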(event `self.Damage.OnComponentBeginOverlap`
  (params (OverlappedComponent :type "PrimitiveComponent Object Reference") (OtherActor :type "Actor Object Reference") (OtherComp :type "PrimitiveComponent Object Reference") (OtherBodyIndex :type Integer) (bFromSweep :type Boolean) (SweepResult :type "HitResult Structure (by ref)"))
  (bind _as_bp_jrpgcharacter_base (`self.As BP JRPGCharacter Base`))
  (bind _playerunitdataid (`/Game/TurnBasedJRPGTemplate/Blueprints/Controllers/BP_JRPGPlayerController.PlayerUnitDataID` (`self.PlayerController`)))
  (bind _spawnlocationx (`/Game/TurnBasedJRPGTemplate/Blueprints/PlayerPawns/BP_JRPGCharacterBase.SpawnLocationX` _as_bp_jrpgcharacter_base))
  (bind _asbp_jrpgcharacter_base (cast `/Game/TurnBasedJRPGTemplate/Blueprints/PlayerPawns/BP_JRPGCharacterBase` OtherActor))
  (bind _output_get (set `self.As BP JRPGCharacter Base` _asbp_jrpgcharacter_base))
  (`MovementComponent.StopMovementImmediately` (`Character.CharacterMovement` _output_get))
  (`KismetSystemLibrary.PrintString` (`KismetStringLibrary.Conv_VectorToString` _spawnlocationx))
  (`self.K2_SetActorLocation` _as_bp_jrpgcharacter_base _spawnlocationx false true)
  (bind _keys (`BlueprintMapLibrary.Map_Keys` _playerunitdataid))
  (bind _values (`BlueprintMapLibrary.Map_Values` _playerunitdataid))
  (for (_array_element _array_index) _values
    (bind _output (`|GetArrayItem` _keys _array_index))
    (bind _playerunitstats (`/Game/TurnBasedJRPGTemplate/Blueprints/Controllers/BP_JRPGFunctionLibrary.GetPlayerUnitStatsFromID` _output _array_element))
    (bind _maxhp (break `/Game/TurnBasedJRPGTemplate/Blueprints/Structs/S_UnitStats` _playerunitstats))
    (bind _returnvalue (`KismetMathLibrary.FTrunc` (* _maxhp 0.1)))
    (bind (_exp _currenthp) (break `/Game/TurnBasedJRPGTemplate/Blueprints/Structs/S_PlayerUnitData` _array_element))
    (if (!= (`KismetMathLibrary.Clamp` _returnvalue 0 (- _currenthp 1)) 0)
      (`GameplayStatics.SpawnEmitterAttached` "/Game/Particles/InfinityBladeEffects/Effects/FX_Ability/Heal/P_Heal_LongDistance_Target.P_Heal_LongDistance_Target" (`/Game/TurnBasedJRPGTemplate/Blueprints/PlayerPawns/BP_JRPGCharacterBase.Pixel2D` (`self.As BP JRPGCharacter Base`))))
    (bind _structout (setmembers `/Game/TurnBasedJRPGTemplate/Blueprints/Structs/S_PlayerUnitData` :`StructRef` _array_element :`currentHP` (`KismetMathLibrary.Clamp` (- _currenthp _returnvalue) 1 _maxhp)))
    (`BlueprintMapLibrary.Map_Add` _playerunitdataid _output _structout)))

(event `self.ReceiveBeginPlay`
  (bind _asbp_jrpgplayer_controller (cast `/Game/TurnBasedJRPGTemplate/Blueprints/Controllers/BP_JRPGPlayerController` (`GameplayStatics.GetPlayerController` 0)))
  (set `self.PlayerController` _asbp_jrpgplayer_controller))

(fn `UserConstructionScript`)