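; BP_PuzzleRestart is an interactable that asks the player to confirm a map change, apparently to restart a puzzle.
; Interacting opens a Yes/No dialogue: Yes stores the door ID and player facing direction in the game instance, then changes to the target map.
; No closes the dialogue and re-enables the interaction detector.
; A sphere overlap toggles the billboard's visibility as the player enters or leaves.
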(event `Shit`
  ;[1 1 1] Play particle effect on interaction
  (`Widget.RemoveFromParent` (`self.Dialogue`))
  (`/Game/TurnBasedJRPGTemplate/Blueprints/Interactables/BP_InteractionDetector.EnableInteraction` (`self.interactionDetector`)))

(event `self.OnInteractedHandler`
  ;[1 1 1] Play particle effect on interaction
  (bind _returnvalue (`|CreateWidget` "/Game/TurnBasedJRPGTemplate/Blueprints/UI/Dialogues/BP_YesNoDialogue.BP_YesNoDialogue_C" null (`self.Dialogue Text`) "Confirm" true null))
  (set `self.Dialogue` _returnvalue)
  (`UserWidget.AddToViewport` _returnvalue 0)
  (add `/Game/TurnBasedJRPGTemplate/Blueprints/UI/Dialogues/BP_YesNoDialogue.OnYesSelected` _returnvalue (delegate `Yes`))
  (add `/Game/TurnBasedJRPGTemplate/Blueprints/UI/Dialogues/BP_YesNoDialogue.OnNoSelected` _returnvalue (delegate `Shit`)))

(event `Yes`
  ;[1 1 1] Play particle effect on interaction
  (bind _output_get (set `self.CharacterBase` (`/Game/TurnBasedJRPGTemplate/Blueprints/Controllers/BP_JRPGPlayerController.exploreCharacter` (`/Game/TurnBasedJRPGTemplate/Blueprints/Interactables/BP_InteractionDetector.jRPGPlayerController` (`self.interactionDetector`)))))
  (bind _asbp_jrpggame_instance (cast `/Game/TurnBasedJRPGTemplate/Blueprints/Controllers/BP_JRPGGameInstance` (`GameplayStatics.GetGameInstance`)))
  (set `self.OurGameInstance` _asbp_jrpggame_instance)
  (set `/Game/TurnBasedJRPGTemplate/Blueprints/Controllers/BP_JRPGGameInstance. Door ID` (`self.door ID`) (`self.OurGameInstance`))
  (set `/Game/TurnBasedJRPGTemplate/Blueprints/Controllers/BP_JRPGGameInstance.E_PlayerDirection` (`/Game/TurnBasedJRPGTemplate/Blueprints/PlayerPawns/BP_JRPGCharacterBase.E_PlayerDirection` _output_get) (`self.OurGameInstance`))
  (`/Game/TurnBasedJRPGTemplate/Blueprints/Controllers/BP_JRPGGameInstance.ChangeMap` _asbp_jrpggame_instance (`self.WhereTo?`)))

(event `self.Sphere.OnComponentBeginOverlap`
  (params (OverlappedComponent :type "PrimitiveComponent Object Reference") (OtherActor :type "Actor Object Reference") (OtherComp :type "PrimitiveComponent Object Reference") (OtherBodyIndex :type Integer) (bFromSweep :type Boolean) (SweepResult :type "HitResult Structure (by ref)"))
  (bind _billboard (`self.Billboard`))
  (if (== OtherActor (`GameplayStatics.GetPlayerCharacter` 0))
    (`/Engine/EditorBlueprintResources/StandardMacros.IsValid` _billboard
      (:`Is Valid`
        (`SceneComponent.ToggleVisibility` _billboard false)))))

(event `self.Sphere.OnComponentEndOverlap`
  (params (OverlappedComponent :type "PrimitiveComponent Object Reference") (OtherActor :type "Actor Object Reference") (OtherComp :type "PrimitiveComponent Object Reference") (OtherBodyIndex :type Integer))
  (bind _billboard (`self.Billboard`))
  (if (== OtherActor (`GameplayStatics.GetPlayerCharacter` 0))
    (`/Engine/EditorBlueprintResources/StandardMacros.IsValid` _billboard
      (:`Is Valid`
        (`SceneComponent.ToggleVisibility` _billboard false)))))

(fn `UserConstructionScript`
  (`parent.UserConstructionScript`))