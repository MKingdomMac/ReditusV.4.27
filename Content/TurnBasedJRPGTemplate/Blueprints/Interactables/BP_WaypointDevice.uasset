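; Waypoint device interactable that behaves like a one-time chest, showing an obtained-items dialogue with gold.
; Open switches the game state, blocks player input and shows the dialogue widget.
; Confirming restores input and game state, refreshes interactions and destroys the actor.
; A sphere overlap toggles the billboard as the player enters or leaves; item variables and the loaded handler are unused stubs.
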(event `self.Open`
  (bind _jrpgplayercontroller (`/Game/TurnBasedJRPGTemplate/Blueprints/Interactables/BP_InteractionDetector.jRPGPlayerController` (`self.interactionDetector`)))
  ;[1 1 1] Open the chest
  (`/Game/TurnBasedJRPGTemplate/Blueprints/Controllers/BP_JRPGPlayerController.ChangeGameState` _jrpgplayercontroller "NewEnumerator2")
  (`/Game/TurnBasedJRPGTemplate/Blueprints/Controllers/BP_JRPGPlayerController.BlockPlayerInput` _jrpgplayercontroller true)
  (bind _returnvalue (`|CreateWidget` :`Class` "/Game/TurnBasedJRPGTemplate/Blueprints/UI/Dialogues/BP_ItemObtainDialogue.BP_ItemObtainDialogue_C" :`dialogueText` (`self.YouFound?`) :`dialogueTitle` "Obtained item(s)!" :`gold` (`self.gold`)))
  (`UserWidget.AddToViewport` _returnvalue 0)
  (add `/Game/TurnBasedJRPGTemplate/Blueprints/UI/Dialogues/BP_ItemObtainDialogue.OnConfirmed` _returnvalue (delegate `OnConfirmedHandler`)))

(event `OnConfirmedHandler`
  (bind _jrpgplayercontroller (`/Game/TurnBasedJRPGTemplate/Blueprints/Interactables/BP_InteractionDetector.jRPGPlayerController` (`self.interactionDetector`)))
  ;[1 1 1] Open the chest
  (`/Game/TurnBasedJRPGTemplate/Blueprints/Controllers/BP_JRPGPlayerController.BlockPlayerInput` _jrpgplayercontroller false)
  (`/Game/TurnBasedJRPGTemplate/Blueprints/Controllers/BP_JRPGPlayerController.RefreshInteractions` _jrpgplayercontroller)
  (`WidgetBlueprintLibrary.SetInputMode_GameOnly` _jrpgplayercontroller)
  (`/Game/TurnBasedJRPGTemplate/Blueprints/Controllers/BP_JRPGPlayerController.ChangeGameState` (`/Game/TurnBasedJRPGTemplate/Blueprints/Interactables/BP_InteractionDetector.jRPGPlayerController` (`self.interactionDetector`)) "NewEnumerator0")
  (`self.K2_DestroyActor`))

(event `self.OnLoadedHandler`
  (params (shouldLoadEnemyPawns :type Boolean))
  ;[1 1 1] Open the chest
)

(event `self.Sphere.OnComponentBeginOverlap`
  (params (OverlappedComponent :type "PrimitiveComponent Object Reference") (OtherActor :type "Actor Object Reference") (OtherComp :type "PrimitiveComponent Object Reference") (OtherBodyIndex :type Integer) (bFromSweep :type Boolean) (SweepResult :type "HitResult Structure (by ref)"))
  (if (== OtherActor (`GameplayStatics.GetPlayerCharacter` 0))
    (`SceneComponent.ToggleVisibility` (`self.Billboard`) false)))

(event `self.Sphere.OnComponentEndOverlap`
  (params (OverlappedComponent :type "PrimitiveComponent Object Reference") (OtherActor :type "Actor Object Reference") (OtherComp :type "PrimitiveComponent Object Reference") (OtherBodyIndex :type Integer))
  (if (== OtherActor (`GameplayStatics.GetPlayerCharacter` 0))
    (`SceneComponent.ToggleVisibility` (`self.Billboard`) false)))

(fn `UserConstructionScript`)