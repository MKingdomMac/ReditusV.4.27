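; BP_Forge is an interactable crafting forge that only works once the Q_FindRecipe quest reaches a required state.
; Interaction runs the parent handler when that state matches, otherwise it shows an info dialogue saying the player lacks the know-how.
; Crafting start and finish events toggle the particle effect and start or stop the crafting sound.
; Its overlap sphere disables player jumping while inside and toggles a billboard on entry and exit.
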(event `self.OnInteractedHandler`
  (`/Game/TurnBasedJRPGTemplate/Blueprints/Interactables/BP_InteractionDetector.EnableInteraction` (`self.interactionDetector`))
  (bind _queststatus (`/Game/TurnBasedJRPGTemplate/Blueprints/Controllers/BP_JRPGPlayerController.GetQuestStatus` (cast `/Game/TurnBasedJRPGTemplate/Blueprints/Controllers/BP_JRPGPlayerController` (`GameplayStatics.GetPlayerController` 0) :!pure true) "/Game/TurnBasedJRPGTemplate/Blueprints/Quests/SideQuests/RediitCamp/Q_FindRecipe.Q_FindRecipe_C"))
  (if (`|EnumEquality` _queststatus "NewEnumerator3")
    (`parent.OnInteractedHandler`)
    (else
      (bind _returnvalue (`|CreateWidget` "/Game/TurnBasedJRPGTemplate/Blueprints/UI/Dialogues/BP_InfoDialogue.BP_InfoDialogue_C" null "You don't know how to use this!" "" false null))
      (`UserWidget.AddToViewport` _returnvalue 0))))

(event `self.OnCraftingStarted`
  (`SceneComponent.ToggleVisibility` (`self.ParticleSystem`) false)
  (bind _returnvalue (`GameplayStatics.SpawnSound2D` (`self.Crafting Sound`) 1.0 1.0 0.0 null))
  (set `self.CraftingSoundPlayed` _returnvalue))

(event `self.CraftingFinished`
  (`SceneComponent.ToggleVisibility` (`self.ParticleSystem`) false)
  (`ActorComponent.Deactivate` (`self.CraftingSoundPlayed`)))

(event `self.Sphere.OnComponentBeginOverlap`
  (params (OverlappedComponent :type "PrimitiveComponent Object Reference") (OtherActor :type "Actor Object Reference") (OtherComp :type "PrimitiveComponent Object Reference") (OtherBodyIndex :type Integer) (bFromSweep :type Boolean) (SweepResult :type "HitResult Structure (by ref)"))
  (if (== OtherActor (`GameplayStatics.GetPlayerCharacter` 0))
    (set `/Game/TurnBasedJRPGTemplate/Blueprints/Controllers/BP_JRPGPlayerController.CanJump` false (cast `/Game/TurnBasedJRPGTemplate/Blueprints/Controllers/BP_JRPGPlayerController` (`GameplayStatics.GetPlayerController` 0) :!pure true))
    (`SceneComponent.ToggleVisibility` (`self.Billboard`) false)))

(event `self.Sphere.OnComponentEndOverlap`
  (params (OverlappedComponent :type "PrimitiveComponent Object Reference") (OtherActor :type "Actor Object Reference") (OtherComp :type "PrimitiveComponent Object Reference") (OtherBodyIndex :type Integer))
  (if (== OtherActor (`GameplayStatics.GetPlayerCharacter` 0))
    (set `/Game/TurnBasedJRPGTemplate/Blueprints/Controllers/BP_JRPGPlayerController.CanJump` true (cast `/Game/TurnBasedJRPGTemplate/Blueprints/Controllers/BP_JRPGPlayerController` (`GameplayStatics.GetPlayerController` 0) :!pure true))
    (`SceneComponent.ToggleVisibility` (`self.Billboard`) false)))

(fn `UserConstructionScript`
  (`parent.UserConstructionScript`))