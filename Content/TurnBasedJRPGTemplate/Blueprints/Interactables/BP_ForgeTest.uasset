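; BP_ForgeTest is an interactable forge for crafting, apparently a test version, that forwards interaction to its parent handler after re-enabling the interaction detector.
; Crafting start and finish events toggle the particle system and start or stop a stored 2D crafting sound.
; Player overlap with the sphere toggles a billboard on entry and exit.
; A recipe-quest check with a "don't know how to use this" dialogue is present but disconnected.
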(event `self.OnInteractedHandler`
  (`/Game/TurnBasedJRPGTemplate/Blueprints/Interactables/BP_InteractionDetector.EnableInteraction` (`self.interactionDetector`))
  (`parent.OnInteractedHandler`))

(event `self.OnCraftingStarted`
  (`SceneComponent.ToggleVisibility` (`self.ParticleSystem`) false)
  (bind _returnvalue (`GameplayStatics.SpawnSound2D` (`self.Crafting Sound`) 1.0 1.0 0.0 null))
  (set `self.CraftingSoundPlayed` _returnvalue))

(event `self.CraftingFinished`
  (`SceneComponent.ToggleVisibility` (`self.ParticleSystem`) false)
  (`ActorComponent.Deactivate` (`self.CraftingSoundPlayed`)))

(event `self.Sphere.OnComponentBeginOverlap`
  (params (OverlappedComponent :type "PrimitiveComponent Object Reference") (OtherActor :type "Actor Object Reference") (OtherComp :type "PrimitiveComponent Object Reference") (OtherBodyIndex :type Integer) (bFromSweep :type Boolean) (SweepResult :type "HitResult Structure (by ref)"))
  (if (== OtherActor (`GameplayStatics.GetPlayerCharacter` 0))
    (`SceneComponent.ToggleVisibility` (`self.Billboard`) false)))

(event `self.Sphere.OnComponentEndOverlap`
  (params (OverlappedComponent :type "PrimitiveComponent Object Reference") (OtherActor :type "Actor Object Reference") (OtherComp :type "PrimitiveComponent Object Reference") (OtherBodyIndex :type Integer))
  (if (== OtherActor (`GameplayStatics.GetPlayerCharacter` 0))
    (`SceneComponent.ToggleVisibility` (`self.Billboard`) false)))

(fn `UserConstructionScript`
  (`parent.UserConstructionScript`))