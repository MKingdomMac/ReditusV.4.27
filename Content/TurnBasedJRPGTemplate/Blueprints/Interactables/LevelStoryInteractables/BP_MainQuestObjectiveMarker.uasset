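; Main quest objective marker actor for level story interactables that removes itself once it is interacted with.
; On BeginPlay it casts its InteractionActor child actor to BP_InteractionDetector, caches it with its JRPG player controller, and binds the interacted and loaded events.
; Both handlers destroy the marker, and an empty Open event is left for child Blueprints to override.
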(event `self.ReceiveBeginPlay`
  ;[1 1 1] Bind event for interaction
  (bind _asbp_interaction_detector (cast `/Game/TurnBasedJRPGTemplate/Blueprints/Interactables/BP_InteractionDetector` (`ChildActorComponent.ChildActor` (`self.InteractionActor`))))
  (bind _output_get (set `self.interactionDetector` _asbp_interaction_detector))
  (set `self.J RPGPlayer Controller` (`/Game/TurnBasedJRPGTemplate/Blueprints/Interactables/BP_InteractionDetector.jRPGPlayerController` _output_get))
  (add `/Game/TurnBasedJRPGTemplate/Blueprints/Interactables/BP_InteractionDetector.OnInteracted` _output_get (delegate `OnInteractedHandler`))
  (add `/Game/TurnBasedJRPGTemplate/Blueprints/Interactables/BP_InteractionDetector.OnLoaded` (`self.interactionDetector`) (delegate `OnLoadedHandler`)))

(event `OnLoadedHandler`
  (params (shouldLoadEnemyPawns :type Boolean))
  ;[1 1 1] Bind event for interaction
  (`self.K2_DestroyActor`))

(event `OnInteractedHandler`
  ;[1 1 1] Bind event for interaction
  (`self.K2_DestroyActor`))

(event `Open`
  ;[1 1 1] Override in child blueprint
)

(fn `UserConstructionScript`)