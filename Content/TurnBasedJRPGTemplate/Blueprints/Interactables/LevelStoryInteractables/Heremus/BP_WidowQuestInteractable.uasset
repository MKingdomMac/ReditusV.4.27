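; Story interactable for the widow's find-evidence-of-husband quest, a lootable that shows its map icon when that quest is in a specific status shortly after BeginPlay.
; Opening it blocks player input and shows the item-obtain dialogue with its loot.
; Confirming restores input, records a story bool, shows the husband dialogue and destroys the actor, which the load handler also does.
; Player overlap with the sphere toggles the billboard's visibility.
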(event `self.ReceiveBeginPlay`
  (`parent.ReceiveBeginPlay`)
  (`KismetSystemLibrary.Delay` 0.6)
  (bind _asbp_jrpgplayer_controller (cast `/Game/TurnBasedJRPGTemplate/Blueprints/Controllers/BP_JRPGPlayerController` (`GameplayStatics.GetPlayerController` 0)))
  (bind _output_get (set `self.As BP JRPGPlayer Controller` _asbp_jrpgplayer_controller))
  (bind _queststatus (`/Game/TurnBasedJRPGTemplate/Blueprints/Controllers/BP_JRPGPlayerController.GetQuestStatus` _output_get "/Game/TurnBasedJRPGTemplate/Blueprints/Quests/ItemQuests/FindEvidenceofHusbandQuest.FindEvidenceofHusbandQuest_C"))
  (if (`|EnumEquality` _queststatus "NewEnumerator1")
    (`MapIconComponent.SetIconVisible` (`self.MapIcon`) true)))

(event `self.Open`
  ;[1 1 1] Open the chest
  (`/Game/TurnBasedJRPGTemplate/Blueprints/Controllers/BP_JRPGPlayerController.BlockPlayerInput` (`/Game/TurnBasedJRPGTemplate/Blueprints/Interactables/BP_InteractionDetector.jRPGPlayerController` (`self.interactionDetector`)) true)
  (bind _returnvalue (`|CreateWidget` "/Game/TurnBasedJRPGTemplate/Blueprints/UI/Dialogues/BP_ItemObtainDialogue.BP_ItemObtainDialogue_C" null (`self.YouFound?`) "" "None" (`self.UsableItemLoot`) (`self.MiscItemsLoot`) (`self.EquipmentLoot`) (`self.gold`) (`self.CraftItems`) (`self.KeyItemLoot`)))
  (`UserWidget.AddToViewport` _returnvalue 0)
  (add `/Game/TurnBasedJRPGTemplate/Blueprints/UI/Dialogues/BP_ItemObtainDialogue.OnConfirmed` _returnvalue (delegate `OnConfirmedHandler`)))

(event `OnConfirmedHandler`
  (bind _jrpgplayercontroller (`/Game/TurnBasedJRPGTemplate/Blueprints/Interactables/BP_InteractionDetector.jRPGPlayerController` (`self.interactionDetector`)))
  ;[1 1 1] Open the chest
  (`/Game/TurnBasedJRPGTemplate/Blueprints/Controllers/BP_JRPGPlayerController.BlockPlayerInput` _jrpgplayercontroller false)
  (`/Game/TurnBasedJRPGTemplate/Blueprints/Controllers/BP_JRPGPlayerController.RefreshInteractions` _jrpgplayercontroller)
  (`WidgetBlueprintLibrary.SetInputMode_GameOnly` _jrpgplayercontroller)
  (`BlueprintMapLibrary.Map_Add` (`/Game/TurnBasedJRPGTemplate/Blueprints/Controllers/BP_JRPGPlayerController.StoryBasedBools` (`self.As BP JRPGPlayer Controller`)) "NewEnumerator21" true)
  (bind _returnvalue (`|CreateWidget` "/DialoguePlugin/UI/DemoDialogueWidget.DemoDialogueWidget_C" null "/Game/DialogueSystem/CodeSpartanDialogues/Heremus/FindMyHusband.FindMyHusband" false false null null))
  (`UserWidget.AddToViewport` _returnvalue 0)
  (`self.K2_DestroyActor`))

(event `self.OnLoadedHandler`
  (params (shouldLoadEnemyPawns :type Boolean))
  ;[1 1 1] Open the chest
  (`self.K2_DestroyActor`))

(event `self.Sphere.OnComponentBeginOverlap`
  (params (OverlappedComponent :type "PrimitiveComponent Object Reference") (OtherActor :type "Actor Object Reference") (OtherComp :type "PrimitiveComponent Object Reference") (OtherBodyIndex :type Integer) (bFromSweep :type Boolean) (SweepResult :type "HitResult Structure (by ref)"))
  (if (== OtherActor (`GameplayStatics.GetPlayerCharacter` 0))
    (`SceneComponent.ToggleVisibility` (`self.Billboard`) false)))

(event `self.Sphere.OnComponentEndOverlap`
  (params (OverlappedComponent :type "PrimitiveComponent Object Reference") (OtherActor :type "Actor Object Reference") (OtherComp :type "PrimitiveComponent Object Reference") (OtherBodyIndex :type Integer))
  (if (== OtherActor (`GameplayStatics.GetPlayerCharacter` 0))
    (`SceneComponent.ToggleVisibility` (`self.Billboard`) false)))

(fn `UserConstructionScript`)