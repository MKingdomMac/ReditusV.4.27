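; Quest interactable for the widow's find-evidence-of-husband quest, opened like a chest to show an item-obtained dialogue.
; Opening blocks player input and passes the configured items, equipment and gold to the dialogue widget.
; Confirming restores input and, if the quest is active, advances it, destroys the actor and marks it interacted.
; Sphere overlaps toggle a billboard, and the load handler destroys the actor.
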(event `self.Open`
  ;[1 1 1] Open the chest
  (`/Game/TurnBasedJRPGTemplate/Blueprints/Controllers/BP_JRPGPlayerController.BlockPlayerInput` (`/Game/TurnBasedJRPGTemplate/Blueprints/Interactables/BP_InteractionDetector.jRPGPlayerController` (`self.interactionDetector`)) true)
  (bind _returnvalue (`|CreateWidget` "/Game/TurnBasedJRPGTemplate/Blueprints/UI/Dialogues/BP_ItemObtainDialogue.BP_ItemObtainDialogue_C" null (`self.YouFound?`) "" null (`self.usableItems`) (`self.miscItems`) (`self.equipment`) (`self.gold`)))
  (`UserWidget.AddToViewport` _returnvalue 0)
  (add `/Game/TurnBasedJRPGTemplate/Blueprints/UI/Dialogues/BP_ItemObtainDialogue.OnConfirmed` _returnvalue (delegate `OnConfirmedHandler`)))

(event `OnConfirmedHandler`
  (bind _jrpgplayercontroller (`/Game/TurnBasedJRPGTemplate/Blueprints/Interactables/BP_InteractionDetector.jRPGPlayerController` (`self.interactionDetector`)))
  ;[1 1 1] Open the chest
  (`/Game/TurnBasedJRPGTemplate/Blueprints/Controllers/BP_JRPGPlayerController.BlockPlayerInput` _jrpgplayercontroller false)
  (`/Game/TurnBasedJRPGTemplate/Blueprints/Controllers/BP_JRPGPlayerController.RefreshInteractions` _jrpgplayercontroller)
  (`WidgetBlueprintLibrary.SetInputMode_GameOnly` _jrpgplayercontroller)
  (bind _queststatus (`/Game/TurnBasedJRPGTemplate/Blueprints/Controllers/BP_JRPGPlayerController.GetQuestStatus` _jrpgplayercontroller "/Game/TurnBasedJRPGTemplate/Blueprints/Quests/ItemQuests/FindEvidenceofHusbandQuest.FindEvidenceofHusbandQuest_C"))
  (switch `/Game/TurnBasedJRPGTemplate/Blueprints/Enums/E_QuestStatus` _queststatus
    (:`NewEnumerator1`
      (`/Game/TurnBasedJRPGTemplate/Blueprints/Controllers/BP_JRPGPlayerController.UpdateQuest` _jrpgplayercontroller "/Game/TurnBasedJRPGTemplate/Blueprints/Quests/ItemQuests/FindEvidenceofHusbandQuest.FindEvidenceofHusbandQuest_C" 1 false false)
      (`self.K2_DestroyActor`)
      (set `self.IsInteracted` true))))

(event `self.OnLoadedHandler`
  (params (shouldLoadEnemyPawns :type Boolean))
  ;[1 1 1] Open the chest
  (`self.K2_DestroyActor`))

(event `self.Sphere.OnComponentBeginOverlap`
  (params (OverlappedComponent :type "PrimitiveComponent Object Reference") (OtherActor :type "Actor Object Reference") (OtherComp :type "PrimitiveComponent Object Reference") (OtherBodyIndex :type Integer) (bFromSweep :type Boolean) (SweepResult :type "HitResult Structure (by ref)"))
  (if (`KismetMathLibrary.BooleanNAND` (== OtherActor (`GameplayStatics.GetPlayerCharacter` 0)) (`self.IsInteracted`))
    (`SceneComponent.ToggleVisibility` (`self.Billboard`) false)))

(event `self.Sphere.OnComponentEndOverlap`
  (params (OverlappedComponent :type "PrimitiveComponent Object Reference") (OtherActor :type "Actor Object Reference") (OtherComp :type "PrimitiveComponent Object Reference") (OtherBodyIndex :type Integer))
  (if (`KismetMathLibrary.BooleanNAND` (== OtherActor (`GameplayStatics.GetPlayerCharacter` 0)) (`self.IsInteracted`))
    (`SceneComponent.ToggleVisibility` (`self.Billboard`) false)))

(fn `UserConstructionScript`)