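; BP_RandomFind is an interactable pickup that gives the player configured gold, items and equipment, with no randomization in its own graphs.
; Open switches game state, blocks input and shows an item-obtained dialogue; confirming restores control and refreshes interactions.
; Confirmation and the load handler destroy the actor, or only its billboard when DontDestroy is set; that load path also blocks input.
; A sphere overlap toggles billboard visibility as the player enters or leaves.
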(event `self.Open`
  (bind _jrpgplayercontroller (`/Game/TurnBasedJRPGTemplate/Blueprints/Interactables/BP_InteractionDetector.jRPGPlayerController` (`self.interactionDetector`)))
  ;[1 1 1] Open the chest
  (`/Game/TurnBasedJRPGTemplate/Blueprints/Controllers/BP_JRPGPlayerController.ChangeGameState` _jrpgplayercontroller "NewEnumerator2")
  (`/Game/TurnBasedJRPGTemplate/Blueprints/Controllers/BP_JRPGPlayerController.BlockPlayerInput` _jrpgplayercontroller true)
  (bind _returnvalue (`|CreateWidget` "/Game/TurnBasedJRPGTemplate/Blueprints/UI/Dialogues/BP_ItemObtainDialogue.BP_ItemObtainDialogue_C" null (`self.YouFound?`) "Obtained item(s)!" "None" (`self.UsableItemLoot`) (`self.MiscItemsLoot`) (`self.EquipmentLoot`) (`self.gold`) (`self.CraftItems`) (`self.KeyItemLoot`)))
  (`UserWidget.AddToViewport` _returnvalue 0)
  (add `/Game/TurnBasedJRPGTemplate/Blueprints/UI/Dialogues/BP_ItemObtainDialogue.OnConfirmed` _returnvalue (delegate `OnConfirmedHandler`)))

(event `OnConfirmedHandler`
  (bind _jrpgplayercontroller (`/Game/TurnBasedJRPGTemplate/Blueprints/Interactables/BP_InteractionDetector.jRPGPlayerController` (`self.interactionDetector`)))
  ;[1 1 1] Open the chest
  (`/Game/TurnBasedJRPGTemplate/Blueprints/Controllers/BP_JRPGPlayerController.BlockPlayerInput` _jrpgplayercontroller false)
  (`/Game/TurnBasedJRPGTemplate/Blueprints/Controllers/BP_JRPGPlayerController.RefreshInteractions` _jrpgplayercontroller)
  (`WidgetBlueprintLibrary.SetInputMode_GameOnly` _jrpgplayercontroller)
  (`/Game/TurnBasedJRPGTemplate/Blueprints/Controllers/BP_JRPGPlayerController.ChangeGameState` (`/Game/TurnBasedJRPGTemplate/Blueprints/Interactables/BP_InteractionDetector.jRPGPlayerController` (`self.interactionDetector`)) "NewEnumerator0")
  (if (`self.DontDestroy`)
    (`ActorComponent.K2_DestroyComponent` (`self.Billboard`))
    (else
      (`self.K2_DestroyActor`))))

(event `self.OnLoadedHandler`
  (params (shouldLoadEnemyPawns :type Boolean))
  ;[1 1 1] Open the chest
  (if (`self.DontDestroy`)
    (`/Game/TurnBasedJRPGTemplate/Blueprints/Controllers/BP_JRPGPlayerController.BlockPlayerInput` (`/Game/TurnBasedJRPGTemplate/Blueprints/Interactables/BP_InteractionDetector.jRPGPlayerController` (`self.interactionDetector`)) true)
    (`ActorComponent.K2_DestroyComponent` (`self.Billboard`))
    (else
      (`self.K2_DestroyActor`))))

(event `self.Sphere.OnComponentBeginOverlap`
  (params (OverlappedComponent :type "PrimitiveComponent Object Reference") (OtherActor :type "Actor Object Reference") (OtherComp :type "PrimitiveComponent Object Reference") (OtherBodyIndex :type Integer) (bFromSweep :type Boolean) (SweepResult :type "HitResult Structure (by ref)"))
  (bind _billboard (`self.Billboard`))
  (if (and (== OtherActor (`GameplayStatics.GetPlayerCharacter` 0)) (`KismetSystemLibrary.IsValid` _billboard))
    (`SceneComponent.ToggleVisibility` _billboard false)))

(event `self.Sphere.OnComponentEndOverlap`
  (params (OverlappedComponent :type "PrimitiveComponent Object Reference") (OtherActor :type "Actor Object Reference") (OtherComp :type "PrimitiveComponent Object Reference") (OtherBodyIndex :type Integer))
  (bind _billboard (`self.Billboard`))
  (if (and (`KismetSystemLibrary.IsValid` _billboard) (== OtherActor (`GameplayStatics.GetPlayerCharacter` 0)))
    (`SceneComponent.ToggleVisibility` _billboard false)))

(fn `UserConstructionScript`)