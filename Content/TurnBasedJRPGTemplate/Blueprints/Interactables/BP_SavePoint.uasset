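; Save point interactable for the turn-based JRPG template, extending parent interaction and load handlers with visual feedback.
; Both being interacted with and being loaded run the parent logic, then briefly activate a particle system before switching it off after a delay.
; The player character entering or leaving the sphere toggles the billboard's visibility.
; No save logic appears in this Blueprint itself.
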(event `self.OnInteractedHandler`
  (bind _particlesystem (`self.ParticleSystem`))
  ;[1 1 1] Play particle effect on interaction
  (`parent.OnInteractedHandler`)
  (`ActorComponent.Activate` _particlesystem false :!label _label)
  (`KismetSystemLibrary.Delay` 3.0)
  (`ActorComponent.Deactivate` _particlesystem))

(event `self.OnLoadedHandler`
  (params (shouldLoadEnemyPawns :type Boolean))
  ;[1 1 1] Play particle effect on interaction
  (`parent.OnLoadedHandler` shouldLoadEnemyPawns)
  (goto _label))

(event `self.Sphere.OnComponentBeginOverlap`
  (params (OverlappedComponent :type "PrimitiveComponent Object Reference") (OtherActor :type "Actor Object Reference") (OtherComp :type "PrimitiveComponent Object Reference") (OtherBodyIndex :type Integer) (bFromSweep :type Boolean) (SweepResult :type "HitResult Structure (by ref)"))
  (bind _billboard (`self.Billboard`))
  (if (== OtherActor (`GameplayStatics.GetPlayerCharacter` 0))
    (`/Engine/EditorBlueprintResources/StandardMacros.IsValid` _billboard
      (:`Is Valid`
        (`SceneComponent.ToggleVisibility` _billboard false)))))

(event `self.Sphere.OnComponentEndOverlap`
  (params (OverlappedComponent :type "PrimitiveComponent Object Reference") (OtherActor :type "Actor Object Reference") (OtherComp :type "PrimitiveComponent Object Reference") (OtherBodyIndex :type Integer))
  (bind _billboard (`self.Billboard`))
  (if (== OtherActor (`GameplayStatics.GetPlayerCharacter` 0))
    (`/Engine/EditorBlueprintResources/StandardMacros.IsValid` _billboard
      (:`Is Valid`
        (`SceneComponent.ToggleVisibility` _billboard false)))))

(fn `UserConstructionScript`
  (`parent.UserConstructionScript`))