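; Timed headshot minigame for the turn-based JRPG battle, in which a shot from an aiming reticle decides whether a headshot lands on the current target enemy.
; On BeginPlay it randomly offsets the reticle child actor, binds to its bullet-shot event and starts a short timeout.
; A shot reports success according to the target's HeadShotPossible flag, while a timeout reports failure.
; Both outcomes hide the enemy's indicator and broadcast the result.
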(event `self.ReceiveBeginPlay`
  (bind (_relativelocation_x _relativelocation_y _relativelocation_z) (`KismetMathLibrary.BreakVector` (`SceneComponent.RelativeLocation` (`self.Rectile`))))
  (`SceneComponent.K2_SetRelativeLocation` (`self.Rectile`) (`KismetMathLibrary.MakeVector` (+ (`KismetMathLibrary.SelectFloat` -100.0 100.0 (`KismetMathLibrary.RandomBoolWithWeight` 0.5)) _relativelocation_x) 0.0 (+ _relativelocation_z (`KismetMathLibrary.RandomFloatInRange` 0.0 100.0))) false false)
  (add `/Game/TurnBasedJRPGTemplate/Blueprints/MiniGames/FocusShotminigame/BP_FocusShotRectile.BulletShot` (cast `/Game/TurnBasedJRPGTemplate/Blueprints/MiniGames/FocusShotminigame/BP_FocusShotRectile` (`ChildActorComponent.ChildActor` (`self.Rectile`)) :!pure true) (delegate `Shot Made`))
  (`KismetSystemLibrary.K2_SetTimerDelegate` (delegate `Time over`) 4.0))

(event `Shot Made`
  (bind _asbp_enemy_unit_base (cast `/Game/TurnBasedJRPGTemplate/Blueprints/Units/EnemyUnits/BP_EnemyUnitBase` (`/Game/TurnBasedJRPGTemplate/Blueprints/Battle/BP_BattleController.currentTargetUnit` (`self.Battle controller`)) :!pure true))
  (`/Game/TurnBasedJRPGTemplate/Blueprints/Units/EnemyUnits/BP_EnemyUnitBase.HideIndicator` _asbp_enemy_unit_base)
  (if (`/Game/TurnBasedJRPGTemplate/Blueprints/Units/EnemyUnits/BP_EnemyUnitBase.HeadShotPossible` _asbp_enemy_unit_base)
    (`self.HeadShotSuccessful` true)
    (else
      (`self.HeadShotSuccessful` false :!label _label))))

(event `Time over`
  (`/Game/TurnBasedJRPGTemplate/Blueprints/Units/EnemyUnits/BP_EnemyUnitBase.HideIndicator` (cast `/Game/TurnBasedJRPGTemplate/Blueprints/Units/EnemyUnits/BP_EnemyUnitBase` (`/Game/TurnBasedJRPGTemplate/Blueprints/Battle/BP_BattleController.currentTargetUnit` (`self.Battle controller`)) :!pure true))
  (goto _label))

(event `self.ReceiveTick`
  (params (DeltaSeconds :type "Float (single-precision)")))

(fn `UserConstructionScript`)