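; BP_FocusShotRectile is the player-controlled aiming reticle pawn for the Focus Shot minigame.
; On BeginPlay it has the JRPG player controller possess it and stores itself there as the reticle.
; Tick adds a sine-driven horizontal drift and random vertical jitter to its location, while move input steers it on the X and Z axes.
; Shoot input calls CallBulletShot through a DoOnce with no reset wired.
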(event `self.ReceiveTick`
  (params (DeltaSeconds :type "Float (single-precision)"))
  (bind (_returnvalue_x _returnvalue_y _returnvalue_z) (`KismetMathLibrary.BreakVector` (`self.K2_GetActorLocation`)))
  (bind _output_get (set `self.Sway Time ` (+ (* DeltaSeconds (`self.Sway Speed `)) (`self.Sway Time `))))
  (set `self.SwayX` (* (`KismetMathLibrary.Sin` _output_get) (`self.Sway strength `)))
  (bind _output_get_2 (set `self.SwayZ` (`KismetMathLibrary.Sin` (`KismetMathLibrary.RandomFloatInRange` -0.5 0.5))))
  (`self.K2_SetActorLocation` (`KismetMathLibrary.MakeVector` (+ (`self.SwayX`) _returnvalue_x) _returnvalue_y (+ _returnvalue_z (`self.SwayZ`)))))

(event `self.ReceiveBeginPlay`
  (bind _asbp_jrpgplayer_controller (cast `/Game/TurnBasedJRPGTemplate/Blueprints/Controllers/BP_JRPGPlayerController` (`GameplayStatics.GetPlayerController` 0) :!pure true))
  (`Controller.Possess` _asbp_jrpgplayer_controller self)
  (set `/Game/TurnBasedJRPGTemplate/Blueprints/Controllers/BP_JRPGPlayerController.Focus Shot Recticle` self _asbp_jrpgplayer_controller))

(event `EnhancedInput|/Game/TurnBasedJRPGTemplate/InputActions/IA_Move`
  (params (ActionValue :type "Vector2D Structure") (ElapsedSeconds :type "Float (single-precision)") (TriggeredSeconds :type "Float (single-precision)"))
  (bind (_x _y) (`KismetMathLibrary.BreakVector2D` ActionValue))
  (:`Triggered`
    (`self.AddMovementInput` (1.0 0.0 0.0) _x)
    (`self.AddMovementInput` (0.0 0.0 -1.0) _y)))

(event `EnhancedInput|/Game/TurnBasedJRPGTemplate/InputActions/IA_Shoot`
  (params (ActionValue :type Boolean) (ElapsedSeconds :type "Float (single-precision)") (TriggeredSeconds :type "Float (single-precision)"))
  (:`Triggered`
    (`/Engine/EditorBlueprintResources/StandardMacros.DoOnce` false
      (:`Completed`
        (`self.BulletShot`)))))

(fn `UserConstructionScript`)