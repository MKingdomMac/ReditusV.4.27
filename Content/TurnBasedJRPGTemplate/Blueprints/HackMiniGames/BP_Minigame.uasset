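; BP_Minigame is the bonus hack side-scroller minigame for the JRPG battle system, hosting Enemy and SideScrollerCharacter child actors.
; On BeginPlay it announces the hack, switches the player controller's game state, and switches again after a short timer to allow input.
; Child actor events decide the outcome: both destroy the character, block the enemy and show a result, while success also flags the battle's target unit.
; After a delay it destroys itself and calls GameOver.
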(event `self.ReceiveBeginPlay`
  ;[1 1 1] Outcome of successful or unsuccessful events!
  (bind _returnvalue (`|CreateWidget` "/Game/TurnBasedJRPGTemplate/Blueprints/UI/Dialogues/BP_InfoDialogueForBattle.BP_InfoDialogueForBattle_C" null "Bonus Hack Initiated!" "" false null 3.0))
  (`UserWidget.AddToViewport` _returnvalue 0)
  (bind _output_get (set `self.As BP JRPGPlayer Controller` (cast `/Game/TurnBasedJRPGTemplate/Blueprints/Controllers/BP_JRPGPlayerController` (`GameplayStatics.GetPlayerController` 0) :!pure true)))
  (set `/Game/TurnBasedJRPGTemplate/Blueprints/Controllers/BP_JRPGPlayerController.gameState` "NewEnumerator2" _output_get)
  (`KismetSystemLibrary.K2_SetTimerDelegate` (delegate `Can do input`) 3.0)
  (add `/Game/TurnBasedJRPGTemplate/Blueprints/HackMiniGames/Enemy.HackSuccessful` (cast `/Game/TurnBasedJRPGTemplate/Blueprints/HackMiniGames/Enemy` (`ChildActorComponent.ChildActor` (`self.Enemy`)) :!pure true) (delegate `GameOver`))
  (add `/Game/TurnBasedJRPGTemplate/Blueprints/HackMiniGames/SideScrollerCharacter.HackUnsuccessful` (cast `/Game/TurnBasedJRPGTemplate/Blueprints/HackMiniGames/SideScrollerCharacter` (`ChildActorComponent.ChildActor` (`self.SideScrollerCharacter`)) :!pure true) (delegate `HackUnsuccessful`)))

(event `HackUnsuccessful`
  ;[1 1 1] Outcome of successful or unsuccessful events!
  (`self.K2_DestroyActor` (cast `/Game/TurnBasedJRPGTemplate/Blueprints/HackMiniGames/SideScrollerCharacter` (`ChildActorComponent.ChildActor` (`self.SideScrollerCharacter`)) :!pure true))
  (set `/Game/TurnBasedJRPGTemplate/Blueprints/HackMiniGames/Enemy.Block` true (cast `/Game/TurnBasedJRPGTemplate/Blueprints/HackMiniGames/Enemy` (`ChildActorComponent.ChildActor` (`self.Enemy`)) :!pure true))
  (bind _returnvalue (`|CreateWidget` "/Game/TurnBasedJRPGTemplate/Blueprints/UI/Dialogues/BP_InfoDialogueForBattle.BP_InfoDialogueForBattle_C" null "Bonus Hack Unsuccessful!!" "" false null 3.0))
  (`UserWidget.AddToViewport` _returnvalue 0)
  (`KismetSystemLibrary.Delay` 3.0)
  (`self.K2_DestroyActor`)
  (`self.Game over`))

(event `GameOver`
  ;[1 1 1] Outcome of successful or unsuccessful events!
  (`self.K2_DestroyActor` (cast `/Game/TurnBasedJRPGTemplate/Blueprints/HackMiniGames/SideScrollerCharacter` (`ChildActorComponent.ChildActor` (`self.SideScrollerCharacter`)) :!pure true))
  (set `/Game/TurnBasedJRPGTemplate/Blueprints/HackMiniGames/Enemy.Block` true (cast `/Game/TurnBasedJRPGTemplate/Blueprints/HackMiniGames/Enemy` (`ChildActorComponent.ChildActor` (`self.Enemy`)) :!pure true))
  (bind _returnvalue (`|CreateWidget` "/Game/TurnBasedJRPGTemplate/Blueprints/UI/Dialogues/BP_InfoDialogueForBattle.BP_InfoDialogueForBattle_C" null "Bonus Hack Successful!" "" false null 3.0))
  (`UserWidget.AddToViewport` _returnvalue 0)
  (set `/Game/TurnBasedJRPGTemplate/Blueprints/Units/EnemyUnits/BP_EnemyUnitBase.BonusHackSuccessful` true (cast `/Game/TurnBasedJRPGTemplate/Blueprints/Units/EnemyUnits/BP_EnemyUnitBase` (`/Game/TurnBasedJRPGTemplate/Blueprints/Battle/BP_BattleController.currentTargetUnit` (`/Game/TurnBasedJRPGTemplate/Blueprints/Controllers/BP_JRPGPlayerController.GetBattleController` (`self.As BP JRPGPlayer Controller`))) :!pure true))
  (`KismetSystemLibrary.Delay` 3.0)
  (`self.K2_DestroyActor`)
  (`self.Game over`))

(event `Can do input`
  ;[1 1 1] Outcome of successful or unsuccessful events!
  (set `/Game/TurnBasedJRPGTemplate/Blueprints/Controllers/BP_JRPGPlayerController.gameState` "NewEnumerator5" (`self.As BP JRPGPlayer Controller`)))

(fn `UserConstructionScript`)