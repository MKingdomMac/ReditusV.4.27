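; Usable battle item for the turn-based JRPG that throws an EMP grenade, restricted to the Augustus (engineer) unit.
; On use it fires a projectile at the current target, whose hit callback plays an explosion, calls DealDamage and signals item use if it lands.
; Other units see a brief warning, get the item refunded and restart their turn.
; A no-effect projectile branch exists but is disconnected.
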(event `self.OnUsedInBattle`
  (params (unit :type "/Game/TurnBasedJRPGTemplate/Blueprints/Units/BP_UnitBase Object Reference") (unitClass :type "/Game/TurnBasedJRPGTemplate/Blueprints/Units/BP_UnitBase Class Reference"))
  (bind _battlecontroller (`self.battleController`))
  (bind _battlecontroller_2 (`self.battleController`))
  (if (== (`GameplayStatics.GetObjectClass` (`/Game/TurnBasedJRPGTemplate/Blueprints/Battle/BP_BattleController.currentAttackingUnit` _battlecontroller)) "/Game/TurnBasedJRPGTemplate/Blueprints/Units/PlayerUnits/BP_AugustusPlayerUnit.BP_AugustusPlayerUnit_C")
    (bind _projectilespawntransform (`/Game/TurnBasedJRPGTemplate/Blueprints/Units/BP_UnitBase.GetProjectileSpawnTransform` (`/Game/TurnBasedJRPGTemplate/Blueprints/Battle/BP_BattleController.currentAttackingUnit` _battlecontroller)))
    (bind _returnvalue (`|SpawnActorFromClass` "/Game/TurnBasedJRPGTemplate/Blueprints/Projectiles/Grenades/BP_EmpGrenadeProjectile.BP_EmpGrenadeProjectile_C" _projectilespawntransform "Undefined" "OverrideRootScale" null (`/Game/TurnBasedJRPGTemplate/Blueprints/Battle/BP_BattleController.currentTargetUnit` _battlecontroller) null))
    (add `/Game/TurnBasedJRPGTemplate/Blueprints/Projectiles/BP_GrenadeProjectileBase.OnProjectileHit` _returnvalue (delegate `Hit`))
    (`/Game/TurnBasedJRPGTemplate/Blueprints/Projectiles/BP_GrenadeProjectileBase.MoveProjectileToTarget` _returnvalue)
    (else
      (bind _returnvalue_2 (`|CreateWidget` "/Game/TurnBasedJRPGTemplate/Blueprints/UI/Dialogues/BP_InfoDialogueForBattle.BP_InfoDialogueForBattle_C" null "Only engineer class can use this item" "" false null))
      (`UserWidget.AddToViewport` _returnvalue_2 0)
      (`KismetSystemLibrary.Delay` 1.0)
      (`Widget.RemoveFromParent` _returnvalue_2)
      (`/Game/TurnBasedJRPGTemplate/Blueprints/Controllers/BP_JRPGPlayerController.AddUsableItemToInventory` (`/Game/TurnBasedJRPGTemplate/Blueprints/Battle/BP_BattleController.jRPGPlayerController` _battlecontroller_2) "Bp_EmpGrenades_C" 1)
      (`/Game/TurnBasedJRPGTemplate/Blueprints/Units/BP_UnitBase.StartTurn` (`/Game/TurnBasedJRPGTemplate/Blueprints/Battle/BP_BattleController.currentAttackingUnit` _battlecontroller_2))
      (`self.K2_DestroyActor`))))

(event `Hit`
  (`GameplayStatics.PlaySoundAtLocation` "/Game/Sounds/Fx/Explosions/Clusters/sfx_exp_cluster6.sfx_exp_cluster6" (0.0 0.0 0.0) (struct) 1.0 1.0 0.0 null null null)
  (bind _ishit (`/Game/TurnBasedJRPGTemplate/Blueprints/Battle/BP_BattleController.DealDamage` (`self.battleController`) 0 1.0 0.0))
  (if _ishit
    (`self.OnItemUsed` :!label _label)))

(event `No Effect`
  (`GameplayStatics.PlaySoundAtLocation` "/Game/Sounds/Fx/Explosions/Clusters/sfx_exp_cluster6.sfx_exp_cluster6" (0.0 0.0 0.0) (struct) 1.0 1.0 0.0 null null null)
  (goto _label))

(fn `UserConstructionScript`
  (`parent.UserConstructionScript`))