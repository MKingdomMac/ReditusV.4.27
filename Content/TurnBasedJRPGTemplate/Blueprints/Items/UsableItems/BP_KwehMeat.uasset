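; Usable Kweh Meat item for the turn-based JRPG that restores 100% of a unit's max HP, in or out of battle.
; In battle it plays the unit's item-use montage, spawns a healing effect on its Pixel2D component, heals, then waits briefly before signaling completion.
; Outside battle it writes the HP, capped at max, into the player controller's unit data map and signals completion immediately.
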(event `self.OnUsedInBattle`
  (params (unit :type "/Game/TurnBasedJRPGTemplate/Blueprints/Units/BP_UnitBase Object Reference") (unitClass :type Name))
  ;[1 1 1] Restore 100% HP in battle
  (`/Game/TurnBasedJRPGTemplate/Blueprints/Units/BP_UnitBase.PlayAnimationMontage` unit (`/Game/TurnBasedJRPGTemplate/Blueprints/Units/BP_UnitBase.itemUseAnimationMontage` unit))
  (`|SpawnActorFromClass` "/Game/TurnBasedJRPGTemplate/Blueprints/Projectiles/ParticleEffects/Healing/BP_HealingEffect.BP_HealingEffect_C" (`SceneComponent.GetSocketTransform` (`/Game/TurnBasedJRPGTemplate/Blueprints/Units/BP_UnitBase.Pixel2D` unit) "None" "RTS_World") "Undefined" "OverrideRootScale" null null)
  (`/Game/TurnBasedJRPGTemplate/Blueprints/Units/BP_UnitBase.Heal` unit (`KismetMathLibrary.FTrunc` (* (`/Game/TurnBasedJRPGTemplate/Blueprints/Units/BP_UnitBase.maxHP` unit) 1.0)) 0)
  (`KismetSystemLibrary.Delay` 1.5)
  (`self.OnItemUsed`))

(event `self.OnUsedOutsideBattle`
  (params (playerUnit :type Name))
  (bind _value (`BlueprintMapLibrary.Map_Find` (`/Game/TurnBasedJRPGTemplate/Blueprints/Controllers/BP_JRPGPlayerController.PlayerUnitDataID` (`self.jRPGPlayerController`)) playerUnit))
  ;[1 1 1] Restore 100% HP outside battle
  (bind _playerunitstats (`/Game/TurnBasedJRPGTemplate/Blueprints/Controllers/BP_JRPGFunctionLibrary.GetPlayerUnitStatsFromID` playerUnit _value))
  (bind ((`maxHP_2_41B41BC24C39ED8CDC0C58B3398B651D` _maxhp)) (break `/Game/TurnBasedJRPGTemplate/Blueprints/Structs/S_UnitStats` _playerunitstats))
  (bind _structout (setmembers `/Game/TurnBasedJRPGTemplate/Blueprints/Structs/S_PlayerUnitData` :`StructRef` _value :`currentHP` (`KismetMathLibrary.Min` _maxhp (+ (`KismetMathLibrary.FTrunc` (* _maxhp 1.0)) (`.currentHP_4_0B53A15447C685E66E26429EA6694AA4` (break `/Game/TurnBasedJRPGTemplate/Blueprints/Structs/S_PlayerUnitData` _value))))))
  (`BlueprintMapLibrary.Map_Add` (`/Game/TurnBasedJRPGTemplate/Blueprints/Controllers/BP_JRPGPlayerController.PlayerUnitDataID` (`self.jRPGPlayerController`)) playerUnit _structout)
  (`self.OnItemUsed`))

(fn `UserConstructionScript`
  (`parent.UserConstructionScript`))