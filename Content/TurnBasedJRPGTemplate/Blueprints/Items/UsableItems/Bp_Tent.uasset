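; Tent usable item for the JRPG template that fully restores the party's HP and MP when used outside battle.
; It loops over every entry in the player controller's unit data map, looks up each unit's max stats and writes the updated struct back into the map.
; It then plays a heal sound and signals that the item was used.
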(event `self.OnUsedOutsideBattle`
  (params (playerUnit :type Name))
  (bind _playerunitdataid (`/Game/TurnBasedJRPGTemplate/Blueprints/Controllers/BP_JRPGPlayerController.PlayerUnitDataID` (`self.jRPGPlayerController`)))
  (bind _keys (`BlueprintMapLibrary.Map_Keys` _playerunitdataid))
  (for _array_element _keys
    (bind _value (`BlueprintMapLibrary.Map_Find` _playerunitdataid _array_element))
    (bind _playerunitstats (`/Game/TurnBasedJRPGTemplate/Blueprints/Controllers/BP_JRPGFunctionLibrary.GetPlayerUnitStatsFromID` _array_element _value))
    (bind ((`maxHP_2_41B41BC24C39ED8CDC0C58B3398B651D` _maxhp) (`maxMP_4_402F570E47A131E33E462B9D0D778331` _maxmp)) (break `/Game/TurnBasedJRPGTemplate/Blueprints/Structs/S_UnitStats` _playerunitstats))
    (bind _structout (setmembers `/Game/TurnBasedJRPGTemplate/Blueprints/Structs/S_PlayerUnitData` :`StructRef` _value :`currentHP` _maxhp :`curentMP` _maxmp :`PoisonDamage` false :`IsBlinded` false :`IsBerserk` false :`IsPetrified` false :`IsZombie` false :`IsImp` false :`IsSilenced` false))
    (`BlueprintMapLibrary.Map_Add` (`/Game/TurnBasedJRPGTemplate/Blueprints/Controllers/BP_JRPGPlayerController.PlayerUnitDataID` (`self.jRPGPlayerController`)) _array_element _structout))
  (`GameplayStatics.PlaySoundAtLocation` "/Game/Sounds/Se/Heal1.Heal1_0" (0.0 0.0 0.0) (struct) 1.0 1.0 0.0 null null null)
  (`self.OnItemUsed`))

(fn `UserConstructionScript`
  (`parent.UserConstructionScript`))