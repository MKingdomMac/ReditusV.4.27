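; BP_WaypointItem is a usable JRPG item that drops a waypoint when used outside battle.
; It spawns a BP_WaypointDevice at the explore character's location and records that actor's transform in the player controller's WaypointSpawns array.
; It then plays a sound at the world origin and calls OnItemUsed to signal that the item was used.
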(event `self.OnUsedOutsideBattle`
  (params (playerUnit :type "/Game/TurnBasedJRPGTemplate/Blueprints/Units/PlayerUnits/BP_PlayerUnitBase Class Reference"))
  ;[1 1 1] Drop Waypoint
  (bind _returnvalue (`|SpawnActorFromClass` "/Game/TurnBasedJRPGTemplate/Blueprints/Interactables/BP_WaypointDevice.BP_WaypointDevice_C" (`KismetMathLibrary.MakeTransform` (`self.K2_GetActorLocation` (`/Game/TurnBasedJRPGTemplate/Blueprints/Controllers/BP_JRPGPlayerController.exploreCharacter` (`self.jRPGPlayerController`)))) "Undefined" "OverrideRootScale" null "Obtained item(s)!" null))
  (`KismetArrayLibrary.Array_Add` (`/Game/TurnBasedJRPGTemplate/Blueprints/Controllers/BP_JRPGPlayerController.WaypointSpawns` (`self.jRPGPlayerController`)) (`self.GetTransform` _returnvalue))
  (`GameplayStatics.PlaySoundAtLocation` "/Game/Sounds/Se/Heal1.Heal1_0" (0.0 0.0 0.0) (struct) 1.0 1.0 0.0 null null null)
  (`self.OnItemUsed`))

(fn `UserConstructionScript`
  (`parent.UserConstructionScript`))