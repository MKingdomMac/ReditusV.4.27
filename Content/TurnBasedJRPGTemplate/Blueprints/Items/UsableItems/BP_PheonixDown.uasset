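; Usable Phoenix Down item that revives a fallen party member with a small fraction of max HP, in or outside battle.
; In battle, it saves the new HP, spawns a replacement unit matching the dead one's placement, and registers it with battle and UI.
; When the revive effect finishes, it rebuilds unit lists and destroys the old actor.
; Outside battle, it only updates saved HP, plays a sound and signals item use.
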(event `self.OnUsedInBattle`
  (params (unit :type "/Game/TurnBasedJRPGTemplate/Blueprints/Units/BP_UnitBase Object Reference") (unitClass :type Name))
  (bind _playerunitclass (`self.playerUnitClass`))
  (bind _battlecontroller (`self.battleController`))
  (bind _battlecontroller_2 (`self.battleController`))
  (bind _battlecontroller_3 (`self.battleController`))
  (bind _returnvalue (`SceneComponent.GetSocketTransform` (`/Game/TurnBasedJRPGTemplate/Blueprints/Units/BP_UnitBase.Pixel2D` unit) "None" "RTS_World"))
  (bind _readytoattackunits (`/Game/TurnBasedJRPGTemplate/Blueprints/Battle/BP_BattleController.readyToAttackUnits` _battlecontroller_2))
  (bind _currentbattle (`/Game/TurnBasedJRPGTemplate/Blueprints/Battle/BP_BattleController.currentBattle` (`self.battleController`)))
  (bind _value (`BlueprintMapLibrary.Map_Find` (`/Game/TurnBasedJRPGTemplate/Blueprints/Controllers/BP_JRPGPlayerController.PlayerUnitDataID` (`self.jRPGPlayerController`)) (`self.playerUnitClass`)))
  (bind (_value_2 _returnvalue_2) (`BlueprintMapLibrary.Map_Find` (`/Game/TurnBasedJRPGTemplate/Blueprints/Controllers/BP_JRPGPlayerController.PlayerUnitDataID` (`self.jRPGPlayerController`)) (`self.playerUnitClass`)))
  (bind (_value_3 _returnvalue_3) (`BlueprintMapLibrary.Map_Find` (`/Game/TurnBasedJRPGTemplate/Blueprints/Battle/BP_BattleBase.DeadCharactersByID` _currentbattle) (`self.playerUnitClass`)))
  ;[1 1 1] Revive unit in battle
  (`/Engine/EditorBlueprintResources/StandardMacros.IsValid` unit
    (:`Is Valid`
      (bind _output_get (set `self.playerUnitClass` unitClass))
      (if _returnvalue_2
        (bind (_playerunitstats _level _found) (`/Game/TurnBasedJRPGTemplate/Blueprints/Controllers/BP_JRPGFunctionLibrary.GetPlayerUnitStatsFromID` _output_get _value_2))
        (if _found
          (if _returnvalue_3
            (bind _structout (setmembers `/Game/TurnBasedJRPGTemplate/Blueprints/Structs/S_PlayerUnitData` :`StructRef` _value :`currentHP` (`KismetMathLibrary.Max` (`KismetMathLibrary.FTrunc` (* (`.maxHP_2_41B41BC24C39ED8CDC0C58B3398B651D` (break `/Game/TurnBasedJRPGTemplate/Blueprints/Structs/S_UnitStats` _playerunitstats)) 0.02)) 1)))
            (`BlueprintMapLibrary.Map_Add` (`/Game/TurnBasedJRPGTemplate/Blueprints/Controllers/BP_JRPGPlayerController.PlayerUnitDataID` (`self.jRPGPlayerController`)) (`self.playerUnitClass`) _structout)
            (bind _returnvalue_4 (`|SpawnActorFromClass` :`Class` "/Game/TurnBasedJRPGTemplate/Blueprints/Units/PlayerUnits/BP_PlayerUnitBase.BP_PlayerUnitBase_C" :`SpawnTransform` _value_3 :`CollisionHandlingOverride` "AlwaysSpawn" :`TransformScaleMethod` "OverrideRootScale" :`CharacterID` _playerunitclass :`level` _level :`battle` _currentbattle :`Instigator` null))
            (`/Engine/EditorBlueprintResources/StandardMacros.IsValid` _returnvalue_4
              (:`Is Valid`
                (`/Game/TurnBasedJRPGTemplate/Blueprints/Units/PlayerUnits/BP_PlayerUnitBase.InitializePlayerUnitID` _returnvalue_4 _playerunitclass _value _battlecontroller_3)
                (`SceneComponent.K2_SetWorldTransform` (`/Game/TurnBasedJRPGTemplate/Blueprints/Units/BP_UnitBase.SkeletalMesh` _returnvalue_4) (`SceneComponent.GetSocketTransform` (`/Game/TurnBasedJRPGTemplate/Blueprints/Units/BP_UnitBase.SkeletalMesh` unit) "None" "RTS_World") false true)
                (`SceneComponent.K2_SetWorldTransform` (`/Game/TurnBasedJRPGTemplate/Blueprints/Units/BP_UnitBase.Pixel2D` _returnvalue_4) _returnvalue false true)
                (set `/Game/TurnBasedJRPGTemplate/Blueprints/Units/BP_UnitBase.initialLocation` (`/Game/TurnBasedJRPGTemplate/Blueprints/Units/BP_UnitBase.initialLocation` unit) _returnvalue_4)
                (set `/Game/TurnBasedJRPGTemplate/Blueprints/Units/BP_UnitBase.initialRotation` (`/Game/TurnBasedJRPGTemplate/Blueprints/Units/BP_UnitBase.initialRotation` unit) _returnvalue_4)
                (`KismetArrayLibrary.Array_Add` (`/Game/TurnBasedJRPGTemplate/Blueprints/Battle/BP_BattleBase.playerUnits` _currentbattle) _returnvalue_4)
                (`SceneComponent.SetHiddenInGame` (`/Game/TurnBasedJRPGTemplate/Blueprints/Units/BP_UnitBase.Pixel2D` unit) true false)
                (`/Game/TurnBasedJRPGTemplate/Blueprints/UI/BP_PlayerUnitListUI.DisplayUnitUI` (`/Game/TurnBasedJRPGTemplate/Blueprints/UI/BP_BattleUI.BP_PlayerUnitListUI` (`/Game/TurnBasedJRPGTemplate/Blueprints/Battle/BP_BattleController.battleUI` _battlecontroller)) _returnvalue_4 _battlecontroller_3)
                (`/Game/TurnBasedJRPGTemplate/Blueprints/Units/BP_UnitBase.UpdateAmpGauge` _returnvalue_4 (`/Game/TurnBasedJRPGTemplate/Blueprints/Units/BP_UnitBase.Current Exhaust Points` _returnvalue_4) 0 false false false true)
                (`BlueprintMapLibrary.Map_Remove` (`/Game/TurnBasedJRPGTemplate/Blueprints/Battle/BP_BattleBase.DeadCharactersByID` (`/Game/TurnBasedJRPGTemplate/Blueprints/Battle/BP_BattleController.currentBattle` _battlecontroller)) (`self.playerUnitClass`))
                (`/Game/TurnBasedJRPGTemplate/Blueprints/UI/BP_TurnOrderList.SetRevivedUnit` (`/Game/TurnBasedJRPGTemplate/Blueprints/UI/BP_BattleUI.BP_TurnOrderList` (`/Game/TurnBasedJRPGTemplate/Blueprints/Battle/BP_BattleController.battleUI` (`self.battleController`))) _returnvalue_4)
                (`GameplayStatics.PlaySoundAtLocation` "/Game/Sounds/Se/Heal3.Heal3_0" (0.0 0.0 0.0) (struct) 1.0 1.0 0.0 null null null)
                (bind _returnvalue_5 (`|SpawnActorFromClass` "/Game/TurnBasedJRPGTemplate/Blueprints/Projectiles/ParticleEffects/Healing/BP_ReviveEffect1.BP_ReviveEffect1_C" _returnvalue "AlwaysSpawn" "OverrideRootScale" null null))
                (`/Engine/EditorBlueprintResources/StandardMacros.IsValid` _returnvalue_5
                  (:`Is Valid`
                    (add `/Game/TurnBasedJRPGTemplate/Blueprints/Projectiles/ParticleEffects/Healing/BP_ReviveEffect1.Particle Destroyed` _returnvalue_5 (delegate `CustomEvent_2`)))
                  (:`Is Not Valid`
                    (`/Game/TurnBasedJRPGTemplate/Blueprints/Battle/BP_BattleBase.SetAllUnitsArray` (`/Game/TurnBasedJRPGTemplate/Blueprints/Battle/BP_BattleController.currentBattle` _battlecontroller_2) :!label _label)
                    (if (!= (`KismetArrayLibrary.Array_Find` _readytoattackunits unit) -1)
                      (`KismetArrayLibrary.Array_RemoveItem` _readytoattackunits unit)
                      (`KismetArrayLibrary.Array_Add` _readytoattackunits _returnvalue_4))
                    (`self.K2_DestroyActor` unit)
                    (`self.OnItemUsed` :!label _label_2))))
              (:`Is Not Valid`
                (`KismetSystemLibrary.PrintString` "Phoenix Down failed: target, saved data, stats, transform, or replacement actor is missing." true true (struct :`R` 1.0 :`G` 0.036022 :`B` 0.135688 :`A` 1.0) 10.0 :!label _label_3)
                (goto _label_2)))
            (else
              (goto _label_3)))
          (else
            (goto _label_3)))
        (else
          (goto _label_3))))
    (:`Is Not Valid`
      (goto _label_3))))

(event `CustomEvent_2`
  ;[1 1 1] Revive unit in battle
  (goto _label))

(event `self.OnUsedOutsideBattle`
  (params (playerUnit :type Name))
  (bind _value (`BlueprintMapLibrary.Map_Find` (`/Game/TurnBasedJRPGTemplate/Blueprints/Controllers/BP_JRPGPlayerController.PlayerUnitDataID` (`self.jRPGPlayerController`)) playerUnit))
  ;[1 1 1] Revive unit outside battle
  (bind _playerunitstats (`/Game/TurnBasedJRPGTemplate/Blueprints/Controllers/BP_JRPGFunctionLibrary.GetPlayerUnitStatsFromID` playerUnit _value))
  (bind _structout (setmembers `/Game/TurnBasedJRPGTemplate/Blueprints/Structs/S_PlayerUnitData` :`StructRef` _value :`currentHP` (`KismetMathLibrary.FTrunc` (* (`.maxHP_2_41B41BC24C39ED8CDC0C58B3398B651D` (break `/Game/TurnBasedJRPGTemplate/Blueprints/Structs/S_UnitStats` _playerunitstats)) 0.02))))
  (`BlueprintMapLibrary.Map_Add` (`/Game/TurnBasedJRPGTemplate/Blueprints/Controllers/BP_JRPGPlayerController.PlayerUnitDataID` (`self.jRPGPlayerController`)) playerUnit _structout)
  (`GameplayStatics.PlaySoundAtLocation` "/Game/Sounds/Se/Heal3.Heal3_0" (0.0 0.0 0.0) (struct) 1.0 1.0 0.0 null null null)
  (`self.OnItemUsed`))

(fn `UserConstructionScript`
  (`parent.UserConstructionScript`))