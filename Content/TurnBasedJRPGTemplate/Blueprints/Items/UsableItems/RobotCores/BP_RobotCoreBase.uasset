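; Base usable item for robot cores that installs a core on a player unit when used outside battle.
; Installing writes the core's affinity and installed flag into that unit's entry in the player controller's unit data map.
; It then plays machine and hammer sounds and shows an info dialogue, whose confirmation triggers a Steam achievement and signals that the item was used.
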(event `self.OnUsedOutsideBattle`
  (params (playerUnit :type Name))
  (bind _structout (setmembers `/Game/TurnBasedJRPGTemplate/Blueprints/Structs/S_PlayerUnitData` :`StructRef` (`BlueprintMapLibrary.Map_Find` (`/Game/TurnBasedJRPGTemplate/Blueprints/Controllers/BP_JRPGPlayerController.PlayerUnitDataID` (`self.jRPGPlayerController`)) playerUnit) :`Exp` 0 :`currentHP` 0 :`curentMP` 0 :`CurrentOverDrivePoints` 0.0 :`CurrentExhaustionPoints` 0 :`PoisonDamage` false :`IsBlinded` false :`IsBerserk` false :`IsPetrified` false :`IsZombie` false :`IsImp` false :`IsSilenced` false :`CurrentUnitAffinity` (`self.CoreAffinity`) :`IsCoreInstalled` true :`HasGivenCore` false :`Boots` null))
  (`BlueprintMapLibrary.Map_Add` (`/Game/TurnBasedJRPGTemplate/Blueprints/Controllers/BP_JRPGPlayerController.PlayerUnitDataID` (`self.jRPGPlayerController`)) playerUnit _structout)
  (`GameplayStatics.PlaySound2D` "/Game/Sounds/Se/Machine.Machine_0" 1.0 1.0 0.0 null null)
  (`GameplayStatics.PlaySound2D` "/Game/Sounds/Se/Hammer.Hammer_0" 1.0 1.0 0.0 null null)
  (`GameplayStatics.PlaySound2D` "/Game/Sounds/Se/Hammer.Hammer_0" 1.0 1.0 0.0 null null)
  (bind _returnvalue (`|CreateWidget` "/Game/TurnBasedJRPGTemplate/Blueprints/UI/Dialogues/BP_InfoDialogue.BP_InfoDialogue_C" null "New Core Installed!" "" false null))
  (`UserWidget.AddToViewport` _returnvalue 0)
  (add `/Game/TurnBasedJRPGTemplate/Blueprints/UI/Dialogues/BP_InfoDialogue.OnConfirmed` _returnvalue (delegate `CoreInstalled`)))

(event `CoreInstalled`
  (`/Game/TurnBasedJRPGTemplate/Blueprints/Controllers/BP_JRPGPlayerController.SteamAchievements` (`self.jRPGPlayerController`) "The Core!")
  (`self.OnItemUsed`))

(fn `UserConstructionScript`
  (`parent.UserConstructionScript`))