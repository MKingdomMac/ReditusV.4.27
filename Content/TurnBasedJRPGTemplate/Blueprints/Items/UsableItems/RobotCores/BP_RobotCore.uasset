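; BP_RobotCore is a usable item that installs a robot core on a player unit when used outside battle.
; It looks up the unit's data in the player controller's PlayerUnits map, sets its affinity to the core's CoreAffinity and marks the core as installed.
; The updated struct is written back to the map, then the item-used call fires.
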(event `self.OnUsedOutsideBattle`
  (params (playerUnit :type "/Game/TurnBasedJRPGTemplate/Blueprints/Units/PlayerUnits/BP_PlayerUnitBase Class Reference") (unitbase :type "/Game/TurnBasedJRPGTemplate/Blueprints/Units/BP_UnitBase Class Reference"))
  (bind _structout (setmembers `/Game/TurnBasedJRPGTemplate/Blueprints/Structs/S_PlayerUnitData` :`StructRef` (`BlueprintMapLibrary.Map_Find` (`/Game/TurnBasedJRPGTemplate/Blueprints/Controllers/BP_JRPGPlayerController.playerUnits` (`self.jRPGPlayerController`)) playerUnit) :`CurrentUnitAffinity` (`self.CoreAffinity`) :`IsCoreInstalled` true))
  (`BlueprintMapLibrary.Map_Add` (`/Game/TurnBasedJRPGTemplate/Blueprints/Controllers/BP_JRPGPlayerController.playerUnits` (`self.jRPGPlayerController`)) playerUnit _structout)
  (`self.OnItemUsed`))

(fn `UserConstructionScript`
  (`parent.UserConstructionScript`))