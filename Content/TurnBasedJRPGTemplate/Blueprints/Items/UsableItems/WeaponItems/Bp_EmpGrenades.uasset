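; Usable EMP grenade item for turn-based battles that damages the current target unit.
; When used, it spawns an EMP grenade projectile with a lightning hit effect at the attacking unit's spawn transform and moves it to the target.
; The projectile's hit callback plays an explosion sound, deals damage through the BattleController with an amp-adjusted multiplier, then signals item use.
; An unconnected "Is Skill Item" refund branch never runs.
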(event `self.OnUsedInBattle`
  (params (unit :type "/Game/TurnBasedJRPGTemplate/Blueprints/Units/BP_UnitBase Object Reference") (unitClass :type Name))
  (bind _battlecontroller (`self.battleController`))
  (bind _projectilespawntransform (`/Game/TurnBasedJRPGTemplate/Blueprints/Units/BP_UnitBase.GetProjectileSpawnTransform` (`/Game/TurnBasedJRPGTemplate/Blueprints/Battle/BP_BattleController.currentAttackingUnit` _battlecontroller)))
  (bind _returnvalue (`|SpawnActorFromClass` "/Game/TurnBasedJRPGTemplate/Blueprints/Projectiles/Grenades/BP_EmpGrenadeProjectile.BP_EmpGrenadeProjectile_C" _projectilespawntransform "Undefined" "OverrideRootScale" null true "/Game/Particles/InfinityBladeEffects/Effects/FX_Combat_Lightning/P_DOT_Lightning_01.P_DOT_Lightning_01" null (`/Game/TurnBasedJRPGTemplate/Blueprints/Battle/BP_BattleController.currentTargetUnit` _battlecontroller) null null))
  (add `/Game/TurnBasedJRPGTemplate/Blueprints/Projectiles/BP_GrenadeProjectileBase.OnProjectileHit` _returnvalue (delegate `Hit`))
  (`/Game/TurnBasedJRPGTemplate/Blueprints/Projectiles/BP_GrenadeProjectileBase.MoveProjectileToTarget` _returnvalue))

(event `Hit`
  (`GameplayStatics.PlaySoundAtLocation` "/Game/Sounds/Fx/Explosions/Clusters/sfx_exp_cluster6.sfx_exp_cluster6" (0.0 0.0 0.0) (struct) 1.0 1.0 0.0 null null null)
  (bind _returnvalue (`self.Calculate Amp Damage` (`self.Damage Multiplier`)))
  (`/Game/TurnBasedJRPGTemplate/Blueprints/Battle/BP_BattleController.DealDamage` (`self.battleController`) 30 _returnvalue 0.0)
  (`self.OnItemUsed`))

(fn `UserConstructionScript`
  (`parent.UserConstructionScript`))