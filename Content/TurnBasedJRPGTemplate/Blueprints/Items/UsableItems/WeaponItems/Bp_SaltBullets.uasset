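; Salt Bullets usable weapon item for the JRPG battle system, which currently refuses direct use in battle.
; On use it briefly shows an "Is skill item." dialogue, refunds itself, restarts the unit's turn and self-destroys.
; A moved-to-target handler plays muzzle flash and sound, then deals damage boosted by amp points.
; The Augustus-only check that would trigger that attack is disconnected.
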(event `self.OnUsedInBattle`
  (params (unit :type "/Game/TurnBasedJRPGTemplate/Blueprints/Units/BP_UnitBase Object Reference") (unitClass :type "/Game/TurnBasedJRPGTemplate/Blueprints/Units/BP_UnitBase Class Reference"))
  (bind _battlecontroller (`self.battleController`))
  (bind _returnvalue (`|CreateWidget` "/Game/TurnBasedJRPGTemplate/Blueprints/UI/Dialogues/BP_InfoDialogueForBattle.BP_InfoDialogueForBattle_C" null "Is skill item." "" false null))
  (`UserWidget.AddToViewport` _returnvalue 0)
  (`KismetSystemLibrary.Delay` 1.0)
  (`Widget.RemoveFromParent` _returnvalue)
  (`/Game/TurnBasedJRPGTemplate/Blueprints/Controllers/BP_JRPGPlayerController.AddUsableItemToInventory` (`/Game/TurnBasedJRPGTemplate/Blueprints/Battle/BP_BattleController.jRPGPlayerController` _battlecontroller) "Bp_SaltBullets_C" 1)
  (`/Game/TurnBasedJRPGTemplate/Blueprints/Units/BP_UnitBase.StartTurn` (`/Game/TurnBasedJRPGTemplate/Blueprints/Battle/BP_BattleController.currentAttackingUnit` _battlecontroller))
  (`self.K2_DestroyActor`))

(event `On moved to target`
  (bind _currentattackingunit (`/Game/TurnBasedJRPGTemplate/Blueprints/Battle/BP_BattleController.currentAttackingUnit` (`self.battleController`)))
  (`/Game/TurnBasedJRPGTemplate/Blueprints/Units/BP_UnitBase.RangeVariablesSet` _currentattackingunit)
  (`KismetSystemLibrary.Delay` 0.1)
  (`/Game/TurnBasedJRPGTemplate/Blueprints/Units/BP_UnitBase.RangeVariablesSet` _currentattackingunit)
  (`GameplayStatics.SpawnEmitterAttached` "/Game/Particles/AdvancedMagicFX13/Particles/P_SaltBullet_Muzzle_Flash.P_SaltBullet_Muzzle_Flash" (`/Game/TurnBasedJRPGTemplate/Blueprints/Units/BP_UnitBase.Pixel2D` _currentattackingunit) "RifleShotAugustus" (0.0 0.0 0.0) (struct :`Yaw` -180.0))
  (`GameplayStatics.PlaySound2D` "/Game/Sounds/Se/Laser1.Laser1_0" 1.0 1.0 0.0 null null)
  (`KismetSystemLibrary.Delay` 0.5)
  (bind _output_get (set `self.Damage Multiplier` (+ (`self.Damage Multiplier`) (`KismetMathLibrary.Conv_IntToDouble` (`/Game/TurnBasedJRPGTemplate/Blueprints/Units/BP_UnitBase.CurrentAmpPointsInPlay` (`/Game/TurnBasedJRPGTemplate/Blueprints/Battle/BP_BattleController.currentAttackingUnit` (`self.battleController`)))))))
  (`/Game/TurnBasedJRPGTemplate/Blueprints/Battle/BP_BattleController.DealDamage` (`self.battleController`) 0 _output_get (`self.Crit`))
  (`self.OnItemUsed`))

(fn `UserConstructionScript`
  (`parent.UserConstructionScript`))