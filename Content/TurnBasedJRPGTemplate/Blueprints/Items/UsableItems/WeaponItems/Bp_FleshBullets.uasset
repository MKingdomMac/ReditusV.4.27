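; Flesh Bullets usable item for the turn-based JRPG battle system, which cannot be consumed directly in battle.
; On use, it briefly shows an "Is Skill Item" dialogue, returns itself to the inventory, restarts the attacking unit's turn and destroys itself.
; Disconnected EMP grenade projectile logic remains in the graph, with hit and no-effect handlers that play an explosion sound and end item use.
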(event `self.OnUsedInBattle`
  (params (unit :type "/Game/TurnBasedJRPGTemplate/Blueprints/Units/BP_UnitBase Object Reference") (unitClass :type "/Game/TurnBasedJRPGTemplate/Blueprints/Units/BP_UnitBase Class Reference"))
  (bind _battlecontroller (`self.battleController`))
  (bind _returnvalue (`|CreateWidget` "/Game/TurnBasedJRPGTemplate/Blueprints/UI/Dialogues/BP_InfoDialogueForBattle.BP_InfoDialogueForBattle_C" null "Is Skill Item" "" false null))
  (`UserWidget.AddToViewport` _returnvalue 0)
  (`KismetSystemLibrary.Delay` 1.0)
  (`Widget.RemoveFromParent` _returnvalue)
  (`/Game/TurnBasedJRPGTemplate/Blueprints/Controllers/BP_JRPGPlayerController.AddUsableItemToInventory` (`/Game/TurnBasedJRPGTemplate/Blueprints/Battle/BP_BattleController.jRPGPlayerController` _battlecontroller) "Bp_FleshBullets_C" 1)
  (`/Game/TurnBasedJRPGTemplate/Blueprints/Units/BP_UnitBase.StartTurn` (`/Game/TurnBasedJRPGTemplate/Blueprints/Battle/BP_BattleController.currentAttackingUnit` _battlecontroller))
  (`self.K2_DestroyActor`))

(event `Hit`
  (`GameplayStatics.PlaySoundAtLocation` "/Game/Sounds/Fx/Explosions/Clusters/sfx_exp_cluster6.sfx_exp_cluster6" (0.0 0.0 0.0) (struct) 1.0 1.0 0.0 null null null)
  (`/Game/TurnBasedJRPGTemplate/Blueprints/Battle/BP_BattleController.DealDamage` (`self.battleController`) 0 1.0 0.0)
  (`self.OnItemUsed` :!label _label))

(event `No Effect`
  (`GameplayStatics.PlaySoundAtLocation` "/Game/Sounds/Fx/Explosions/Clusters/sfx_exp_cluster6.sfx_exp_cluster6" (0.0 0.0 0.0) (struct) 1.0 1.0 0.0 null null null)
  (goto _label))

(fn `UserConstructionScript`
  (`parent.UserConstructionScript`))