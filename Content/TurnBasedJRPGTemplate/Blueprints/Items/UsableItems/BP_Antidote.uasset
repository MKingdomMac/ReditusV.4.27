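; BP_Antidote is a usable JRPG item that cures poison, both in and out of battle.
; In battle, it signals the end of the unit's damage-over-time buff, spawns an effect at the status socket, removes poison and reports use after a short delay.
; Outside battle, it clears the poison flag in the player controller's unit data map and reports use immediately.
; Both paths play a heal sound.
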(event `self.OnUsedInBattle`
  (params (unit :type "/Game/TurnBasedJRPGTemplate/Blueprints/Units/BP_UnitBase Object Reference") (unitClass :type Name))
  ;[1 1 1] Remove Poison
  (`/Game/TurnBasedJRPGTemplate/Blueprints/Units/BP_UnitBase.OnBuffEnded` unit false false true false false false false false false false false)
  (`|SpawnActorFromClass` "/Game/TurnBasedJRPGTemplate/Blueprints/Projectiles/ParticleEffects/Healing/BP_AntidoteEffect.BP_AntidoteEffect_C" (`SceneComponent.GetSocketTransform` (`/Game/TurnBasedJRPGTemplate/Blueprints/Units/BP_UnitBase.Pixel2D` unit) "StatusSocket" "RTS_World") "Undefined" "OverrideRootScale" null null)
  (`GameplayStatics.PlaySoundAtLocation` "/Game/Sounds/Se/Heal1.Heal1_0" (0.0 0.0 0.0) (struct) 1.0 1.0 0.0 null null null)
  (`/Game/TurnBasedJRPGTemplate/Blueprints/Units/BP_UnitBase.Remove Poison` unit)
  (`KismetSystemLibrary.Delay` 1.5)
  (`self.OnItemUsed`))

(event `self.OnUsedOutsideBattle`
  (params (playerUnit :type Name))
  ;[1 1 1] Remove Poison Outside of Battle
  (bind _structout (setmembers `/Game/TurnBasedJRPGTemplate/Blueprints/Structs/S_PlayerUnitData` :`StructRef` (`BlueprintMapLibrary.Map_Find` (`/Game/TurnBasedJRPGTemplate/Blueprints/Controllers/BP_JRPGPlayerController.PlayerUnitDataID` (`self.jRPGPlayerController`)) playerUnit) :`PoisonDamage` false))
  (`BlueprintMapLibrary.Map_Add` (`/Game/TurnBasedJRPGTemplate/Blueprints/Controllers/BP_JRPGPlayerController.PlayerUnitDataID` (`self.jRPGPlayerController`)) playerUnit _structout)
  (`GameplayStatics.PlaySoundAtLocation` "/Game/Sounds/Se/Heal1.Heal1_0" (0.0 0.0 0.0) (struct) 1.0 1.0 0.0 null null null)
  (`self.OnItemUsed`))

(fn `UserConstructionScript`
  (`parent.UserConstructionScript`))