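; Fire Shot equipment mesh Blueprint that alters an Airloft player unit when equipped or removed.
; Both equipment events cast the mesh component's owner to BP_AirloftPlayerUnit, then switch its IsRangedUnit flag on or off.
; Both events also set EnemyElementWeakness to the same enum entry, so unequipping does not restore a previous element.
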(event `self.EquipmentOn`
  (params (unitMeshComponent :type "SkeletalMeshComponent Object Reference"))
  (bind _asbp_airloft_player_unit (cast `/Game/TurnBasedJRPGTemplate/Blueprints/Units/PlayerUnits/BP_AirloftPlayerUnit` (`ActorComponent.GetOwner` unitMeshComponent)))
  (set `/Game/TurnBasedJRPGTemplate/Blueprints/Units/BP_UnitBase.IsRangedUnit` true _asbp_airloft_player_unit)
  (set `/Game/TurnBasedJRPGTemplate/Blueprints/Units/BP_UnitBase.Enemy Element Weakness` "NewEnumerator5" _asbp_airloft_player_unit))

(event `self.EquipmentOff`
  (params (unitMeshComponent :type "SkeletalMeshComponent Object Reference"))
  (bind _asbp_airloft_player_unit (cast `/Game/TurnBasedJRPGTemplate/Blueprints/Units/PlayerUnits/BP_AirloftPlayerUnit` (`ActorComponent.GetOwner` unitMeshComponent)))
  (set `/Game/TurnBasedJRPGTemplate/Blueprints/Units/BP_UnitBase.IsRangedUnit` false _asbp_airloft_player_unit)
  (set `/Game/TurnBasedJRPGTemplate/Blueprints/Units/BP_UnitBase.Enemy Element Weakness` "NewEnumerator5" _asbp_airloft_player_unit))

(fn `UserConstructionScript`
  (`parent.UserConstructionScript`))