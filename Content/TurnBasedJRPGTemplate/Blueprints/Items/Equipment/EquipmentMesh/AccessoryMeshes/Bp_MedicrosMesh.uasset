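; Accessory equipment mesh actor for the Medicros item in the turn-based JRPG template, granting poison immunity to the unit wearing it.
; Its equip event casts the mesh component's owner to BP_UnitBase, adds BP_Poison to that unit's Immunities and prints a debug message.
; The unequip event removes the same immunity.
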(event `self.EquipmentOn`
  (params (unitMeshComponent :type "SkeletalMeshComponent Object Reference"))
  (bind _asbp_unit_base (cast `/Game/TurnBasedJRPGTemplate/Blueprints/Units/BP_UnitBase` (`ActorComponent.GetOwner` unitMeshComponent)))
  (`KismetSystemLibrary.PrintString` "meshapplied" true true (struct :`R` 1.0 :`G` 0.020778 :`B` 0.030725 :`A` 1.0) 10.0)
  (`KismetArrayLibrary.Array_Add` (`/Game/TurnBasedJRPGTemplate/Blueprints/Units/BP_UnitBase.Immunities` _asbp_unit_base) "/Game/TurnBasedJRPGTemplate/Blueprints/Skills/Buffs/BP_Poison.BP_Poison_C"))

(event `self.EquipmentOff`
  (params (unitMeshComponent :type "SkeletalMeshComponent Object Reference"))
  (bind _asbp_unit_base (cast `/Game/TurnBasedJRPGTemplate/Blueprints/Units/BP_UnitBase` (`ActorComponent.GetOwner` unitMeshComponent)))
  (`KismetArrayLibrary.Array_RemoveItem` (`/Game/TurnBasedJRPGTemplate/Blueprints/Units/BP_UnitBase.Immunities` _asbp_unit_base) "/Game/TurnBasedJRPGTemplate/Blueprints/Skills/Buffs/BP_Poison.BP_Poison_C"))

(fn `UserConstructionScript`
  (`parent.UserConstructionScript`))