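; Scrap rifle weapon mesh Blueprint that configures a player unit for ranged attacks when equipped.
; On equip, it casts the mesh owner to BP_PlayerUnitBase, sets the gunshot projectile and weapon particle effect, calls ScrapRifleEquipped and flags the unit as ranged.
; On unequip, it clears the projectile and ranged flag but calls ScrapSwordUnequipped rather than a rifle-named counterpart, leaving the particle effect unchanged.
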(event `self.EquipmentOn`
  (params (unitMeshComponent :type "SkeletalMeshComponent Object Reference"))
  (bind _asbp_player_unit_base (cast `/Game/TurnBasedJRPGTemplate/Blueprints/Units/PlayerUnits/BP_PlayerUnitBase` (`ActorComponent.GetOwner` unitMeshComponent)))
  (set `/Game/TurnBasedJRPGTemplate/Blueprints/Units/BP_UnitBase.projectile` "/Game/TurnBasedJRPGTemplate/Blueprints/Projectiles/PlayerGunProjectiles/BP_GunshotProjectile.BP_GunshotProjectile_C" _asbp_player_unit_base)
  (set `/Game/TurnBasedJRPGTemplate/Blueprints/Units/BP_UnitBase.AttackWeaponParticleEffectPlayer` "NewEnumerator2" _asbp_player_unit_base)
  (`/Game/TurnBasedJRPGTemplate/Blueprints/Units/BP_UnitBase.ScrapRifleEquipped` _asbp_player_unit_base)
  (set `/Game/TurnBasedJRPGTemplate/Blueprints/Units/BP_UnitBase.IsRangedUnit` true _asbp_player_unit_base))

(event `self.EquipmentOff`
  (params (unitMeshComponent :type "SkeletalMeshComponent Object Reference"))
  (bind _asbp_player_unit_base (cast `/Game/TurnBasedJRPGTemplate/Blueprints/Units/PlayerUnits/BP_PlayerUnitBase` (`ActorComponent.GetOwner` unitMeshComponent)))
  (set `/Game/TurnBasedJRPGTemplate/Blueprints/Units/BP_UnitBase.projectile` null _asbp_player_unit_base)
  (`/Game/TurnBasedJRPGTemplate/Blueprints/Units/BP_UnitBase.ScrapSwordUnequipped` _asbp_player_unit_base)
  (set `/Game/TurnBasedJRPGTemplate/Blueprints/Units/BP_UnitBase.IsRangedUnit` false _asbp_player_unit_base))

(fn `UserConstructionScript`
  (`parent.UserConstructionScript`))