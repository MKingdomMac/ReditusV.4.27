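; Scorpion Rifle equipment mesh Blueprint that gives Augustus player units gunshot attacks while the weapon is equipped.
; On equip, it sets the gunshot projectile and particle effect type on every Augustus unit found by a class search.
; On unequip, it clears only the projectile, and only on the Augustus unit owning the supplied mesh component.
; Ranged-unit flag toggles are left unwired.
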(event `self.EquipmentOn`
  (params (unitMeshComponent :type "SkeletalMeshComponent Object Reference"))
  (bind _outactors (`GameplayStatics.GetAllActorsOfClass` "/Game/TurnBasedJRPGTemplate/Blueprints/Units/PlayerUnits/BP_AugustusPlayerUnit.BP_AugustusPlayerUnit_C"))
  (for _array_element _outactors
    (set `/Game/TurnBasedJRPGTemplate/Blueprints/Units/BP_UnitBase.projectile` "/Game/TurnBasedJRPGTemplate/Blueprints/Projectiles/PlayerGunProjectiles/BP_GunshotProjectile.BP_GunshotProjectile_C" _array_element)
    (set `/Game/TurnBasedJRPGTemplate/Blueprints/Units/BP_UnitBase.PlayerChParticleEffect` "NewEnumerator2" _array_element)))

(event `self.EquipmentOff`
  (params (unitMeshComponent :type "SkeletalMeshComponent Object Reference"))
  (bind _asbp_augustus_player_unit (cast `/Game/TurnBasedJRPGTemplate/Blueprints/Units/PlayerUnits/BP_AugustusPlayerUnit` (`ActorComponent.GetOwner` unitMeshComponent)))
  (set `/Game/TurnBasedJRPGTemplate/Blueprints/Units/BP_UnitBase.projectile` null _asbp_augustus_player_unit))

(fn `UserConstructionScript`
  (`parent.UserConstructionScript`))