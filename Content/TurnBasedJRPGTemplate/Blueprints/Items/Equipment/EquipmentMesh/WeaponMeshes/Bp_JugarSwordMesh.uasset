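; Weapon mesh Blueprint for the Jugar sword in the turn-based JRPG, handling equip and unequip hooks through Scrap Sword unit calls.
; Equipping finds every BP_CaeserPlayerUnit, sets its particle-effect enum, calls ScrapSwordEquipped and prints "Failed" even on this path.
; Unequipping instead casts the mesh component's owner to BP_UnitBase and calls ScrapSwordUnequipped, printing "Failed" when the cast fails.
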(event `self.EquipmentOn`
  (params (unitMeshComponent :type "SkeletalMeshComponent Object Reference"))
  (bind _outactors (`GameplayStatics.GetAllActorsOfClass` "/Game/TurnBasedJRPGTemplate/Blueprints/Units/PlayerUnits/BP_CaeserPlayerUnit.BP_CaeserPlayerUnit_C"))
  (for _array_element _outactors
    (set `/Game/TurnBasedJRPGTemplate/Blueprints/Units/BP_UnitBase.PlayerChParticleEffect` "NewEnumerator6" _array_element)
    (`/Game/TurnBasedJRPGTemplate/Blueprints/Units/BP_UnitBase.ScrapSwordEquipped` _array_element)
    (`KismetSystemLibrary.PrintString` "Failed" :!label _label)))

(event `self.EquipmentOff`
  (params (unitMeshComponent :type "SkeletalMeshComponent Object Reference"))
  (bind _asbp_unit_base (cast `/Game/TurnBasedJRPGTemplate/Blueprints/Units/BP_UnitBase` (`ActorComponent.GetOwner` unitMeshComponent))
    (:`then`
      (`/Game/TurnBasedJRPGTemplate/Blueprints/Units/BP_UnitBase.ScrapSwordUnequipped` _asbp_unit_base))
    (:`CastFailed`
      (goto _label))))

(fn `UserConstructionScript`
  (`parent.UserConstructionScript`))