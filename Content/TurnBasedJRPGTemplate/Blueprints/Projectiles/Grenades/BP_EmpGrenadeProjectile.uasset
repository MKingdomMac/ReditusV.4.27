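; EMP grenade projectile for the turn-based JRPG template, shown as a Paper flipbook.
; It plays a 2D sound on spawn after running the parent BeginPlay.
; On DestroyProjectile it spawns either a legacy particle emitter or a system effect at double scale, chosen by a flag, and hides the flipbook.
; After a short delay it deactivates the effect and destroys itself.
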(event `self.ReceiveBeginPlay`
  ;[1 1 1] Play sound at beginning
  (`parent.ReceiveBeginPlay`)
  (`GameplayStatics.PlaySound2D` null 1.0 1.0 0.0 null null))

(event `self.DestroyProjectile`
  (if (`self.LegacyParticleHitEffect?`)
    (bind _returnvalue (`GameplayStatics.SpawnEmitterAtLocation` (`self.hitEffect`) (`self.K2_GetActorLocation`) (struct) (2.0 2.0 2.0)))
    (`SceneComponent.SetVisibility` (`self.PaperFlipbook`) false false)
    (`KismetSystemLibrary.Delay` 0.5)
    (`ActorComponent.Deactivate` _returnvalue)
    (`self.K2_DestroyActor`)
    (else
      (bind _returnvalue_2 (`NiagaraFunctionLibrary.SpawnSystemAtLocation` (`self.System Effect `) (`self.K2_GetActorLocation`) (struct) (2.0 2.0 2.0)))
      (`SceneComponent.SetVisibility` (`self.PaperFlipbook`) false false)
      (`KismetSystemLibrary.Delay` 0.5)
      (`ActorComponent.Deactivate` _returnvalue_2)
      (`self.K2_DestroyActor`))))

(fn `UserConstructionScript`
  (`parent.UserConstructionScript`))