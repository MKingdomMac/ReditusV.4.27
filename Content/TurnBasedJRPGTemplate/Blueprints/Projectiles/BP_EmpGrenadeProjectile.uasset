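; BP_EmpGrenadeProjectile is the EMP grenade projectile Blueprint for a turn-based JRPG template, extending a parent's begin-play and construction logic.
; It plays a 2D sound when spawned.
; On DestroyProjectile it spawns the hit effect at its location and hides its Paper2D flipbook.
; After a short delay it deactivates the emitter and destroys itself, so the effect shows briefly before cleanup.
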(event `self.ReceiveBeginPlay`
  ;[1 1 1] Play sound at beginning
  (`parent.ReceiveBeginPlay`)
  (`GameplayStatics.PlaySound2D` null 1.0 1.0 0.0 null null))

(event `self.DestroyProjectile`
  (bind _returnvalue (`GameplayStatics.SpawnEmitterAtLocation` (`self.hitEffect`) (`self.K2_GetActorLocation`)))
  (`SceneComponent.SetVisibility` (`self.PaperFlipbook`) false false)
  (`KismetSystemLibrary.Delay` 0.5)
  (`ActorComponent.Deactivate` _returnvalue)
  (`self.K2_DestroyActor`))

(fn `UserConstructionScript`
  (`parent.UserConstructionScript`))