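; Guard Up buff skill for the turn-based JRPG battle system, which applies the Protect buff from the DT_Buffs data table.
; UseSkill briefly switches the current attacking unit's enemy skill animation enum, then changes it again after a short delay.
; It then applies the buff by ID with that unit as caster, prints a debug string and signals that the skill was used.
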(event `/Game/TurnBasedJRPGTemplate/Blueprints/Skills/BP_SkillBase.UseSkill`
  (bind _currentattackingunit (`/Game/TurnBasedJRPGTemplate/Blueprints/Battle/BP_BattleController.currentAttackingUnit` (`self.battleController`)))
  ;[1 1 1] Applies Particle Effect
  (set `/Game/TurnBasedJRPGTemplate/Blueprints/Units/BP_UnitBase.E_EnemySkillsAttackAnimations` "NewEnumerator11" _currentattackingunit)
  (`KismetSystemLibrary.Delay` 0.2)
  (set `/Game/TurnBasedJRPGTemplate/Blueprints/Units/BP_UnitBase.E_EnemySkillsAttackAnimations` "NewEnumerator4" _currentattackingunit)
  (`ReditusTableBuffLibrary.ApplyBuffByID` (`/Game/TurnBasedJRPGTemplate/Blueprints/Battle/BP_BattleController.currentAttackingUnit` (`self.battleController`)) "/Game/TurnBasedJRPGTemplate/Blueprints/DataTable/DT_Buffs.DT_Buffs" "Protect")
  (`KismetSystemLibrary.PrintString` "apply buff")
  (`self.OnSkillUsed`))

(fn `UserConstructionScript`
  (`parent.UserConstructionScript`))