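; BP_TableBuffSkill is a turn-based battle skill that applies temporary buffs to the units selected by its skill type.
; UseSkill briefly pulses IsUsingItem on the attacking unit, resolves targets through SkillTypeFunction, applies non-permanent buffs and signals that the skill is used.
; An unconnected chain holds an attack animation switch, lightning particle and sound, so that effect never plays.
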(event `/Game/TurnBasedJRPGTemplate/Blueprints/Skills/BP_SkillBase.UseSkill`
  (bind _currentattackingunit (`/Game/TurnBasedJRPGTemplate/Blueprints/Battle/BP_BattleController.currentAttackingUnit` (`self.battleController`)))
  ;[1 1 1] Applies Particle Effect
  (set `/Game/TurnBasedJRPGTemplate/Blueprints/Units/BP_UnitBase.IsUsingItem` true _currentattackingunit)
  (`KismetSystemLibrary.Delay` 0.1)
  (set `/Game/TurnBasedJRPGTemplate/Blueprints/Units/BP_UnitBase.IsUsingItem` false _currentattackingunit)
  (bind _resolvedtargetsresult (`self.SkillTypeFunction` (`self.skillType`)))
  (`self.ApplyBuffs` _resolvedtargetsresult)
  (`self.OnSkillUsed`))

(fn `UserConstructionScript`
  (`parent.UserConstructionScript`))