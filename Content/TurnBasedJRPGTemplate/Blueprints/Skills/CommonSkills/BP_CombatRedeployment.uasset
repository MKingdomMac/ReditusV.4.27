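; BP_CombatRedeployment is a turn-based combat skill that applies buffs to the current target unit and flags the BattleController to reset its index.
; UseSkill plays a power-up sound and briefly shows an exclamation-mark emitter on the attacking unit's status socket.
; It then sets ResetIndex, applies the buffs and, after a delay, signals that the skill is used.
; Disconnected leftover nodes hold an unused self-targeting buff variant.
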(event `/Game/TurnBasedJRPGTemplate/Blueprints/Skills/BP_SkillBase.UseSkill`
  (bind _battlecontroller (`self.battleController`))
  ;[1 1 1] Applies Particle Effect
  (`GameplayStatics.PlaySound2D` "/Game/Sounds/Se/Powerup.Powerup_0" 1.0 1.0 0.0 null null)
  (bind _returnvalue (`GameplayStatics.SpawnEmitterAttached` "/Game/Particles/GoodParticleStatus/Particles/Head_Status/PS_GPS_ExclamationMark.PS_GPS_ExclamationMark" (`/Game/TurnBasedJRPGTemplate/Blueprints/Units/BP_UnitBase.Pixel2D` (`/Game/TurnBasedJRPGTemplate/Blueprints/Battle/BP_BattleController.currentAttackingUnit` _battlecontroller)) "StatusSocket"))
  (`KismetSystemLibrary.Delay` 0.5)
  (`ActorComponent.Deactivate` _returnvalue)
  (set `/Game/TurnBasedJRPGTemplate/Blueprints/Battle/BP_BattleController.ResetIndex` true _battlecontroller)
  (`self.ApplyBuffs` (`|MakeArray` (`/Game/TurnBasedJRPGTemplate/Blueprints/Battle/BP_BattleController.currentTargetUnit` _battlecontroller)))
  (`KismetSystemLibrary.Delay` 1.0)
  (`self.OnSkillUsed`))

(fn `UserConstructionScript`
  (`parent.UserConstructionScript`))