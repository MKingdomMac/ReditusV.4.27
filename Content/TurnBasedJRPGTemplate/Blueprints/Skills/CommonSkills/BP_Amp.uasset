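; BP_Amp is a common skill in the turn-based JRPG template that buffs the unit using it.
; On UseSkill it makes the attacking unit the current target, attaches a power-up particle to its Pixel2D component, applies buffs and plays a sound.
; After a short fixed delay it calls OnSkillUsed to signal that the skill has finished.
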(event `/Game/TurnBasedJRPGTemplate/Blueprints/Skills/BP_SkillBase.UseSkill`
  (bind _battlecontroller (`self.battleController`))
  ;[1 1 1] Applies Particle Effect
  (set `/Game/TurnBasedJRPGTemplate/Blueprints/Battle/BP_BattleController.currentTargetUnit` (`/Game/TurnBasedJRPGTemplate/Blueprints/Battle/BP_BattleController.currentAttackingUnit` _battlecontroller) _battlecontroller)
  (`GameplayStatics.SpawnEmitterAttached` "/Game/Particles/GoodParticleStatus/Particles/Buff_Status/PS_GPS_Buff_PowerUp.PS_GPS_Buff_PowerUp" (`/Game/TurnBasedJRPGTemplate/Blueprints/Units/BP_UnitBase.Pixel2D` (`/Game/TurnBasedJRPGTemplate/Blueprints/Battle/BP_BattleController.currentTargetUnit` _battlecontroller)))
  (`self.ApplyBuffs` (`|MakeArray` (`/Game/TurnBasedJRPGTemplate/Blueprints/Battle/BP_BattleController.currentTargetUnit` (`self.battleController`))))
  (`GameplayStatics.PlaySound2D` "/Game/Sounds/Se/Powerup.Powerup_0" 1.0 1.0 0.0 null null)
  (`KismetSystemLibrary.Delay` 1.5)
  (`self.OnSkillUsed`))

(fn `UserConstructionScript`
  (`parent.UserConstructionScript`))