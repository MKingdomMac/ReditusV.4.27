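; BP_Protect is a common turn-based battle skill that applies its buffs to the current target unit.
; UseSkill briefly switches the attacking unit's skill animation enum, then attaches a lightning particle emitter to the target's Pixel2D component and plays a sound.
; After a fixed delay it deactivates the emitter, calls ApplyBuffs on the target and signals that the skill is used.
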(event `/Game/TurnBasedJRPGTemplate/Blueprints/Skills/BP_SkillBase.UseSkill`
  (bind _currentattackingunit (`/Game/TurnBasedJRPGTemplate/Blueprints/Battle/BP_BattleController.currentAttackingUnit` (`self.battleController`)))
  ;[1 1 1] Applies Particle Effect
  (set `/Game/TurnBasedJRPGTemplate/Blueprints/Units/BP_UnitBase.E_EnemySkillsAttackAnimations` "NewEnumerator11" _currentattackingunit)
  (`KismetSystemLibrary.Delay` 0.2)
  (set `/Game/TurnBasedJRPGTemplate/Blueprints/Units/BP_UnitBase.E_EnemySkillsAttackAnimations` "NewEnumerator4" _currentattackingunit)
  (bind _returnvalue (`GameplayStatics.SpawnEmitterAttached` "/Game/Particles/InfinityBladeEffects/Effects/FX_Combat_Lightning/P_DOT_Lightning_01.P_DOT_Lightning_01" (`/Game/TurnBasedJRPGTemplate/Blueprints/Units/BP_UnitBase.Pixel2D` (`/Game/TurnBasedJRPGTemplate/Blueprints/Battle/BP_BattleController.currentTargetUnit` (`self.battleController`)))))
  (`GameplayStatics.PlaySound2D` "/Game/Sounds/Se/Neon.Neon_0" 1.0 1.0 0.0 null null)
  (`KismetSystemLibrary.Delay` 1.5)
  (`ActorComponent.Deactivate` _returnvalue)
  (`self.ApplyBuffs` (`|MakeArray` (`/Game/TurnBasedJRPGTemplate/Blueprints/Battle/BP_BattleController.currentTargetUnit` (`self.battleController`))))
  (`self.OnSkillUsed`))

(fn `UserConstructionScript`
  (`parent.UserConstructionScript`))