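; Buff Blueprint in the turn-based JRPG template that applies a Blind status to its target unit, named for Augustus's Overdrive skill.
; On apply it sets IsBlind on the target, updates the unit's status particle and fires its buff-begins callback; on end it reverses all three.
; For player units, both events also write IsBlinded into the player controller's PlayerUnitDataID map, keyed by CharacterID.
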(event `self.ApplyBuff`
  (bind _targetunit (`self.targetUnit`))
  (bind _asbp_player_unit_base (cast `/Game/TurnBasedJRPGTemplate/Blueprints/Units/PlayerUnits/BP_PlayerUnitBase` _targetunit :!pure true))
  (bind _characterid (`/Game/TurnBasedJRPGTemplate/Blueprints/Units/PlayerUnits/BP_PlayerUnitBase.CharacterID` _asbp_player_unit_base))
  (bind _playerunitdataid (`/Game/TurnBasedJRPGTemplate/Blueprints/Controllers/BP_JRPGPlayerController.PlayerUnitDataID` (cast `/Game/TurnBasedJRPGTemplate/Blueprints/Controllers/BP_JRPGPlayerController` (`GameplayStatics.GetPlayerController` 0) :!pure true)))
  (bind _output_get (set `/Game/TurnBasedJRPGTemplate/Blueprints/Units/BP_UnitBase.Is Blind?` true _targetunit))
  (`KismetSystemLibrary.PrintString` "blinded")
  (if _output_get
    (`/Game/Particles/GoodParticleStatus/Blueprint/BP_GoodParticleStatus.GoodParticleStatus Update` (`/Game/TurnBasedJRPGTemplate/Blueprints/Units/BP_UnitBase.BP_GoodParticleStatus` _targetunit) "NewEnumerator19")
    (`/Game/TurnBasedJRPGTemplate/Blueprints/Units/BP_UnitBase.OnBuffBegins` _targetunit false false false false false false false false false true false false)
    (`/Engine/EditorBlueprintResources/StandardMacros.IsValid` _asbp_player_unit_base
      (:`Is Valid`
        (bind _structout (setmembers `/Game/TurnBasedJRPGTemplate/Blueprints/Structs/S_PlayerUnitData` :`StructRef` (`BlueprintMapLibrary.Map_Find` _playerunitdataid _characterid) :`IsBlinded` true))
        (`BlueprintMapLibrary.Map_Add` _playerunitdataid _characterid _structout)))))

(event `self.OnBuffEnded`
  (bind _targetunit (`self.targetUnit`))
  (bind _asbp_player_unit_base (cast `/Game/TurnBasedJRPGTemplate/Blueprints/Units/PlayerUnits/BP_PlayerUnitBase` _targetunit :!pure true))
  (bind _characterid (`/Game/TurnBasedJRPGTemplate/Blueprints/Units/PlayerUnits/BP_PlayerUnitBase.CharacterID` _asbp_player_unit_base))
  (bind _playerunitdataid (`/Game/TurnBasedJRPGTemplate/Blueprints/Controllers/BP_JRPGPlayerController.PlayerUnitDataID` (cast `/Game/TurnBasedJRPGTemplate/Blueprints/Controllers/BP_JRPGPlayerController` (`GameplayStatics.GetPlayerController` 0) :!pure true)))
  (set `/Game/TurnBasedJRPGTemplate/Blueprints/Units/BP_UnitBase.Is Blind?` false (`self.targetUnit`))
  (`/Game/Particles/GoodParticleStatus/Blueprint/BP_GoodParticleStatus.GoodParticleStatus Update` (`/Game/TurnBasedJRPGTemplate/Blueprints/Units/BP_UnitBase.BP_GoodParticleStatus` _targetunit) "NewEnumerator2")
  (`/Game/TurnBasedJRPGTemplate/Blueprints/Units/BP_UnitBase.OnBuffEnded` _targetunit false false false false false false false false false false false)
  (`/Engine/EditorBlueprintResources/StandardMacros.IsValid` _asbp_player_unit_base
    (:`Is Valid`
      (bind _structout (setmembers `/Game/TurnBasedJRPGTemplate/Blueprints/Structs/S_PlayerUnitData` :`StructRef` (`BlueprintMapLibrary.Map_Find` _playerunitdataid _characterid) :`IsBlinded` false))
      (`BlueprintMapLibrary.Map_Add` _playerunitdataid _characterid _structout))))

(fn `UserConstructionScript`
  (`parent.UserConstructionScript`))