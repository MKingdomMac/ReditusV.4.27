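; BP_RobotOnlyStun is a stun buff for the turn-based JRPG template; nothing here enforces the robot-only restriction its name implies.
; On apply, it flags the target unit as stunned, caches its Speed, overrides it with a fixed value and updates the unit's status particle.
; When the buff ends, it clears the flag, restores the cached Speed and switches the particle state, debug-printing Speed both times.
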(event `self.ApplyBuff`
  (bind _targetunit (`self.targetUnit`))
  (bind _output_get (set `/Game/TurnBasedJRPGTemplate/Blueprints/Units/BP_UnitBase.isStun` true _targetunit))
  (if _output_get
    (set `self.Default Speed` (`/Game/TurnBasedJRPGTemplate/Blueprints/Units/BP_UnitBase.speed` _targetunit))
    (bind _output_get_2 (set `/Game/TurnBasedJRPGTemplate/Blueprints/Units/BP_UnitBase.speed` 10 _targetunit))
    (`KismetSystemLibrary.PrintString` (`KismetStringLibrary.Conv_IntToString` _output_get_2))
    (`/Game/Particles/GoodParticleStatus/Blueprint/BP_GoodParticleStatus.GoodParticleStatus Update` (`/Game/TurnBasedJRPGTemplate/Blueprints/Units/BP_UnitBase.BP_GoodParticleStatus` _targetunit) "NewEnumerator4")))

(event `self.OnBuffEnded`
  (bind _targetunit (`self.targetUnit`))
  (set `/Game/TurnBasedJRPGTemplate/Blueprints/Units/BP_UnitBase.isStun` false _targetunit)
  (bind _output_get (set `/Game/TurnBasedJRPGTemplate/Blueprints/Units/BP_UnitBase.speed` (`self.Default Speed`) _targetunit))
  (`KismetSystemLibrary.PrintString` (`KismetStringLibrary.Conv_IntToString` _output_get))
  (`/Game/Particles/GoodParticleStatus/Blueprint/BP_GoodParticleStatus.GoodParticleStatus Update` (`/Game/TurnBasedJRPGTemplate/Blueprints/Units/BP_UnitBase.BP_GoodParticleStatus` _targetunit) "NewEnumerator2"))

(fn `UserConstructionScript`
  (`parent.UserConstructionScript`))