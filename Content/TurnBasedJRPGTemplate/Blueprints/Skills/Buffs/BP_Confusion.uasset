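; BP_Confusion is a turn-based JRPG skill buff that puts its target unit into the confused state.
; On apply, it fires the unit's buff-begin notification only if not already confused, then sets IsConfused, prints a debug message and updates the unit's status particle component.
; On end, it clears the flag, fires the buff-ended notification and switches the status particle to another state.
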(event `self.ApplyBuff`
  (bind _targetunit (`self.targetUnit`))
  (`|ExecutionSequence`
    (:`then_0`
      (if (not (`/Game/TurnBasedJRPGTemplate/Blueprints/Units/BP_UnitBase.Is Confused` _targetunit))
        (`/Game/TurnBasedJRPGTemplate/Blueprints/Units/BP_UnitBase.OnBuffBegins` _targetunit true false false false false false false false false false false false)))
    (:`then_1`
      (bind _output_get (set `/Game/TurnBasedJRPGTemplate/Blueprints/Units/BP_UnitBase.Is Confused` true _targetunit))
      (if _output_get
        (`KismetSystemLibrary.PrintString` "is confused now")
        (`/Game/Particles/GoodParticleStatus/Blueprint/BP_GoodParticleStatus.GoodParticleStatus Update` (`/Game/TurnBasedJRPGTemplate/Blueprints/Units/BP_UnitBase.BP_GoodParticleStatus` _targetunit) "NewEnumerator6")))))

(event `self.OnBuffEnded`
  (bind _targetunit (`self.targetUnit`))
  (set `/Game/TurnBasedJRPGTemplate/Blueprints/Units/BP_UnitBase.Is Confused` false (`self.targetUnit`))
  (`/Game/TurnBasedJRPGTemplate/Blueprints/Units/BP_UnitBase.OnBuffEnded` _targetunit true false false false false false false false false false false)
  (`/Game/Particles/GoodParticleStatus/Blueprint/BP_GoodParticleStatus.GoodParticleStatus Update` (`/Game/TurnBasedJRPGTemplate/Blueprints/Units/BP_UnitBase.BP_GoodParticleStatus` _targetunit) "NewEnumerator2"))

(fn `UserConstructionScript`
  (`parent.UserConstructionScript`))