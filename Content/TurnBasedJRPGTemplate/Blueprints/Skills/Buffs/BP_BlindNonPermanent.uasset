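; Non-permanent blind status buff for the turn-based JRPG battle system, applied to a target unit.
; On apply it fires the unit's buff-begin callback if not already blinded, sets IsBlind, prints a debug message and updates the unit's status particle.
; When the buff ends it clears IsBlind, fires the buff-end callback and switches the particle.
; Disconnected nodes for saving blindness into player unit data never run.
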(event `self.ApplyBuff`
  (bind _targetunit (`self.targetUnit`))
  (`|ExecutionSequence`
    (:`then_0`
      (if (not (`/Game/TurnBasedJRPGTemplate/Blueprints/Units/BP_UnitBase.Is Blind?` _targetunit))
        (`/Game/TurnBasedJRPGTemplate/Blueprints/Units/BP_UnitBase.OnBuffBegins` _targetunit false false false false false false false false false true false false)))
    (:`then_1`
      (bind _output_get (set `/Game/TurnBasedJRPGTemplate/Blueprints/Units/BP_UnitBase.Is Blind?` true _targetunit))
      (`KismetSystemLibrary.PrintString` "blinded")
      (if _output_get
        (`/Game/Particles/GoodParticleStatus/Blueprint/BP_GoodParticleStatus.GoodParticleStatus Update` (`/Game/TurnBasedJRPGTemplate/Blueprints/Units/BP_UnitBase.BP_GoodParticleStatus` _targetunit) "NewEnumerator19")))))

(event `self.OnBuffEnded`
  (bind _targetunit (`self.targetUnit`))
  (set `/Game/TurnBasedJRPGTemplate/Blueprints/Units/BP_UnitBase.Is Blind?` false (`self.targetUnit`))
  (`/Game/TurnBasedJRPGTemplate/Blueprints/Units/BP_UnitBase.OnBuffEnded` _targetunit false false false false false false false false false false false)
  (`/Game/Particles/GoodParticleStatus/Blueprint/BP_GoodParticleStatus.GoodParticleStatus Update` (`/Game/TurnBasedJRPGTemplate/Blueprints/Units/BP_UnitBase.BP_GoodParticleStatus` _targetunit) "NewEnumerator2"))

(fn `UserConstructionScript`
  (`parent.UserConstructionScript`))