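; BP_Staggered is a turn-based battle buff that puts its target unit into a staggered, stunned state.
; On apply it sets the stun flag, saves and overrides the unit's Speed, plays an attached particle and break sound, and updates the unit's status particle.
; When the buff ends it clears the stun, restores Speed, switches the status particle and sets current stamina from the unit's UnitChangesWeakness value.
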(event `self.ApplyBuff`
  (bind _targetunit (`self.targetUnit`))
  (bind _output_get (set `/Game/TurnBasedJRPGTemplate/Blueprints/Units/BP_UnitBase.isStun` true _targetunit))
  (if _output_get
    (set `self.Default Speed` (`/Game/TurnBasedJRPGTemplate/Blueprints/Units/BP_UnitBase.speed` _targetunit))
    (set `/Game/TurnBasedJRPGTemplate/Blueprints/Units/BP_UnitBase.speed` 10 _targetunit)
    (`GameplayStatics.SpawnEmitterAttached` "/Game/Particles/AdvancedMagicFX13/Particles/P_ky_gaither.P_ky_gaither" (`/Game/TurnBasedJRPGTemplate/Blueprints/Units/BP_UnitBase.Pixel2D` _targetunit))
    (`GameplayStatics.PlaySoundAtLocation` "/Game/Sounds/Se/Break.Break_0" (0.0 0.0 0.0) (struct) 3.0 1.0 0.0 null null null)
    (`/Game/Particles/GoodParticleStatus/Blueprint/BP_GoodParticleStatus.GoodParticleStatus Update` (`/Game/TurnBasedJRPGTemplate/Blueprints/Units/BP_UnitBase.BP_GoodParticleStatus` _targetunit) "NewEnumerator4")))

(event `self.OnBuffEnded`
  (bind _targetunit (`self.targetUnit`))
  (bind _targetunit_2 (`self.targetUnit`))
  (set `/Game/TurnBasedJRPGTemplate/Blueprints/Units/BP_UnitBase.isStun` false (`self.targetUnit`))
  (set `/Game/TurnBasedJRPGTemplate/Blueprints/Units/BP_UnitBase.speed` (`self.Default Speed`) _targetunit)
  (`/Game/Particles/GoodParticleStatus/Blueprint/BP_GoodParticleStatus.GoodParticleStatus Update` (`/Game/TurnBasedJRPGTemplate/Blueprints/Units/BP_UnitBase.BP_GoodParticleStatus` _targetunit) "NewEnumerator2")
  (`/Game/TurnBasedJRPGTemplate/Blueprints/Units/BP_UnitBase.SetCurrentStamina` _targetunit_2 (`/Game/TurnBasedJRPGTemplate/Blueprints/Units/BP_UnitBase.UnitChangesWeakness` _targetunit_2)))

(fn `UserConstructionScript`
  (`parent.UserConstructionScript`))