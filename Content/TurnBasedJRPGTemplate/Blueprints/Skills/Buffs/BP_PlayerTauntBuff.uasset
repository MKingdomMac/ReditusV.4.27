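; Taunt buff for the turn-based JRPG battle system that marks a unit as taunted by the attacking unit.
; Applying it flags TargetUnit as taunted and sets the battle controller's current target's TauntedTarget to the current attacker.
; When it ends, it clears the flag, then after a short delay updates the good-status particle on whichever unit is attacking at that moment.
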(event `self.ApplyBuff`
  (bind _battlecontroller (`self.battleController`))
  (set `/Game/TurnBasedJRPGTemplate/Blueprints/Units/BP_UnitBase.IsTaunted` true (`self.targetUnit`))
  (set `/Game/TurnBasedJRPGTemplate/Blueprints/Units/BP_UnitBase.TauntedTarget` (`/Game/TurnBasedJRPGTemplate/Blueprints/Battle/BP_BattleController.currentAttackingUnit` _battlecontroller) (`/Game/TurnBasedJRPGTemplate/Blueprints/Battle/BP_BattleController.currentTargetUnit` _battlecontroller)))

(event `self.OnBuffEnded`
  (set `/Game/TurnBasedJRPGTemplate/Blueprints/Units/BP_UnitBase.IsTaunted` false (`self.targetUnit`))
  (`KismetSystemLibrary.Delay` 1.0)
  (`/Game/Particles/GoodParticleStatus/Blueprint/BP_GoodParticleStatus.GoodParticleStatus Update` (`/Game/TurnBasedJRPGTemplate/Blueprints/Units/BP_UnitBase.BP_GoodParticleStatus` (`/Game/TurnBasedJRPGTemplate/Blueprints/Battle/BP_BattleController.currentAttackingUnit` (`self.battleController`))) "NewEnumerator2"))

(fn `UserConstructionScript`
  (`parent.UserConstructionScript`))