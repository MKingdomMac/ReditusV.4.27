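; BP_CritIncrease is a skill buff for the turn-based JRPG template that temporarily changes the target unit's critical stat.
; ApplyBuff caches the unit's current Critical in DefaultCrit, then overwrites it with a hard-coded value rather than adding to it.
; OnBuffEnded writes the cached value back.
; BeginPlay calls the parent and prints a leftover-style debug string.
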(event `self.ReceiveBeginPlay`
  (`parent.ReceiveBeginPlay`)
  (`KismetSystemLibrary.PrintString` "Hello"))

(event `self.ApplyBuff`
  ;[1 1 1] Increases units critical hit
  (set `self.DefaultCrit` (`/Game/TurnBasedJRPGTemplate/Blueprints/Units/BP_UnitBase.Critical` (`self.targetUnit`)))
  (set `/Game/TurnBasedJRPGTemplate/Blueprints/Units/BP_UnitBase.Critical` 50.0 (`self.targetUnit`)))

(event `self.OnBuffEnded`
  ;[1 1 1] Increases units critical hit
  (set `/Game/TurnBasedJRPGTemplate/Blueprints/Units/BP_UnitBase.Critical` (`self.DefaultCrit`) (`self.targetUnit`)))

(fn `UserConstructionScript`
  (`parent.UserConstructionScript`))