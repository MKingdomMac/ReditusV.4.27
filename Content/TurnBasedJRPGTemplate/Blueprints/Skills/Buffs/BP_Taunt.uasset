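; BP_Taunt is a skill buff for turn-based battles that marks its target unit as taunted.
; On apply, it sets the unit's IsTaunted flag and stores the battle controller's current target unit as TauntedTarget.
; When the buff ends, it clears the flag but leaves TauntedTarget set.
; Its status particle update calls are disconnected, so it triggers no visual change itself.
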(event `self.ApplyBuff`
  (bind _targetunit (`self.targetUnit`))
  (set `/Game/TurnBasedJRPGTemplate/Blueprints/Units/BP_UnitBase.IsTaunted` true _targetunit)
  (set `/Game/TurnBasedJRPGTemplate/Blueprints/Units/BP_UnitBase.TauntedTarget` (`/Game/TurnBasedJRPGTemplate/Blueprints/Battle/BP_BattleController.currentTargetUnit` (`self.battleController`)) _targetunit))

(event `self.OnBuffEnded`
  (set `/Game/TurnBasedJRPGTemplate/Blueprints/Units/BP_UnitBase.IsTaunted` false (`self.targetUnit`)))

(fn `UserConstructionScript`
  (`parent.UserConstructionScript`))