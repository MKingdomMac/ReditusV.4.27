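; BP_Swallow is a buff for the turn-based JRPG battle system that takes a swallowed unit out of action.
; Applying it stuns the target and stores it as the BattleController's SwallowedUnit.
; When it ends, it clears the stun, unhides the target and sends the swallowed unit jumping back to its start location.
; It then sets TargetUnit to a random player unit and calls the controller's DealDamage.
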(event `self.ApplyBuff`
  (bind _targetunit (`self.targetUnit`))
  (set `/Game/TurnBasedJRPGTemplate/Blueprints/Units/BP_UnitBase.isStun` true _targetunit)
  (set `/Game/TurnBasedJRPGTemplate/Blueprints/Battle/BP_BattleController.SwallowedUnit` _targetunit (`self.battleController`)))

(event `self.OnBuffEnded`
  (bind _targetunit (`self.targetUnit`))
  (bind _battlecontroller (`self.battleController`))
  (bind _swallowedunit (`/Game/TurnBasedJRPGTemplate/Blueprints/Battle/BP_BattleController.SwallowedUnit` (`self.battleController`)))
  (bind _playerunits (`/Game/TurnBasedJRPGTemplate/Blueprints/Battle/BP_BattleBase.playerUnits` (`/Game/TurnBasedJRPGTemplate/Blueprints/Battle/BP_BattleController.currentBattle` _battlecontroller)))
  (set `/Game/TurnBasedJRPGTemplate/Blueprints/Units/BP_UnitBase.isStun` false _targetunit)
  (`self.SetActorHiddenInGame` _targetunit false)
  (`/Game/TurnBasedJRPGTemplate/Blueprints/Units/BP_UnitBase.MoveToTarget` _swallowedunit (`/Game/TurnBasedJRPGTemplate/Blueprints/Units/BP_UnitBase.startLocation` _swallowedunit) false true)
  (set `self.targetUnit` (`|GetArrayItem` _playerunits (`KismetMathLibrary.RandomIntegerInRange` 0 (`KismetArrayLibrary.Array_LastIndex` _playerunits))))
  (`/Game/TurnBasedJRPGTemplate/Blueprints/Battle/BP_BattleController.DealDamage` _battlecontroller 0 1.0 0.0))

(fn `UserConstructionScript`
  (`parent.UserConstructionScript`))