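; BP_HitIncrease is a skill buff for the turn-based JRPG template that temporarily raises the target unit's Hit stat by a fixed amount.
; ApplyBuff announces the buff if not already active, sets the HitIncrease flag, caches Hit and adds the bonus.
; OnBuffEnded clears the flag, restores the cached value and notifies the unit.
; Only the begin notification checks the flag, so the caching and bonus run on every application.
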(event `self.ApplyBuff`
  (bind _targetunit (`self.targetUnit`))
  ;[1 1 1] Increases units critical hit
  (`|ExecutionSequence`
    (:`then_0`
      (if (not (`/Game/TurnBasedJRPGTemplate/Blueprints/Units/BP_UnitBase.HitIncrease` _targetunit))
        (`/Game/TurnBasedJRPGTemplate/Blueprints/Units/BP_UnitBase.OnBuffBegins` _targetunit false false false false false false false false false false true false)))
    (:`then_1`
      (set `/Game/TurnBasedJRPGTemplate/Blueprints/Units/BP_UnitBase.HitIncrease` true _targetunit)
      (set `self.DefaultHit` (`/Game/TurnBasedJRPGTemplate/Blueprints/Units/BP_UnitBase.hit` _targetunit))
      (bind _output_get (set `/Game/TurnBasedJRPGTemplate/Blueprints/Units/BP_UnitBase.hit` (+ (`/Game/TurnBasedJRPGTemplate/Blueprints/Units/BP_UnitBase.hit` _targetunit) 10) _targetunit)))))

(event `self.OnBuffEnded`
  (bind _targetunit (`self.targetUnit`))
  ;[1 1 1] Increases units critical hit
  (set `/Game/TurnBasedJRPGTemplate/Blueprints/Units/BP_UnitBase.HitIncrease` false _targetunit)
  (set `/Game/TurnBasedJRPGTemplate/Blueprints/Units/BP_UnitBase.hit` (`self.DefaultHit`) _targetunit)
  (`/Game/TurnBasedJRPGTemplate/Blueprints/Units/BP_UnitBase.OnBuffEnded` _targetunit false false false false false false false false false true false))

(fn `UserConstructionScript`
  (`parent.UserConstructionScript`))