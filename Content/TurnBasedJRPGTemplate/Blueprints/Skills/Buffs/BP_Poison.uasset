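; BP_Poison is a JRPG buff that applies the poisoned damage-over-time state to a target unit and saves it.
; ApplyBuff sets IsDOT, firing the unit's buff-begin call only if not already set, and OnBuffEnded reverses it.
; Both write the PoisonDamage flag into the player controller's PlayerUnitDataID map by CharacterID, casting the target to BP_PlayerUnitBase.
; The file holds no damage logic, and BeginPlay prints a debug string.
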(event `self.ReceiveBeginPlay`
  (`parent.ReceiveBeginPlay`)
  (`KismetSystemLibrary.PrintString` "Hello"))

(event `self.ApplyBuff`
  (bind _targetunit (`self.targetUnit`))
  (bind _playerunitdataid (`/Game/TurnBasedJRPGTemplate/Blueprints/Controllers/BP_JRPGPlayerController.PlayerUnitDataID` (cast `/Game/TurnBasedJRPGTemplate/Blueprints/Controllers/BP_JRPGPlayerController` (`GameplayStatics.GetPlayerController` 0) :!pure true)))
  (bind _characterid (`/Game/TurnBasedJRPGTemplate/Blueprints/Units/PlayerUnits/BP_PlayerUnitBase.CharacterID` (cast `/Game/TurnBasedJRPGTemplate/Blueprints/Units/PlayerUnits/BP_PlayerUnitBase` _targetunit :!pure true)))
  ;[1 1 1] Inside the BP_Poison, it apply and save the "poisoned state"
  (`|ExecutionSequence`
    (:`then_0`
      (if (not (`/Game/TurnBasedJRPGTemplate/Blueprints/Units/BP_UnitBase.Is DOT` _targetunit))
        (`/Game/TurnBasedJRPGTemplate/Blueprints/Units/BP_UnitBase.OnBuffBegins` _targetunit false false true false false false false false false false false false)))
    (:`then_1`
      (set `/Game/TurnBasedJRPGTemplate/Blueprints/Units/BP_UnitBase.Is DOT` true _targetunit)
      (bind _structout (setmembers `/Game/TurnBasedJRPGTemplate/Blueprints/Structs/S_PlayerUnitData` :`StructRef` (`BlueprintMapLibrary.Map_Find` _playerunitdataid _characterid) :`PoisonDamage` true))
      (`BlueprintMapLibrary.Map_Add` _playerunitdataid _characterid _structout))))

(event `self.OnBuffEnded`
  (bind _targetunit (`self.targetUnit`))
  (bind _playerunitdataid (`/Game/TurnBasedJRPGTemplate/Blueprints/Controllers/BP_JRPGPlayerController.PlayerUnitDataID` (cast `/Game/TurnBasedJRPGTemplate/Blueprints/Controllers/BP_JRPGPlayerController` (`GameplayStatics.GetPlayerController` 0) :!pure true)))
  (bind _characterid (`/Game/TurnBasedJRPGTemplate/Blueprints/Units/PlayerUnits/BP_PlayerUnitBase.CharacterID` (cast `/Game/TurnBasedJRPGTemplate/Blueprints/Units/PlayerUnits/BP_PlayerUnitBase` _targetunit :!pure true)))
  ;[1 1 1] Inside the BP_Poison, it apply and save the "poisoned state"
  (set `/Game/TurnBasedJRPGTemplate/Blueprints/Units/BP_UnitBase.Is DOT` false _targetunit)
  (`/Game/TurnBasedJRPGTemplate/Blueprints/Units/BP_UnitBase.OnBuffEnded` _targetunit false false false false false false false false false false false)
  (bind _structout (setmembers `/Game/TurnBasedJRPGTemplate/Blueprints/Structs/S_PlayerUnitData` :`StructRef` (`BlueprintMapLibrary.Map_Find` _playerunitdataid _characterid) :`PoisonDamage` false))
  (`BlueprintMapLibrary.Map_Add` _playerunitdataid _characterid _structout))

(fn `UserConstructionScript`
  (`parent.UserConstructionScript`))