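; BP_Flee is a turn-based battle buff that makes the thief enemy, the battle controller's TheftUnit, escape when the buff ends.
; Applying it does nothing; on expiry it ends that unit's turn, removes it from the battle's unit lists, plays mist and wind effects, and destroys the actor.
; If no enemy units remain afterward, it signals that the battle is over.
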(event `self.ApplyBuff`)

(event `self.OnBuffEnded`
  (bind _battlecontroller (`self.battleController`))
  (bind _currentbattle (`/Game/TurnBasedJRPGTemplate/Blueprints/Battle/BP_BattleController.currentBattle` _battlecontroller))
  (bind _theftunit (`/Game/TurnBasedJRPGTemplate/Blueprints/Battle/BP_BattleController.TheftUnit` _battlecontroller))
  (bind _currentbattle_2 (`/Game/TurnBasedJRPGTemplate/Blueprints/Battle/BP_BattleController.currentBattle` _battlecontroller))
  (`/Game/TurnBasedJRPGTemplate/Blueprints/Units/BP_UnitBase.EndTurn` _theftunit)
  (`KismetArrayLibrary.Array_RemoveItem` (`/Game/TurnBasedJRPGTemplate/Blueprints/Battle/BP_BattleBase.AllUnits` _currentbattle_2) _theftunit)
  (`KismetArrayLibrary.Array_RemoveItem` (`/Game/TurnBasedJRPGTemplate/Blueprints/Battle/BP_BattleBase.enemyUnits` _currentbattle_2) (cast `/Game/TurnBasedJRPGTemplate/Blueprints/Units/EnemyUnits/BP_EnemyUnitBase` _theftunit :!pure true))
  (`NiagaraFunctionLibrary.SpawnSystemAtLocation` "/Game/Particles/sA_PosionSkills_1/Fx/NS_Gas_Mist_2.NS_Gas_Mist_2" (`self.K2_GetActorLocation` _theftunit))
  (`GameplayStatics.PlaySoundAtLocation` "/Game/Sounds/Se/Wind6.Wind6_0" (0.0 0.0 0.0) (struct) 1.0 1.0 0.0 null null null)
  (`self.K2_DestroyActor` _theftunit)
  (if (== (`KismetArrayLibrary.Array_Length` (`/Game/TurnBasedJRPGTemplate/Blueprints/Battle/BP_BattleBase.enemyUnits` _currentbattle)) 0)
    (`/Game/TurnBasedJRPGTemplate/Blueprints/Battle/BP_BattleBase.OnBattleOver` _currentbattle "NewEnumerator0")))

(fn `UserConstructionScript`
  (`parent.UserConstructionScript`))