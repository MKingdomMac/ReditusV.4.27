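; BP_Sleep is a sleep status effect for units in the turn-based JRPG template, built as a buff.
; Applying it sets IsSleeping on the target unit and updates that unit's BPGoodParticleStatus component to a new status visual.
; When the buff ends, it clears the flag, switches the particle status to another state and prints a debug message.
; Sleep's gameplay consequences and duration are not handled in these graphs.
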(event `self.ApplyBuff`
  (bind _targetunit (`self.targetUnit`))
  (set `/Game/TurnBasedJRPGTemplate/Blueprints/Units/BP_UnitBase.IsSleeping` true _targetunit)
  (`/Game/Particles/GoodParticleStatus/Blueprint/BP_GoodParticleStatus.GoodParticleStatus Update` (`/Game/TurnBasedJRPGTemplate/Blueprints/Units/BP_UnitBase.BP_GoodParticleStatus` _targetunit) "NewEnumerator5"))

(event `self.OnBuffEnded`
  (set `/Game/TurnBasedJRPGTemplate/Blueprints/Units/BP_UnitBase.IsSleeping` false (`self.targetUnit`))
  (`/Game/Particles/GoodParticleStatus/Blueprint/BP_GoodParticleStatus.GoodParticleStatus Update` (`/Game/TurnBasedJRPGTemplate/Blueprints/Units/BP_UnitBase.BP_GoodParticleStatus` (`self.targetUnit`)) "NewEnumerator2")
  (`KismetSystemLibrary.PrintString` "SleepEnded"))

(fn `UserConstructionScript`
  (`parent.UserConstructionScript`))