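; BP_Stun is a status effect for the turn-based JRPG that stuns its target unit.
; ApplyBuff announces a new stun, sets the stun flag, saves the unit's Speed, overrides it with a fixed value and updates its status particle.
; The save repeats on every application, so restacking stores the already overridden Speed.
; OnBuffEnded clears the flag, restores the saved Speed, switches the particle and notifies the unit.
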(event `self.ApplyBuff`
  (bind _targetunit (`self.targetUnit`))
  (`|ExecutionSequence`
    (:`then_0`
      (if (not (`/Game/TurnBasedJRPGTemplate/Blueprints/Units/BP_UnitBase.isStun` _targetunit))
        (`/Game/TurnBasedJRPGTemplate/Blueprints/Units/BP_UnitBase.OnBuffBegins` _targetunit false true false false false false false false false false false false)))
    (:`then_1`
      (bind _output_get (set `/Game/TurnBasedJRPGTemplate/Blueprints/Units/BP_UnitBase.isStun` true _targetunit))
      (if _output_get
        (set `self.Default Speed` (`/Game/TurnBasedJRPGTemplate/Blueprints/Units/BP_UnitBase.speed` _targetunit))
        (set `/Game/TurnBasedJRPGTemplate/Blueprints/Units/BP_UnitBase.speed` 10 _targetunit)
        (`/Game/Particles/GoodParticleStatus/Blueprint/BP_GoodParticleStatus.GoodParticleStatus Update` (`/Game/TurnBasedJRPGTemplate/Blueprints/Units/BP_UnitBase.BP_GoodParticleStatus` _targetunit) "NewEnumerator4")))))

(event `self.OnBuffEnded`
  (bind _targetunit (`self.targetUnit`))
  (set `/Game/TurnBasedJRPGTemplate/Blueprints/Units/BP_UnitBase.isStun` false (`self.targetUnit`))
  (set `/Game/TurnBasedJRPGTemplate/Blueprints/Units/BP_UnitBase.speed` (`self.Default Speed`) _targetunit)
  (`/Game/Particles/GoodParticleStatus/Blueprint/BP_GoodParticleStatus.GoodParticleStatus Update` (`/Game/TurnBasedJRPGTemplate/Blueprints/Units/BP_UnitBase.BP_GoodParticleStatus` _targetunit) "NewEnumerator2")
  (`/Game/TurnBasedJRPGTemplate/Blueprints/Units/BP_UnitBase.OnBuffEnded` _targetunit false true false false false false false false false false false))

(fn `UserConstructionScript`
  (`parent.UserConstructionScript`))