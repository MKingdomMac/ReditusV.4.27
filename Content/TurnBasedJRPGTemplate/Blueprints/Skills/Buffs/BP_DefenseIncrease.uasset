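; Defense buff for the turn-based JRPG template that protects a target unit by raising its Defense by half.
; On apply it caches the original Defense, sets IsProtected and attaches the "Protect" visuals from DT_BuffVisuals to the unit's Pixel2D component.
; Only the buff-begins notification is skipped for already protected units.
; On end it restores the cached Defense, stops the visuals, notifies the unit and clears the flag.
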(event `self.ApplyBuff`
  (bind _targetunit (`self.targetUnit`))
  (bind _targetunit_2 (`self.targetUnit`))
  ;[1 1 1] Inside the BP_Poison, it apply and save the "poisoned state"
  (`|ExecutionSequence`
    (:`then_0`
      (if (not (`/Game/TurnBasedJRPGTemplate/Blueprints/Units/BP_UnitBase.IsProtected` _targetunit_2))
        (`/Game/TurnBasedJRPGTemplate/Blueprints/Units/BP_UnitBase.OnBuffBegins` _targetunit false false false false false false false true false false false false)))
    (:`then_1`
      (bind _output_get (set `self.DefaultDefense` (`/Game/TurnBasedJRPGTemplate/Blueprints/Units/BP_UnitBase.defense` _targetunit_2)))
      (set `/Game/TurnBasedJRPGTemplate/Blueprints/Units/BP_UnitBase.defense` (`KismetMathLibrary.FTrunc` (* _output_get 1.5)) _targetunit)
      (bind _returnvalue (`ReditusBuffVisualLibrary.StartBuffVisuals` self (`/Game/TurnBasedJRPGTemplate/Blueprints/Units/BP_UnitBase.Pixel2D` _targetunit) "/Game/TurnBasedJRPGTemplate/Blueprints/DataTable/DT_BuffVisuals.DT_BuffVisuals" "Protect"))
      (set `self.particle` _returnvalue)
      (set `/Game/TurnBasedJRPGTemplate/Blueprints/Units/BP_UnitBase.IsProtected` true _targetunit))))

(event `self.OnBuffEnded`
  (bind _targetunit (`self.targetUnit`))
  ;[1 1 1] Inside the BP_Poison, it apply and save the "poisoned state"
  (set `/Game/TurnBasedJRPGTemplate/Blueprints/Units/BP_UnitBase.defense` (`self.DefaultDefense`) (`self.targetUnit`))
  (`ReditusBuffVisualLibrary.StopBuffVisuals` self)
  (`KismetSystemLibrary.PrintString` "Deactivated")
  (`/Game/TurnBasedJRPGTemplate/Blueprints/Units/BP_UnitBase.OnBuffEnded` _targetunit false false false false false false false true false false false)
  (set `/Game/TurnBasedJRPGTemplate/Blueprints/Units/BP_UnitBase.IsProtected` false _targetunit))

(fn `UserConstructionScript`
  (`parent.UserConstructionScript`))