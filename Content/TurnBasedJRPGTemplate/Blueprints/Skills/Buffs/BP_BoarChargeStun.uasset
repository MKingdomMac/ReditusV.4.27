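; Stun buff for the turn-based JRPG template, named for the Boar Charge skill, that stuns its target unit.
; On apply, it signals the buff start only if the unit is not already stunned, then sets the stun flag and updates the unit's status particle.
; When the buff ends, it clears the flag, signals the end on the unit and switches the particle status again.
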(event `self.ApplyBuff`
  (bind _targetunit (`self.targetUnit`))
  (`|ExecutionSequence`
    (:`then_0`
      (if (not (`/Game/TurnBasedJRPGTemplate/Blueprints/Units/BP_UnitBase.isStun` _targetunit))
        (`/Game/TurnBasedJRPGTemplate/Blueprints/Units/BP_UnitBase.OnBuffBegins` _targetunit false true false false false false false false false false false false)))
    (:`then_1`
      (bind _output_get (set `/Game/TurnBasedJRPGTemplate/Blueprints/Units/BP_UnitBase.isStun` true _targetunit))
      (if _output_get
        (`/Game/Particles/GoodParticleStatus/Blueprint/BP_GoodParticleStatus.GoodParticleStatus Update` (`/Game/TurnBasedJRPGTemplate/Blueprints/Units/BP_UnitBase.BP_GoodParticleStatus` _targetunit) "NewEnumerator4")))))

(event `self.OnBuffEnded`
  (bind _targetunit (`self.targetUnit`))
  (set `/Game/TurnBasedJRPGTemplate/Blueprints/Units/BP_UnitBase.isStun` false _targetunit)
  (`/Game/TurnBasedJRPGTemplate/Blueprints/Units/BP_UnitBase.OnBuffEnded` _targetunit false true false false false false false false false false false)
  (`/Game/Particles/GoodParticleStatus/Blueprint/BP_GoodParticleStatus.GoodParticleStatus Update` (`/Game/TurnBasedJRPGTemplate/Blueprints/Units/BP_UnitBase.BP_GoodParticleStatus` (`self.targetUnit`)) "NewEnumerator2"))

(fn `UserConstructionScript`
  (`parent.UserConstructionScript`))