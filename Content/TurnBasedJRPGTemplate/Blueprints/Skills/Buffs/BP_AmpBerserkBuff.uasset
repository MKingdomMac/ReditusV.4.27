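; BP_AmpBerserkBuff is a turn-based JRPG skill buff that puts its target unit into a Berserk state.
; On apply it sets the unit's IsBerserk flag, prints a debug string and notifies the unit that the buff began.
; It also switches the unit's good-status particle component to one state, then to another after a short delay.
; When the buff ends it clears the flag and notifies the unit.
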(event `self.ApplyBuff`
  (bind _targetunit (`self.targetUnit`))
  (bind _bp_goodparticlestatus (`/Game/TurnBasedJRPGTemplate/Blueprints/Units/BP_UnitBase.BP_GoodParticleStatus` _targetunit))
  (bind _output_get (set `/Game/TurnBasedJRPGTemplate/Blueprints/Units/BP_UnitBase.IsBerserk??` true _targetunit))
  (`KismetSystemLibrary.PrintString` "Berserk")
  (if _output_get
    (`/Game/TurnBasedJRPGTemplate/Blueprints/Units/BP_UnitBase.OnBuffBegins` _targetunit false false false false true false false false false false false false)
    (`/Game/Particles/GoodParticleStatus/Blueprint/BP_GoodParticleStatus.GoodParticleStatus Update` _bp_goodparticlestatus "NewEnumerator21")
    (`KismetSystemLibrary.Delay` 2.0)
    (`/Game/Particles/GoodParticleStatus/Blueprint/BP_GoodParticleStatus.GoodParticleStatus Update` _bp_goodparticlestatus "NewEnumerator2")))

(event `self.OnBuffEnded`
  (set `/Game/TurnBasedJRPGTemplate/Blueprints/Units/BP_UnitBase.IsBerserk??` false (`self.targetUnit`))
  (`/Game/TurnBasedJRPGTemplate/Blueprints/Units/BP_UnitBase.OnBuffEnded` (`self.targetUnit`) false false false false true false false false false false false))

(fn `UserConstructionScript`
  (`parent.UserConstructionScript`))