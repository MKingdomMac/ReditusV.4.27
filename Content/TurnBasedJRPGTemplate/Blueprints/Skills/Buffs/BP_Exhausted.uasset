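; BP_Exhausted is a turn-based battle debuff that weakens the target unit's defense and attack range while it is exhausted.
; On apply it caches those stats, scales them down and sets the exhausted state, skipping only the begin notification if the unit is protected.
; On end it restores the cached stats, clears amp points, refills exhaustion points and resets the ailment unless a DOT is active.
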(event `self.ApplyBuff`
  (bind _targetunit (`self.targetUnit`))
  (bind _targetunit_2 (`self.targetUnit`))
  (bind _targetunit_3 (`self.targetUnit`))
  ;[1 1 1] Inside the BP_Poison, it apply and save the "poisoned state"
  (`|ExecutionSequence`
    (:`then_0`
      (if (not (`/Game/TurnBasedJRPGTemplate/Blueprints/Units/BP_UnitBase.IsProtected` _targetunit_2))
        (`/Game/TurnBasedJRPGTemplate/Blueprints/Units/BP_UnitBase.OnBuffBegins` _targetunit_3 false false false false false false false false false false false true)))
    (:`then_1`
      (bind _output_get (set `self.DefaultDefense` (`/Game/TurnBasedJRPGTemplate/Blueprints/Units/BP_UnitBase.defense` _targetunit_2)))
      (set `/Game/TurnBasedJRPGTemplate/Blueprints/Units/BP_UnitBase.defense` (`KismetMathLibrary.FTrunc` (* _output_get 0.75)) _targetunit_3)
      (bind _output_get_2 (set `self.DefaultMinAttack` (`/Game/TurnBasedJRPGTemplate/Blueprints/Units/BP_UnitBase.minAttack` _targetunit_3)))
      (set `/Game/TurnBasedJRPGTemplate/Blueprints/Units/BP_UnitBase.minAttack` (`KismetMathLibrary.FTrunc` (* _output_get_2 0.75)) _targetunit_3)
      (bind _output_get_3 (set `self.DefaultMaxAttack` (`/Game/TurnBasedJRPGTemplate/Blueprints/Units/BP_UnitBase.maxAttack` _targetunit_3)))
      (set `/Game/TurnBasedJRPGTemplate/Blueprints/Units/BP_UnitBase.maxAttack` (`KismetMathLibrary.FTrunc` (* _output_get_3 0.75)) _targetunit_3)
      (set `self.particle` null)
      (set `/Game/TurnBasedJRPGTemplate/Blueprints/Units/BP_UnitBase.Ailments` "NewEnumerator0" _targetunit)
      (set `/Game/TurnBasedJRPGTemplate/Blueprints/Units/BP_UnitBase.IsExhausted` true _targetunit))))

(event `self.OnBuffEnded`
  (bind _targetunit (`self.targetUnit`))
  (bind _targetunit_2 (`self.targetUnit`))
  ;[1 1 1] Inside the BP_Poison, it apply and save the "poisoned state"
  (set `/Game/TurnBasedJRPGTemplate/Blueprints/Units/BP_UnitBase.defense` (`self.DefaultDefense`) _targetunit_2)
  (set `/Game/TurnBasedJRPGTemplate/Blueprints/Units/BP_UnitBase.minAttack` (`self.DefaultMinAttack`) _targetunit_2)
  (set `/Game/TurnBasedJRPGTemplate/Blueprints/Units/BP_UnitBase.maxAttack` (`self.DefaultMaxAttack`) _targetunit_2)
  (`KismetSystemLibrary.PrintString` "Deactivated")
  (`/Game/TurnBasedJRPGTemplate/Blueprints/Units/BP_UnitBase.OnBuffEnded` (`self.targetUnit`) false false false false false false false false false false true)
  (set `/Game/TurnBasedJRPGTemplate/Blueprints/Units/BP_UnitBase.IsExhausted` false _targetunit)
  (set `/Game/TurnBasedJRPGTemplate/Blueprints/Units/BP_UnitBase.TotalAmpPoints` 0 _targetunit)
  (`/Game/TurnBasedJRPGTemplate/Blueprints/Units/BP_UnitBase.SetExhaustionPoints` _targetunit (`/Game/TurnBasedJRPGTemplate/Blueprints/Units/BP_UnitBase.MaxExhaustionPoints` _targetunit))
  (`/Game/TurnBasedJRPGTemplate/Blueprints/Units/BP_UnitBase.AddAmpPoints` _targetunit 0)
  (if (not (`/Game/TurnBasedJRPGTemplate/Blueprints/Units/BP_UnitBase.Is DOT` _targetunit))
    (set `/Game/TurnBasedJRPGTemplate/Blueprints/Units/BP_UnitBase.Ailments` "NewEnumerator3" (`self.targetUnit`))))

(fn `UserConstructionScript`
  (`parent.UserConstructionScript`))