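; BP_Inoculate is a healing skill that cures poison on a target unit, both in battle and while exploring.
; In battle it spawns an antidote effect at the current target's StatusSocket, plays a heal sound, calls RemovePoison, then signals skill use after a short delay.
; In exploration it clears the PoisonDamage flag in the player controller's unit data map, plays the sound and signals immediately.
; BeginPlay calls IsRemovePoison.
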(event `self.ReceiveBeginPlay`
  (`self.Is Remove Poison`))

(event `self.UseBattleSkillInExplore`
  (params (targetUnit :type Name))
  (bind _structout (setmembers `/Game/TurnBasedJRPGTemplate/Blueprints/Structs/S_PlayerUnitData` :`StructRef` (`BlueprintMapLibrary.Map_Find` (`/Game/TurnBasedJRPGTemplate/Blueprints/Controllers/BP_JRPGPlayerController.PlayerUnitDataID` (`self.jRPGPlayerController`)) targetUnit) :`PoisonDamage` false))
  (`BlueprintMapLibrary.Map_Add` (`/Game/TurnBasedJRPGTemplate/Blueprints/Controllers/BP_JRPGPlayerController.PlayerUnitDataID` (`self.jRPGPlayerController`)) targetUnit _structout)
  (`GameplayStatics.PlaySoundAtLocation` "/Game/Sounds/Se/Heal1.Heal1_0" (0.0 0.0 0.0) (struct) 1.0 1.0 0.0 null null null)
  (`self.OnSkillUsed`))

(event `self.UseSkill`
  (bind _currenttargetunit (`/Game/TurnBasedJRPGTemplate/Blueprints/Battle/BP_BattleController.currentTargetUnit` (`self.battleController`)))
  ;[1 1 1] Applies Particle Effect
  (`|SpawnActorFromClass` "/Game/TurnBasedJRPGTemplate/Blueprints/Projectiles/ParticleEffects/Healing/BP_AntidoteEffect.BP_AntidoteEffect_C" (`SceneComponent.GetSocketTransform` (`/Game/TurnBasedJRPGTemplate/Blueprints/Units/BP_UnitBase.Pixel2D` _currenttargetunit) "StatusSocket" "RTS_World") "Undefined" "OverrideRootScale" null null)
  (`GameplayStatics.PlaySoundAtLocation` "/Game/Sounds/Se/Heal1.Heal1_0" (0.0 0.0 0.0) (struct) 1.0 1.0 0.0 null null null)
  (`/Game/TurnBasedJRPGTemplate/Blueprints/Units/BP_UnitBase.Remove Poison` _currenttargetunit)
  (`KismetSystemLibrary.Delay` 1.5)
  (`self.OnSkillUsed`))

(fn `UserConstructionScript`
  (`parent.UserConstructionScript`))