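; Enemy skill for the turn-based JRPG battle in which the attacker consumes one of its own allies.
; It picks a random enemy unit, recursively rerolling on any matching the attacker's class, then jump-moves to it.
; On arrival it heals by the victim's current HP and zeroes that HP.
; A lone attacker instead jumps to the existing target, then damages a randomly re-picked player unit.
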(event `If self is selected`
  (bind _battlecontroller (`self.battleController`))
  (bind _enemyunits (`/Game/TurnBasedJRPGTemplate/Blueprints/Battle/BP_BattleBase.enemyUnits` (`/Game/TurnBasedJRPGTemplate/Blueprints/Battle/BP_BattleController.currentBattle` (`self.battleController`))))
  (if (== (`KismetArrayLibrary.Array_Length` _enemyunits) 1) :!label _label
    (`self.AttackEnemyIfAlone`)
    (else
      (bind _output_get (set `/Game/TurnBasedJRPGTemplate/Blueprints/Battle/BP_BattleController.currentTargetUnit` (`|GetArrayItem` _enemyunits (`KismetMathLibrary.RandomIntegerInRange` 0 (`KismetArrayLibrary.Array_LastIndex` _enemyunits))) (`self.battleController`)))
      (if (== (`GameplayStatics.GetObjectClass` _output_get) (`GameplayStatics.GetObjectClass` (`/Game/TurnBasedJRPGTemplate/Blueprints/Battle/BP_BattleController.currentAttackingUnit` (`self.battleController`))))
        (`KismetSystemLibrary.PrintString` "SelfSelected" true true (struct :`G` 0.66 :`B` 1.0 :`A` 1.0) 0.2)
        (`self.If self is selected`)
        (else
          (`/Game/TurnBasedJRPGTemplate/Blueprints/Battle/BP_BattleController.MoveToTarget` _battlecontroller (`SceneComponent.K2_GetComponentLocation` (`/Game/TurnBasedJRPGTemplate/Blueprints/Units/BP_UnitBase.MeleeAttackerLocation` (`/Game/TurnBasedJRPGTemplate/Blueprints/Battle/BP_BattleController.currentTargetUnit` _battlecontroller))) (delegate `CustomEvent_0`) false true))))))

(event `/Game/TurnBasedJRPGTemplate/Blueprints/Skills/BP_SkillBase.UseSkill`
  (goto _label))

(event `CustomEvent_0`
  (bind _battlecontroller (`self.battleController`))
  (bind _currenttargetunit (`/Game/TurnBasedJRPGTemplate/Blueprints/Battle/BP_BattleController.currentTargetUnit` _battlecontroller))
  (`/Game/TurnBasedJRPGTemplate/Blueprints/Units/BP_UnitBase.Heal` (`/Game/TurnBasedJRPGTemplate/Blueprints/Battle/BP_BattleController.currentAttackingUnit` _battlecontroller) (`/Game/TurnBasedJRPGTemplate/Blueprints/Units/BP_UnitBase.currentHP` _currenttargetunit) 0)
  (`/Game/TurnBasedJRPGTemplate/Blueprints/Units/BP_UnitBase.SetHP` _currenttargetunit 0)
  (`/Game/TurnBasedJRPGTemplate/Blueprints/Skills/BP_SkillBase.OnSkillUsed`))

(event `AttackEnemyIfAlone`
  (`/Game/TurnBasedJRPGTemplate/Blueprints/Battle/BP_BattleController.MoveToTarget` (`self.battleController`) (`SceneComponent.K2_GetComponentLocation` (`/Game/TurnBasedJRPGTemplate/Blueprints/Units/BP_UnitBase.MeleeAttackerLocation` (`/Game/TurnBasedJRPGTemplate/Blueprints/Battle/BP_BattleController.currentTargetUnit` (`self.battleController`)))) (delegate `Kill`) false true))

(event `Kill`
  (bind _battlecontroller (`self.battleController`))
  (bind _playerunits (`/Game/TurnBasedJRPGTemplate/Blueprints/Battle/BP_BattleBase.playerUnits` (`/Game/TurnBasedJRPGTemplate/Blueprints/Battle/BP_BattleController.currentBattle` (`self.battleController`))))
  (set `/Game/TurnBasedJRPGTemplate/Blueprints/Battle/BP_BattleController.currentTargetUnit` (`|GetArrayItem` _playerunits (`KismetMathLibrary.RandomIntegerInRange` 0 (`KismetArrayLibrary.Array_LastIndex` _playerunits))) _battlecontroller)
  (`/Game/TurnBasedJRPGTemplate/Blueprints/Battle/BP_BattleController.DealDamage` _battlecontroller 10 1.0 0.0)
  (`/Game/TurnBasedJRPGTemplate/Blueprints/Skills/BP_SkillBase.OnSkillUsed`))

(fn `UserConstructionScript`
  (`parent.UserConstructionScript`))