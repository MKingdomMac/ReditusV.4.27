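; BP_StirUp is an enemy skill in the DeepHeremus folder of the turn-based JRPG that grants temporary buffs to enemy units.
; UseSkill loops backwards through the battle's enemy units, setting each as target, then switches the attacker's animation, plays a power-up emitter and sound, applies buffs and signals completion.
; Delays sit inside the loop without pausing it, so the delayed steps act on the last target set.
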(event `/Game/TurnBasedJRPGTemplate/Blueprints/Skills/BP_SkillBase.UseSkill`
  (bind _battlecontroller (`self.battleController`))
  (bind _currentattackingunit (`/Game/TurnBasedJRPGTemplate/Blueprints/Battle/BP_BattleController.currentAttackingUnit` (`self.battleController`)))
  ;[1 1 1] Applies Particle Effect
  (bind (_arrayindex _arrayelement) (`/Engine/EditorBlueprintResources/StandardMacros.ReverseForEachLoop` (`/Game/TurnBasedJRPGTemplate/Blueprints/Battle/BP_BattleBase.enemyUnits` (`/Game/TurnBasedJRPGTemplate/Blueprints/Battle/BP_BattleController.currentBattle` _battlecontroller)))
    (:`LoopBody`
      (bind _output_get (set `/Game/TurnBasedJRPGTemplate/Blueprints/Battle/BP_BattleController.currentTargetUnit` _arrayelement _battlecontroller))
      (set `/Game/TurnBasedJRPGTemplate/Blueprints/Units/BP_UnitBase.E_EnemySkillsAttackAnimations` "NewEnumerator11" _currentattackingunit)
      (`KismetSystemLibrary.Delay` 0.2)
      (set `/Game/TurnBasedJRPGTemplate/Blueprints/Units/BP_UnitBase.E_EnemySkillsAttackAnimations` "NewEnumerator4" _currentattackingunit)
      (`GameplayStatics.SpawnEmitterAttached` "/Game/Particles/GoodParticleStatus/Particles/Buff_Status/PS_GPS_Buff_PowerUp.PS_GPS_Buff_PowerUp" (`/Game/TurnBasedJRPGTemplate/Blueprints/Units/BP_UnitBase.Pixel2D` _output_get))
      (`GameplayStatics.PlaySound2D` "/Game/Sounds/Se/Neon.Neon_0" 1.0 1.0 0.0 null null)
      (`KismetSystemLibrary.Delay` 1.5)
      (`self.ApplyBuffs` (`|MakeArray` (`/Game/TurnBasedJRPGTemplate/Blueprints/Battle/BP_BattleController.currentTargetUnit` (`self.battleController`))))
      (`self.OnSkillUsed`))))

(fn `UserConstructionScript`
  (`parent.UserConstructionScript`))