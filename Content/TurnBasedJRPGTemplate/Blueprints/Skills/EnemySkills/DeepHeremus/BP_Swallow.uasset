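; BP_Swallow is an enemy skill, filed under DeepHeremus, that makes the attacking unit appear to swallow its current target.
; On use, it sets the target's move speed and moves it to the attacker's location without a jump attack.
; When the move completes, a bound event hides the target, waits briefly, applies non-permanent buffs to it and signals that the skill was used.
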(event `/Game/TurnBasedJRPGTemplate/Blueprints/Skills/BP_SkillBase.UseSkill`
  (bind _battlecontroller (`self.battleController`))
  (bind _currenttargetunit (`/Game/TurnBasedJRPGTemplate/Blueprints/Battle/BP_BattleController.currentTargetUnit` _battlecontroller))
  (set `/Game/TurnBasedJRPGTemplate/Blueprints/Units/BP_UnitBase.moveSpeed` 300.0 _currenttargetunit)
  (`/Game/TurnBasedJRPGTemplate/Blueprints/Units/BP_UnitBase.MoveToTarget` _currenttargetunit (`self.K2_GetActorLocation` (`/Game/TurnBasedJRPGTemplate/Blueprints/Battle/BP_BattleController.currentAttackingUnit` _battlecontroller)) false false)
  (add `/Game/TurnBasedJRPGTemplate/Blueprints/Units/BP_UnitBase.OnMovedToTarget` _currenttargetunit (delegate `MoveToTarget`)))

(event `MoveToTarget`
  (bind _currenttargetunit (`/Game/TurnBasedJRPGTemplate/Blueprints/Battle/BP_BattleController.currentTargetUnit` (`self.battleController`)))
  (`self.SetActorHiddenInGame` _currenttargetunit true)
  (`KismetSystemLibrary.Delay` 1.0)
  (`self.ApplyBuffs` (`|MakeArray` _currenttargetunit))
  (`/Game/TurnBasedJRPGTemplate/Blueprints/Skills/BP_SkillBase.OnSkillUsed`))

(fn `UserConstructionScript`
  (`parent.UserConstructionScript`))