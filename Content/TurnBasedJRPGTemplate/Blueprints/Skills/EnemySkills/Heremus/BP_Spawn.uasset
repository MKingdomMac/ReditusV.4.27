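; BP_Spawn is an enemy skill of Heremus that summons a BP_HeremusHarrier into the current battle.
; On UseSkill it loops over the battle's enemy spawn locations and acts only on the last one.
; It spawns the Harrier at that point's location and rotation, passes it the current battle, and adds it to the battle's enemy units.
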(event `/Game/TurnBasedJRPGTemplate/Blueprints/Skills/BP_SkillBase.UseSkill`
  (bind _currentbattle (`/Game/TurnBasedJRPGTemplate/Blueprints/Battle/BP_BattleController.currentBattle` (`self.battleController`)))
  (bind _enemyspawnlocations (`/Game/TurnBasedJRPGTemplate/Blueprints/Battle/BP_BattleBase.enemySpawnLocations` _currentbattle))
  ;[1 1 1] Move to target
  (for (_array_element _array_index) _enemyspawnlocations
    (if (== (`KismetArrayLibrary.Array_LastIndex` _enemyspawnlocations) _array_index)
      (bind _returnvalue (`|SpawnActorFromClass` :`Class` "/Game/TurnBasedJRPGTemplate/Blueprints/Units/EnemyUnits/HeremusEnemyUnits/BP_HeremusHarrier.BP_HeremusHarrier_C" :`SpawnTransform` (`KismetMathLibrary.MakeTransform` (`self.K2_GetActorLocation` _array_element) (`self.K2_GetActorRotation` _array_element)) :`CollisionHandlingOverride` "Undefined" :`TransformScaleMethod` "OverrideRootScale" :`battle` _currentbattle :`Instigator` null))
      (`KismetArrayLibrary.Array_Add` (`/Game/TurnBasedJRPGTemplate/Blueprints/Battle/BP_BattleBase.enemyUnits` _currentbattle) _returnvalue))))

(fn `UserConstructionScript`
  (`parent.UserConstructionScript`))