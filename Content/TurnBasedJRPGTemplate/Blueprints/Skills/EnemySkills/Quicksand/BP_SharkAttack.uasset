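; Shark Attack enemy skill for the turn-based battle system, filed under the Quicksand enemy.
; On use, it chains BattleController moves through callbacks: forward to the target's ranged attacker spot, a short pause, then a jump attack to the melee spot.
; It then deals damage and, on a hit against a target not immune to Sleep, applies its non-permanent buffs.
; It signals skill completion either way.
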(event `/Game/TurnBasedJRPGTemplate/Blueprints/Skills/BP_SkillBase.UseSkill`
  (bind _battlecontroller (`self.battleController`))
  (`/Game/TurnBasedJRPGTemplate/Blueprints/Battle/BP_BattleController.MoveToTarget` _battlecontroller (`SceneComponent.K2_GetComponentLocation` (`/Game/TurnBasedJRPGTemplate/Blueprints/Units/BP_UnitBase.RangedAttackerLocation` (`/Game/TurnBasedJRPGTemplate/Blueprints/Battle/BP_BattleController.currentTargetUnit` _battlecontroller))) (delegate `CustomEvent_1`) true false))

(event `CustomEvent_1`
  (bind _battlecontroller (`self.battleController`))
  (`KismetSystemLibrary.Delay` 1.0)
  (`/Game/TurnBasedJRPGTemplate/Blueprints/Battle/BP_BattleController.MoveToTarget` _battlecontroller (`SceneComponent.K2_GetComponentLocation` (`/Game/TurnBasedJRPGTemplate/Blueprints/Units/BP_UnitBase.MeleeAttackerLocation` (`/Game/TurnBasedJRPGTemplate/Blueprints/Battle/BP_BattleController.currentTargetUnit` _battlecontroller))) (delegate `CustomEvent`) false true))

(event `CustomEvent`
  (bind _currenttargetunit (`/Game/TurnBasedJRPGTemplate/Blueprints/Battle/BP_BattleController.currentTargetUnit` (`self.battleController`)))
  (bind _ishit (`/Game/TurnBasedJRPGTemplate/Blueprints/Battle/BP_BattleController.DealDamage` (`self.battleController`) 0 1.0 1.0))
  (if (and _ishit (not (`KismetArrayLibrary.Array_Contains` (`/Game/TurnBasedJRPGTemplate/Blueprints/Units/BP_UnitBase.Immunities` _currenttargetunit) "/Game/TurnBasedJRPGTemplate/Blueprints/Skills/Buffs/BP_Sleep.BP_Sleep_C")))
    (`self.ApplyBuffs` (`|MakeArray` _currenttargetunit))
    (`/Game/TurnBasedJRPGTemplate/Blueprints/Skills/BP_SkillBase.OnSkillUsed`)
    (else
      (`/Game/TurnBasedJRPGTemplate/Blueprints/Skills/BP_SkillBase.OnSkillUsed`))))

(fn `UserConstructionScript`
  (`parent.UserConstructionScript`))