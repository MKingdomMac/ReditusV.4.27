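; BP_TargetSpot is a hero skill for Caeser in the turn-based JRPG that buffs every player unit in the current battle.
; UseSkill walks the party in reverse, setting each unit as the current target, attaching an Eagle Vision particle to its StatusSocket and applying non-permanent buffs.
; It then plays a heal sound and signals skill completion after a short delay.
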(event `/Game/TurnBasedJRPGTemplate/Blueprints/Skills/BP_SkillBase.UseSkill`
  (bind _battlecontroller (`self.battleController`))
  ;[1 1 1] Heal fully
  (bind (_arrayindex _arrayelement) (`/Engine/EditorBlueprintResources/StandardMacros.ReverseForEachLoop` (`/Game/TurnBasedJRPGTemplate/Blueprints/Battle/BP_BattleBase.playerUnits` (`/Game/TurnBasedJRPGTemplate/Blueprints/Battle/BP_BattleController.currentBattle` _battlecontroller)))
    (:`LoopBody`
      (bind _output_get (set `/Game/TurnBasedJRPGTemplate/Blueprints/Battle/BP_BattleController.currentTargetUnit` _arrayelement _battlecontroller))
      (`GameplayStatics.SpawnEmitterAttached` "/Game/Particles/GoodParticleStatus/Particles/Head_Status/PS_GPS_EagleVision.PS_GPS_EagleVision" (`/Game/TurnBasedJRPGTemplate/Blueprints/Units/BP_UnitBase.Pixel2D` _output_get) "StatusSocket")
      (`self.ApplyBuffs` (`|MakeArray` _output_get)))
    (:`Completed`
      (`GameplayStatics.PlaySound2D` "/Game/Sounds/JrpgBlueprintSounds/CUE_Heal.CUE_Heal" 1.0 1.0 0.0 null null)
      (`KismetSystemLibrary.Delay` 1.0)
      (`self.OnSkillUsed`))))

(fn `UserConstructionScript`
  (`parent.UserConstructionScript`))