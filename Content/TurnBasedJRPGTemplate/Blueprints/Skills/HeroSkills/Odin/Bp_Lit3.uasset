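; Bp_Lit3 is a skill Blueprint in Odin's hero skill set for the turn-based JRPG, currently little more than a stub.
; UseSkill, commented CaeserShotgunAttack, only calls the parent implementation, so all working behavior is inherited.
; The hold-action input event is empty, and the debug prints are never executed.
; GetNextIndex holds unused wrap-around index logic.
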(event `EnhancedInput|/Game/TurnBasedJRPGTemplate/InputActions/IA_HoldAction`
  (params (ActionValue :type Boolean) (ElapsedSeconds :type "Float (single-precision)") (TriggeredSeconds :type "Float (single-precision)")))

(event `/Game/TurnBasedJRPGTemplate/Blueprints/Skills/BP_SkillBase.UseSkill`
  ;[1 1 1] CaeserShotgunAttack
  (`parent.UseSkill`))

(fn `UserConstructionScript`
  (`parent.UserConstructionScript`))