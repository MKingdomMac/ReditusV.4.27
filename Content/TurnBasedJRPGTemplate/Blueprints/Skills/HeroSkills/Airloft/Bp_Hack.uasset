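; Airloft's Hack battle skill, which tries to recruit a robot enemy through a negotiation dialogue.
; UseSkill rejects non-robots, certain status-afflicted targets and robots already in the party, restarting the turn.
; Otherwise the hero moves in, the camera isolates the target, and a tutorial or random bot dialogue plays.
; Its result branches to Fight (party buff), Join (recruitment) or Run (enemy removed); the hack minigame and disassembly code are disconnected.
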(event `Fight`
  (bind _battlecontroller (`self.battleController`))
  ;[1 1 1] Fight Dialogue Decision
  (`/Game/TurnBasedJRPGTemplate/Blueprints/Battle/BP_BattleController.MoveToTarget` _battlecontroller (`/Game/TurnBasedJRPGTemplate/Blueprints/Units/BP_UnitBase.initialLocation` (`/Game/TurnBasedJRPGTemplate/Blueprints/Battle/BP_BattleController.currentAttackingUnit` _battlecontroller)) (delegate `MoveThenFightHandler`) false false))

(event `MoveThenFightHandler`
  (bind _battlecontroller (`self.battleController`))
  (bind _battlecontroller_2 (`self.battleController`))
  ;[1 1 1] Fight Dialogue Decision
  (`self.EnemyUnitsVisible?` false)
  (`Widget.SetVisibility` (`/Game/TurnBasedJRPGTemplate/Blueprints/Battle/BP_BattleController.battleUI` _battlecontroller_2) "Visible")
  (`PlayerController.SetViewTargetWithBlend` (`GameplayStatics.GetPlayerController` 0) (`/Game/TurnBasedJRPGTemplate/Blueprints/Battle/BP_BattleBase.staticCamera` (`/Game/TurnBasedJRPGTemplate/Blueprints/Battle/BP_BattleController.currentBattle` _battlecontroller_2)) 0.5 "VTBlend_Cubic" 0.5 false)
  (`KismetSystemLibrary.Delay` 0.2)
  (`NiagaraFunctionLibrary.SpawnSystemAttached` "/Game/Particles/RPGEffects/ParticlesNiagara/Mage/LightningBolt/NS_Mage_LIghtning_Bolt.NS_Mage_LIghtning_Bolt" (`/Game/TurnBasedJRPGTemplate/Blueprints/Units/BP_UnitBase.Pixel2D` (`/Game/TurnBasedJRPGTemplate/Blueprints/Battle/BP_BattleController.currentAttackingUnit` _battlecontroller)) "None" (0.0 0.0 0.0) (struct) "KeepRelativeOffset")
  (`GameplayStatics.PlaySound2D` "/Game/Sounds/Se/Thunder6.Thunder6_0" 1.0 1.0 0.0 null null)
  (`self.ApplyBuffs` (`/Game/TurnBasedJRPGTemplate/Blueprints/Battle/BP_BattleBase.playerUnits` (`/Game/TurnBasedJRPGTemplate/Blueprints/Battle/BP_BattleController.currentBattle` _battlecontroller)))
  (`self.OnSkillAnimationEnded`))

(event `SetDialogues`
  (bind _dialoguepool_botdialogue (break `/Game/TurnBasedJRPGTemplate/Blueprints/Structs/S_DialoguePool` (`self.DialoguePool`)))
  ;[1 1 1] Decide Which Dialogue Based On Enemy Personality
  (if (`/Game/TurnBasedJRPGTemplate/Blueprints/Controllers/BP_JRPGPlayerController.AirloftHackTutorial` (`self.J RPGPlayer Controller`))
    (set `self.Dialogue` "/Game/DialogueSystem/RecruitmentDialogues/PlayfulDialogues/D_PlayfulDialogue1_1.D_PlayfulDialogue1_1")
    (else
      (set `self.Dialogue` (`KismetArrayLibrary.Array_Random` _dialoguepool_botdialogue)))))

(event `RemoveEnemyFromBattle`
  (bind _battlecontroller (`self.battleController`))
  (bind _battlecontroller_2 (`self.battleController`))
  (bind _currenttargetunit (`/Game/TurnBasedJRPGTemplate/Blueprints/Battle/BP_BattleController.currentTargetUnit` _battlecontroller_2))
  ;[1 1 1] Enemy runs from battle
  (`self.EnemyUnitsVisible?` false)
  (`/Game/TurnBasedJRPGTemplate/Blueprints/Battle/BP_BattleBase.OnEnemyUnitDiedHandler` (`/Game/TurnBasedJRPGTemplate/Blueprints/Battle/BP_BattleController.currentBattle` _battlecontroller_2) _currenttargetunit)
  (`GameplayStatics.PlaySound2D` "/Game/Sounds/Se/Run.Run_0" 1.0 1.0 0.0 null null)
  (`self.K2_DestroyActor` _currenttargetunit)
  (`Widget.SetVisibility` (`/Game/TurnBasedJRPGTemplate/Blueprints/Battle/BP_BattleController.battleUI` _battlecontroller) "Visible")
  (`PlayerController.SetViewTargetWithBlend` (`GameplayStatics.GetPlayerController` 0) (`/Game/TurnBasedJRPGTemplate/Blueprints/Battle/BP_BattleBase.staticCamera` (`/Game/TurnBasedJRPGTemplate/Blueprints/Battle/BP_BattleController.currentBattle` _battlecontroller)) 0.5 "VTBlend_Cubic" 0.5 false)
  (`self.OnSkillAnimationEnded`))

(event `Enemy Join`
  (bind _battlecontroller (`self.battleController`))
  ;[1 1 1] Enemy Recruited
  (`self.EnemyUnitsVisible?` false)
  (`Widget.SetVisibility` (`/Game/TurnBasedJRPGTemplate/Blueprints/Battle/BP_BattleController.battleUI` _battlecontroller) "Visible")
  (`PlayerController.SetViewTargetWithBlend` (`GameplayStatics.GetPlayerController` 0) (`/Game/TurnBasedJRPGTemplate/Blueprints/Battle/BP_BattleBase.staticCamera` (`/Game/TurnBasedJRPGTemplate/Blueprints/Battle/BP_BattleController.currentBattle` _battlecontroller)) 0.5 "VTBlend_Cubic" 0.5 false)
  (`/Game/TurnBasedJRPGTemplate/Blueprints/Battle/BP_BattleController.MoveToTarget` _battlecontroller (`/Game/TurnBasedJRPGTemplate/Blueprints/Units/BP_UnitBase.initialLocation` (`/Game/TurnBasedJRPGTemplate/Blueprints/Battle/BP_BattleController.currentAttackingUnit` _battlecontroller)) (delegate `MoveBack`) false false))

(event `MoveBack`
  ;[1 1 1] Enemy Recruited
  (`KismetSystemLibrary.Delay` 1.0)
  (`/Game/TurnBasedJRPGTemplate/Blueprints/Units/BP_UnitBase.MoveToTarget` (`/Game/TurnBasedJRPGTemplate/Blueprints/Battle/BP_BattleController.currentTargetUnit` (`self.battleController`)) (`SceneComponent.K2_GetComponentLocation` (`/Game/TurnBasedJRPGTemplate/Blueprints/Units/BP_UnitBase.MeleeAttackerLocation` (`/Game/TurnBasedJRPGTemplate/Blueprints/Battle/BP_BattleController.currentAttackingUnit` (`self.battleController`)))) true false)
  (`KismetSystemLibrary.Delay` 1.0)
  (`/Game/TurnBasedJRPGTemplate/Blueprints/Battle/BP_BattleController.EnemyRecruited` (`self.battleController`))
  (`/Game/TurnBasedJRPGTemplate/Blueprints/Controllers/BP_JRPGPlayerController.SteamAchievements` (`self.J RPGPlayer Controller`) "Hacker!"))

(event `/Game/TurnBasedJRPGTemplate/Blueprints/Skills/BP_SkillBase.UseSkill`
  (bind _battlecontroller (`self.battleController`))
  (bind _currenttargetunit (`/Game/TurnBasedJRPGTemplate/Blueprints/Battle/BP_BattleController.currentTargetUnit` _battlecontroller))
  (bind _asbp_player_unit_base (cast `/Game/TurnBasedJRPGTemplate/Blueprints/Units/PlayerUnits/BP_PlayerUnitBase` (`/Game/TurnBasedJRPGTemplate/Blueprints/Battle/BP_BattleController.currentAttackingUnit` _battlecontroller) :!pure true))
  ;[1 1 1] Recrut
  (set `self.J RPGPlayer Controller` (`/Game/TurnBasedJRPGTemplate/Blueprints/Battle/BP_BattleController.jRPGPlayerController` (`self.battleController`)))
  (if (and (not (`/Game/TurnBasedJRPGTemplate/Blueprints/Units/BP_UnitBase.IsSleeping` _currenttargetunit)) (`|EnumEquality` (`/Game/TurnBasedJRPGTemplate/Blueprints/Units/BP_UnitBase.E_EnemyClass` _currenttargetunit) "NewEnumerator0") (not (`/Game/TurnBasedJRPGTemplate/Blueprints/Units/BP_UnitBase.Is Confused` _currenttargetunit)) (not (`/Game/TurnBasedJRPGTemplate/Blueprints/Units/BP_UnitBase.IsBerserk??` _currenttargetunit)) (not (`/Game/TurnBasedJRPGTemplate/Blueprints/Units/BP_UnitBase.Is DOT` _currenttargetunit)))
    (if (`BlueprintMapLibrary.Map_Contains` (`/Game/TurnBasedJRPGTemplate/Blueprints/Controllers/BP_JRPGPlayerController.PlayerUnitDataID` (`/Game/TurnBasedJRPGTemplate/Blueprints/Battle/BP_BattleController.jRPGPlayerController` _battlecontroller)) (`/Game/TurnBasedJRPGTemplate/Blueprints/Units/EnemyUnits/BP_EnemyUnitBase.RecruitedUnit` (cast `/Game/TurnBasedJRPGTemplate/Blueprints/Units/EnemyUnits/BP_EnemyUnitBase` (`/Game/TurnBasedJRPGTemplate/Blueprints/Battle/BP_BattleController.currentTargetUnit` _battlecontroller) :!pure true)))
      ;;[1 1 1] get ready
      (bind _returnvalue (`|CreateWidget` "/Game/TurnBasedJRPGTemplate/Blueprints/UI/Dialogues/BP_InfoDialogue.BP_InfoDialogue_C" null "Robot is already in Party!" "" true _asbp_player_unit_base))
      (`UserWidget.AddToViewport` _returnvalue 0)
      (`KismetSystemLibrary.Delay` 2.0)
      (`Widget.RemoveFromParent` _returnvalue)
      (set `/Game/TurnBasedJRPGTemplate/Blueprints/Controllers/BP_JRPGPlayerController.gameState` "NewEnumerator1" (`/Game/TurnBasedJRPGTemplate/Blueprints/Battle/BP_BattleController.jRPGPlayerController` (`self.battleController`)))
      (`/Game/TurnBasedJRPGTemplate/Blueprints/Units/BP_UnitBase.StartTurn` (`/Game/TurnBasedJRPGTemplate/Blueprints/Battle/BP_BattleController.currentAttackingUnit` (`self.battleController`)))
      (else
        (`/Game/TurnBasedJRPGTemplate/Blueprints/Battle/BP_BattleController.MoveToTarget` _battlecontroller (`SceneComponent.K2_GetComponentLocation` (`/Game/TurnBasedJRPGTemplate/Blueprints/Units/BP_UnitBase.MeleeAttackerLocation` _currenttargetunit)) (delegate `MovedForward`) true false)))
    (else
      ;;[1 1 1] If Enemy is not Robot
      (bind _returnvalue_2 (`|CreateWidget` "/Game/TurnBasedJRPGTemplate/Blueprints/UI/Dialogues/BP_InfoDialogue.BP_InfoDialogue_C" null "Unable to hack!" "" true _asbp_player_unit_base))
      (`UserWidget.AddToViewport` _returnvalue_2 0)
      (`KismetSystemLibrary.Delay` 2.0)
      (`Widget.RemoveFromParent` _returnvalue_2)
      (set `/Game/TurnBasedJRPGTemplate/Blueprints/Controllers/BP_JRPGPlayerController.gameState` "NewEnumerator1" (`/Game/TurnBasedJRPGTemplate/Blueprints/Battle/BP_BattleController.jRPGPlayerController` (`self.battleController`)))
      (`/Game/TurnBasedJRPGTemplate/Blueprints/Units/BP_UnitBase.StartTurn` (`/Game/TurnBasedJRPGTemplate/Blueprints/Battle/BP_BattleController.currentAttackingUnit` (`self.battleController`))))))

(event `MovedForward`
  (bind _battlecontroller (`self.battleController`))
  (bind _battlecontroller_2 (`self.battleController`))
  (bind _asbp_player_unit_base (cast `/Game/TurnBasedJRPGTemplate/Blueprints/Units/PlayerUnits/BP_PlayerUnitBase` (`/Game/TurnBasedJRPGTemplate/Blueprints/Battle/BP_BattleController.currentAttackingUnit` (`self.battleController`)) :!pure true))
  ;[1 1 1] Recrut
  ;;[1 1 1] get ready
  (set `/Game/TurnBasedJRPGTemplate/Blueprints/Units/PlayerUnits/BP_PlayerUnitBase.isInputBlocked` false (cast `/Game/TurnBasedJRPGTemplate/Blueprints/Units/PlayerUnits/BP_PlayerUnitBase` (`/Game/TurnBasedJRPGTemplate/Blueprints/Battle/BP_BattleController.currentAttackingUnit` (`self.battleController`)) :!pure true))
  (`self.SetDialogues`)
  ;;[1 1 1] Set All Units Hidden Except Target
  (for _array_element (`/Game/TurnBasedJRPGTemplate/Blueprints/Battle/BP_BattleBase.enemyUnits` (`/Game/TurnBasedJRPGTemplate/Blueprints/Battle/BP_BattleController.currentBattle` _battlecontroller_2))
    (if (!= _array_element (`/Game/TurnBasedJRPGTemplate/Blueprints/Battle/BP_BattleController.currentTargetUnit` _battlecontroller_2))
      (`self.SetActorHiddenInGame` _array_element true)
      (`Widget.SetVisibility` (`/Game/TurnBasedJRPGTemplate/Blueprints/Battle/BP_BattleController.battleUI` _battlecontroller_2) "Hidden")))
  ;;[1 1 1] ZoomInOnRecruiting
  (`PlayerController.SetViewTargetWithBlend` (`GameplayStatics.GetPlayerController` 0) (`ChildActorComponent.ChildActor` (`/Game/TurnBasedJRPGTemplate/Blueprints/Units/BP_UnitBase.FrontCameraActor` (`/Game/TurnBasedJRPGTemplate/Blueprints/Battle/BP_BattleController.currentAttackingUnit` _battlecontroller_2))) 0.5 "VTBlend_Cubic" 0.5 false)
  (`KismetSystemLibrary.Delay` 1.0)
  (`NiagaraFunctionLibrary.SpawnSystemAttached` "/Game/Particles/RPGEffects/ParticlesNiagara/Mage/LightningBolt/NS_Mage_LIghtning_Bolt.NS_Mage_LIghtning_Bolt" (`/Game/TurnBasedJRPGTemplate/Blueprints/Units/BP_UnitBase.Pixel2D` (`/Game/TurnBasedJRPGTemplate/Blueprints/Battle/BP_BattleController.currentTargetUnit` (`self.battleController`))) "None" (0.0 0.0 0.0) (struct) "KeepRelativeOffset")
  (`GameplayStatics.PlaySound2D` "/Game/Sounds/Se/Thunder6.Thunder6_0" 1.0 1.0 0.0 null null)
  (`KismetSystemLibrary.Delay` 1.0)
  (`GameplayStatics.PlaySound2D` "/Game/Sounds/Se/Airloft_talk.Airloft_talk" 1.0 1.0 0.0 null null)
  (set `/Game/TurnBasedJRPGTemplate/Blueprints/Battle/BP_BattleController.battleTheme` null _battlecontroller)
  (`/Game/TurnBasedJRPGTemplate/Blueprints/Battle/BP_BattleController.PlayBattleTheme` _battlecontroller)
  (set `/Game/TurnBasedJRPGTemplate/Blueprints/Units/BP_UnitBase.IsHacking` true (`/Game/TurnBasedJRPGTemplate/Blueprints/Battle/BP_BattleController.currentAttackingUnit` (`self.battleController`)))
  ;;[1 1 1] BonusHackOpportunity
  (`KismetSystemLibrary.Delay` 1.0)
  (bind _returnvalue (`|CreateWidget` "/DialoguePlugin/UI/DemoDialogueWidget.DemoDialogueWidget_C" null (`self.Dialogue`) false false _asbp_player_unit_base null :!label _label))
  (`UserWidget.AddToViewport` _returnvalue 0)
  (set `self.DialogueWidget` _returnvalue)
  (set `/Game/TurnBasedJRPGTemplate/Blueprints/Units/PlayerUnits/BP_PlayerUnitBase.SelectType` "NewEnumerator0" _asbp_player_unit_base)
  ;;[1 1 1] End Negotation Reset Negotiation Points
  (add `/DialoguePlugin/UI/DemoDialogueWidget.Removed` (`self.DialogueWidget`) (delegate `RecruitmentHandler`)))

(event `RecruitmentHandler`
  (params (RecruitmentEvents :type "/Game/TurnBasedJRPGTemplate/Blueprints/Enums/E_RecruitmentEvents Enum" :default "NewEnumerator0"))
  ;[1 1 1] Recrut
  ;;[1 1 1] End Negotation Reset Negotiation Points
  (set `/Game/TurnBasedJRPGTemplate/Blueprints/Controllers/BP_JRPGPlayerController.NegotiationPoints` 0.0 (`self.J RPGPlayer Controller`))
  (switch `/Game/TurnBasedJRPGTemplate/Blueprints/Enums/E_RecruitmentEvents` RecruitmentEvents
    (:`NewEnumerator0`
      (`self.Fight`))
    (:`NewEnumerator1`
      (`self.Enemy Join`))
    (:`NewEnumerator2`
      (`self.RemoveEnemyFromBattle`)))
  (set `/Game/TurnBasedJRPGTemplate/Blueprints/Units/BP_UnitBase.IsHacking` false (`/Game/TurnBasedJRPGTemplate/Blueprints/Battle/BP_BattleController.currentAttackingUnit` (`self.battleController`))))

(event `self.UseSkillOnNotify`
  ;[1 1 1] Recrut
  (`/Game/TurnBasedJRPGTemplate/Blueprints/Units/BP_UnitBase.SetHP` (`/Game/TurnBasedJRPGTemplate/Blueprints/Battle/BP_BattleController.currentTargetUnit` (`self.battleController`)) 0))

(event `self.OnSkillAnimationEnded`
  ;[1 1 1] Recrut
  (`self.OnSkillUsed`))

(event `Gameover`
  ;[1 1 1] Recrut
  ;;[1 1 1] BonusHackOpportunity
  (`PlayerController.SetViewTargetWithBlend` (`GameplayStatics.GetPlayerController` 0) (`ChildActorComponent.ChildActor` (`/Game/TurnBasedJRPGTemplate/Blueprints/Units/BP_UnitBase.FrontCameraActor` (`/Game/TurnBasedJRPGTemplate/Blueprints/Battle/BP_BattleController.currentAttackingUnit` (`self.battleController`)))) 0.0 "VTBlend_Cubic" 0.0 false)
  (goto _label))

(fn `EnemyUnitsVisible?`
  (params (`EnemyUnitsHidden?` :type Boolean))
  (bind _battlecontroller (`self.battleController`))
  (for _array_element (`/Game/TurnBasedJRPGTemplate/Blueprints/Battle/BP_BattleBase.enemyUnits` (`/Game/TurnBasedJRPGTemplate/Blueprints/Battle/BP_BattleController.currentBattle` _battlecontroller))
    (if (!= _array_element (`/Game/TurnBasedJRPGTemplate/Blueprints/Battle/BP_BattleController.currentTargetUnit` _battlecontroller))
      (`self.SetActorHiddenInGame` _array_element `EnemyUnitsHidden?`))))

(fn `UserConstructionScript`
  (`parent.UserConstructionScript`))