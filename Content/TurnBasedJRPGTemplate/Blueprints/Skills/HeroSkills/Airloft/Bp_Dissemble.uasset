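; Airloft's Dissemble hero skill, which finishes off a weakened enemy and records its skill on the player controller.
; It requires a target at or below about 15% HP, of a specific enemy class and flagged dissemblable.
; Success zeroes target HP, even when already dissembled, and timed dialogue widgets report each outcome before the skill-used callback.
; The duplicate check compares the whole stored array to the one skill, rather than testing membership.
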(event `/Game/TurnBasedJRPGTemplate/Blueprints/Skills/BP_SkillBase.UseSkill`
  (bind _battlecontroller (`self.battleController`))
  (bind _currenttargetunit (`/Game/TurnBasedJRPGTemplate/Blueprints/Battle/BP_BattleController.currentTargetUnit` _battlecontroller))
  (bind _dissembled_skill (`/Game/TurnBasedJRPGTemplate/Blueprints/Controllers/BP_JRPGPlayerController.Dissembled Skill` (`/Game/TurnBasedJRPGTemplate/Blueprints/Battle/BP_BattleController.jRPGPlayerController` _battlecontroller)))
  (bind _skill_to_disassemble (`/Game/TurnBasedJRPGTemplate/Blueprints/Units/BP_UnitBase.Skill to Disassemble` _currenttargetunit))
  ;[1 1 1] Disassemble
  (if (and (<= (`/Game/TurnBasedJRPGTemplate/Blueprints/Units/BP_UnitBase.currentHP` _currenttargetunit) (`KismetMathLibrary.FCeil` (* (`/Game/TurnBasedJRPGTemplate/Blueprints/Units/BP_UnitBase.maxHP` _currenttargetunit) 0.15))) (`|EnumEquality` (`/Game/TurnBasedJRPGTemplate/Blueprints/Units/BP_UnitBase.E_EnemyClass` _currenttargetunit) "NewEnumerator0") (`/Game/TurnBasedJRPGTemplate/Blueprints/Units/BP_UnitBase.CanDissemble` _currenttargetunit))
    (if (`KismetArrayLibrary.Array_Identical` _dissembled_skill (`|MakeArray` _skill_to_disassemble))
      (bind _returnvalue (`|CreateWidget` "/Game/TurnBasedJRPGTemplate/Blueprints/UI/Dialogues/BP_InfoDialogue.BP_InfoDialogue_C" null "Already Dissembled!" "" false null))
      (`UserWidget.AddToViewport` _returnvalue 0)
      (`KismetSystemLibrary.Delay` 2.0)
      (`Widget.RemoveFromParent` _returnvalue)
      (else
        (`KismetArrayLibrary.Array_Add` _dissembled_skill _skill_to_disassemble)
        (bind _returnvalue_2 (`|CreateWidget` "/Game/TurnBasedJRPGTemplate/Blueprints/UI/Dialogues/BP_InfoDialogue.BP_InfoDialogue_C" null "Dissembled!" "" false null))
        (`UserWidget.AddToViewport` _returnvalue_2 0)
        (`KismetSystemLibrary.Delay` 2.0)
        (`Widget.RemoveFromParent` _returnvalue_2)))
    (`self.UseSkillOnNotify`)
    (`KismetSystemLibrary.Delay` 1.0)
    (else
      (bind _returnvalue_3 (`|CreateWidget` "/Game/TurnBasedJRPGTemplate/Blueprints/UI/Dialogues/BP_InfoDialogue.BP_InfoDialogue_C" null "Unable to disassemble!" "" false null))
      (`UserWidget.AddToViewport` _returnvalue_3 0)
      (`KismetSystemLibrary.Delay` 2.0)
      (`Widget.RemoveFromParent` _returnvalue_3)))
  (`self.OnSkillAnimationEnded`))

(event `self.UseSkillOnNotify`
  ;[1 1 1] Disassemble
  (`/Game/TurnBasedJRPGTemplate/Blueprints/Units/BP_UnitBase.SetHP` (`/Game/TurnBasedJRPGTemplate/Blueprints/Battle/BP_BattleController.currentTargetUnit` (`self.battleController`)) 0))

(event `self.OnSkillAnimationEnded`
  ;[1 1 1] Disassemble
  (`self.OnSkillUsed`))

(fn `UserConstructionScript`
  (`parent.UserConstructionScript`))