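; BP_OverdriveTechBase is a base Blueprint for overdrive techs in a turn-based JRPG.
; UseOverdrive only fires the OnOverdriveUsed dispatcher, and the OnSkillUsed call is left unwired.
; ApplyBuffs rolls each buff class's success chance against every living target.
; Successful rolls call AddDuration on an existing buff, or spawn a buff actor far off-map, register it in the unit's ActiveBuffs map and apply it.
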(event `/Game/TurnBasedJRPGTemplate/Blueprints/Skills/BP_SkillBase.UseOverdrive`
  ;[1 1 1] Beginning of Skill
  (`/Game/TurnBasedJRPGTemplate/Blueprints/Skills/BP_SkillBase.OnOverdriveUsed`))

(event `self.ApplyBuffs`
  (params (targetUnits :type "Array of /Game/TurnBasedJRPGTemplate/Blueprints/Units/BP_UnitBase Object Reference (by ref)") (BuffPermanent :type Boolean))
  ;[1 1 1] Buffs If Any
  (for _array_element targetUnits
    (`/Engine/EditorBlueprintResources/StandardMacros.IsValid` _array_element
      (:`Is Valid`
        (bind _isunitdead (`/Game/TurnBasedJRPGTemplate/Blueprints/Units/BP_UnitBase.IsUnitDead` _array_element))
        (if (not _isunitdead)
          (for _array_element_2 (`self.buffs`)
            (if (>= (`.successChance` (defaults `Object` _array_element_2)) (`KismetMathLibrary.RandomFloatInRange` 0.0 1.0))
              (bind _activebuffs (`/Game/TurnBasedJRPGTemplate/Blueprints/Units/BP_UnitBase.activeBuffs` _array_element))
              (bind (_value _returnvalue) (`BlueprintMapLibrary.Map_Find` _activebuffs _array_element_2))
              (if _returnvalue
                (`/Game/TurnBasedJRPGTemplate/Blueprints/Skills/Buffs/BP_BuffBase.AddDuration` _value 0)
                (else
                  (bind _returnvalue_2 (`|SpawnActorFromClass` _array_element_2 (`KismetMathLibrary.MakeTransform` (999999.0 999999.0 999999.0)) "Undefined" "OverrideRootScale" null (`self.battleController`) _array_element false null))
                  (`BlueprintMapLibrary.Map_Add` _activebuffs _array_element_2 _returnvalue_2)
                  (`KismetSystemLibrary.PrintString` "BuffShouldApply")
                  (`/Game/TurnBasedJRPGTemplate/Blueprints/Skills/Buffs/BP_BuffBase.ApplyBuff` _returnvalue_2))))))))))

(fn `UserConstructionScript`
  (`parent.UserConstructionScript`))