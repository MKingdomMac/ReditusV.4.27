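; BP_DoubleHit is a turn-based battle skill that strikes the current target, intended as a double attack.
; It optionally moves the attacker to the target through BattleController, then plays the skill animation.
; Each animation notify deals normal-multiplier damage if the target is alive and applies non-permanent buffs to it on a hit.
; When the animation ends, the attacker returns to its initial location if it moved, then the skill reports completion.
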(event `/Game/TurnBasedJRPGTemplate/Blueprints/Skills/BP_SkillBase.UseSkill`
  ;[1 1 1] Move to target
  (`KismetSystemLibrary.PrintString` "suckit")
  (if (`/Game/TurnBasedJRPGTemplate/Blueprints/Battle/BP_BattleController.shouldUnitsMoveToTarget` (`self.battleController`))
    (`/Game/TurnBasedJRPGTemplate/Blueprints/Battle/BP_BattleController.MoveToTarget` (`self.battleController`) (`SceneComponent.K2_GetComponentLocation` (`Actor.RootComponent` (`/Game/TurnBasedJRPGTemplate/Blueprints/Battle/BP_BattleController.currentTargetUnit` (`self.battleController`)))) (delegate `OnUnitMovedToTargetHandler`) true false)
    (else
      (`self.PlaySkillAnimation` :!label _label))))

(event `OnUnitMovedToTargetHandler`
  ;[1 1 1] Move to target
  (goto _label))

(event `self.UseSkillOnNotify`
  (bind _battlecontroller (`self.battleController`))
  ;[1 1 1] Attack twice
  (bind _isunitdead (`/Game/TurnBasedJRPGTemplate/Blueprints/Units/BP_UnitBase.IsUnitDead` (`/Game/TurnBasedJRPGTemplate/Blueprints/Battle/BP_BattleController.currentTargetUnit` _battlecontroller)))
  (if (not _isunitdead)
    (bind _ishit (`/Game/TurnBasedJRPGTemplate/Blueprints/Battle/BP_BattleController.DealDamage` _battlecontroller 0 1.0 0.0))
    (if _ishit
      (`self.ApplyBuffs` (`|MakeArray` (`/Game/TurnBasedJRPGTemplate/Blueprints/Battle/BP_BattleController.currentTargetUnit` (`self.battleController`)))))))

(event `self.OnSkillAnimationEnded`
  ;[1 1 1] Attack twice
  (if (`/Game/TurnBasedJRPGTemplate/Blueprints/Battle/BP_BattleController.shouldUnitsMoveToTarget` (`self.battleController`))
    (`/Game/TurnBasedJRPGTemplate/Blueprints/Battle/BP_BattleController.MoveToTarget` (`self.battleController`) (`/Game/TurnBasedJRPGTemplate/Blueprints/Units/BP_UnitBase.initialLocation` (`/Game/TurnBasedJRPGTemplate/Blueprints/Battle/BP_BattleController.currentAttackingUnit` (`self.battleController`))) (delegate `OnUnitMovedBackHandler`) false false)
    (else
      (`self.OnSkillUsed` :!label _label_2))))

(event `OnUnitMovedBackHandler`
  ;[1 1 1] Attack twice
  (goto _label_2))

(fn `UserConstructionScript`
  (`parent.UserConstructionScript`))