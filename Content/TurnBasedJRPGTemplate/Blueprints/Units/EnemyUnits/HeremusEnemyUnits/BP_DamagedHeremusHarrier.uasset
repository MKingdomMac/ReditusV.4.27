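; BP_DamagedHeremusHarrier is an enemy battle unit for a damaged Heremus Harrier that plays ambush dialogue when it spawns.
; After a short delay on BeginPlay, it shows a demo dialogue widget that blocks input, then removes it after another delay.
; It fills its stats from level-based initial, first-level and last-level data.
; It supplies two projectile spawn transforms from sockets on its Pixel2D component.
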(event `self.ReceiveBeginPlay`
  (`parent.ReceiveBeginPlay`)
  (`KismetSystemLibrary.Delay` 4.0)
  (bind _returnvalue (`|CreateWidget` "/DialoguePlugin/UI/DemoDialogueWidget.DemoDialogueWidget_C" null "/Game/DialogueSystem/CodeSpartanDialogues/Heremus/Ambush/DuringAmbush.DuringAmbush" true true null null))
  (`UserWidget.AddToViewport` _returnvalue 0)
  (`KismetSystemLibrary.Delay` 4.0)
  (`Widget.RemoveFromParent` _returnvalue))

(event `self.SetUnitStats`
  (bind _stats (`/Game/TurnBasedJRPGTemplate/Blueprints/Controllers/BP_JRPGFunctionLibrary.GetUnitStats` (`self.level`) (`self.maxLevel`) (`self.initialStats`) (`self.firstLevelStats`) (`self.lastLevelStats`)))
  (bind (_maxhp _maxmp _attack _defense _speed _hit _magicalattack _magicdefense _actiontime _criticalhit _maxoverdrivepoints) (break `/Game/TurnBasedJRPGTemplate/Blueprints/Structs/S_UnitStats` _stats))
  (set `self.maxHP` _maxhp)
  (set `self.maxMP` _maxmp)
  (set `self.maxAttack` _attack)
  (set `self.defense` _defense)
  (set `self.speed` _speed)
  (set `self.hit` _hit)
  (set `self.maxMagicalAttack` _magicalattack)
  (set `self.magicalDefense` _magicdefense)
  (set `self.Critical` _criticalhit)
  (set `self.MaxOverdrivePoints` _maxoverdrivepoints))

(fn `GetProjectileSpawnTransform`
  (returns (projectileSpawnTransform :type "Transform Structure") (projectileSpawnTransform2 :type "Transform Structure"))
  (return (`SceneComponent.GetSocketTransform` (`self.Pixel2D`) "HeremusHarrier1" "RTS_World") (`SceneComponent.GetSocketTransform` (`self.Pixel2D`) "HeremusHarrier2" "RTS_World")))

(fn `UserConstructionScript`
  (`parent.UserConstructionScript`))