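; BP_Scourge is an enemy unit for turn-based battles that opens with a taunt.
; On turn start, a FirstTurn flag gates a one-time call to the BattleController to prepare BP_ScourgeTaunt, with a debug print; once set, turns defer to the parent logic.
; Both projectile spawn transforms come from the HeadWaves socket on its Pixel2D component.
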(event `self.StartTurn`
  (`self.OnTurnStarted`)
  (if (`self.FirstTurn`)
    (`parent.StartTurn`)
    (else
      (set `self.FirstTurn` true)
      (`/Game/TurnBasedJRPGTemplate/Blueprints/Battle/BP_BattleController.EnemyPrepareForSkill` (`self.battleController`) "/Game/TurnBasedJRPGTemplate/Blueprints/Skills/EnemySkills/Heremus/BP_ScourgeTaunt.BP_ScourgeTaunt_C" false false)
      (`KismetSystemLibrary.PrintString` "Taunt" true true (struct :`R` 1.0 :`G` 0.825233 :`A` 1.0)))))

(fn `GetProjectileSpawnTransform`
  (returns (projectileSpawnTransform :type "Transform Structure") (projectileSpawnTransform2 :type "Transform Structure"))
  (bind _returnvalue (`SceneComponent.GetSocketTransform` (`self.Pixel2D`) "HeadWaves" "RTS_World"))
  (return _returnvalue _returnvalue))

(fn `UserConstructionScript`
  (`parent.UserConstructionScript`))