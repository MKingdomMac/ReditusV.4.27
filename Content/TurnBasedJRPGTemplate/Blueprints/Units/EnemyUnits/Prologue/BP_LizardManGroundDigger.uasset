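; Enemy battle unit for the Lizard Man Ground Digger in the prologue of the turn-based JRPG.
; On turn start, if the controller's first battle tutorial flag is set, it shows a Caeser parry tutorial widget and delays the normal turn.
; When that dialogue is removed, it clears the flag and runs the parent turn.
; Projectile spawn transforms come from two HeremusHarrier sockets on its Pixel2D component.
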(event `self.StartTurn`
  (bind _battlecontroller (`self.battleController`))
  (if (`/Game/TurnBasedJRPGTemplate/Blueprints/Battle/BP_BattleController.BattleTutorial_1` _battlecontroller)
    (bind _returnvalue (`|CreateWidget` "/Game/TurnBasedJRPGTemplate/Blueprints/UI/BP_CaeserTutParry.BP_CaeserTutParry_C" null (`/Game/TurnBasedJRPGTemplate/Blueprints/Battle/BP_BattleController.jRPGPlayerController` _battlecontroller)))
    (`UserWidget.AddToViewport` _returnvalue 0)
    (add `/Game/TurnBasedJRPGTemplate/Blueprints/UI/BP_CaeserTutParry.DialogueRemoved` _returnvalue (delegate `TutFinished`))
    (else
      (`parent.StartTurn`))))

(event `TutFinished`
  (set `/Game/TurnBasedJRPGTemplate/Blueprints/Battle/BP_BattleController.BattleTutorial_1` false (`self.battleController`))
  (`parent.StartTurn`)
  (`KismetSystemLibrary.PrintString` "fuck fuck u"))

(fn `GetProjectileSpawnTransform`
  (returns (projectileSpawnTransform :type "Transform Structure") (projectileSpawnTransform2 :type "Transform Structure"))
  (return (`SceneComponent.GetSocketTransform` (`self.Pixel2D`) "HeremusHarrier1" "RTS_World") (`SceneComponent.GetSocketTransform` (`self.Pixel2D`) "HeremusHarrier2" "RTS_World")))

(fn `UserConstructionScript`
  (`parent.UserConstructionScript`))