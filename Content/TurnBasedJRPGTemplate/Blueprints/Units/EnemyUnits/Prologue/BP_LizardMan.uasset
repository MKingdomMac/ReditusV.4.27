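; Lizard Man enemy unit from the Prologue units of the turn-based JRPG template.
; Overrides projectile spawning to return two world-space transforms from the HeremusHarrier sockets on its Pixel2D component.
; StartTurn is overridden but empty, so the parent turn logic is not called.
; A disconnected branch that picks a no-skill attack when protected, or the parent turn otherwise, never runs.
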(event `self.StartTurn`)

(fn `GetProjectileSpawnTransform`
  (returns (projectileSpawnTransform :type "Transform Structure") (projectileSpawnTransform2 :type "Transform Structure"))
  (return (`SceneComponent.GetSocketTransform` (`self.Pixel2D`) "HeremusHarrier1" "RTS_World") (`SceneComponent.GetSocketTransform` (`self.Pixel2D`) "HeremusHarrier2" "RTS_World")))

(fn `UserConstructionScript`
  (`parent.UserConstructionScript`))