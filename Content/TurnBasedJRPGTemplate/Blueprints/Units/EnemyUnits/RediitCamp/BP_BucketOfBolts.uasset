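; Bucket of Bolts enemy battle unit from the Rediit Camp set in the turn-based JRPG template.
; It derives its combat stats from level through GetUnitStats and supplies two projectile spawn transforms from HeremusHarrier sockets on its Pixel2D component.
; Turn start just calls the parent; a parry tutorial popup that would clear the battle controller's tutorial flag on dismissal is left unconnected.
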(event `self.StartTurn`
  (`parent.StartTurn`))

(event `removed`
  (set `/Game/TurnBasedJRPGTemplate/Blueprints/Battle/BP_BattleController.BattleTutorial_1` false (`self.battleController`)))

(event `self.ReceiveBeginPlay`
  (`parent.ReceiveBeginPlay`))

(event `self.SetUnitStats`
  (bind _stats (`/Game/TurnBasedJRPGTemplate/Blueprints/Controllers/BP_JRPGFunctionLibrary.GetUnitStats` (`self.level`) (`self.maxLevel`) (`self.initialStats`) (`self.firstLevelStats`) (`self.lastLevelStats`)))
  (bind (_maxhp _maxmp _attack _defense _speed _hit _magicalattack _magicdefense _actiontime _criticalhit _maxoverdrivepoints) (break `/Game/TurnBasedJRPGTemplate/Blueprints/Structs/S_UnitStats` _stats))
  (set `self.maxHP` _maxhp)
  (set `self.maxMP` _maxmp)
  (set `self.maxAttack` _attack)
  (set `self.defense` _defense)
  (set `self.speed` _speed)
  (set `self.hit` _hit)
  (set `self.maxMagicalAttack` _magicalattack)
  (set `self.magicalDefense` _magicdefense)
  (set `self.Critical` _criticalhit)
  (set `self.MaxOverdrivePoints` _maxoverdrivepoints))

(fn `GetProjectileSpawnTransform`
  (returns (projectileSpawnTransform :type "Transform Structure") (projectileSpawnTransform2 :type "Transform Structure"))
  (return (`SceneComponent.GetSocketTransform` (`self.Pixel2D`) "HeremusHarrier1" "RTS_World") (`SceneComponent.GetSocketTransform` (`self.Pixel2D`) "HeremusHarrier2" "RTS_World")))

(fn `UserConstructionScript`
  (`parent.UserConstructionScript`))