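; BP_Reaver_2 is a Bandit Cave enemy unit for turn-based JRPG battles, extending a parent unit Blueprint.
; When berserk, it overrides the turn start to pick a target from its status flags, pause briefly, then make a regular attack through the BattleController; otherwise the parent logic runs.
; It also overrides projectile spawning to return the Pixel2D component's world transform for both spawn points.
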(event `self.StartTurn`
  (bind _battlecontroller (`self.battleController`))
  (if (`self.IsBerserk??`)
    (`self.OnTurnStarted`)
    (bind _targetunit (`self.GetTargetUnit` true (`self.Is Confused`) (`self.IsBerserk??`) (`self.IsCharmed??`) false (`self.IsTaunted`)))
    (set `self.currentTarget` _targetunit)
    (`KismetSystemLibrary.Delay` 0.3)
    (`/Game/TurnBasedJRPGTemplate/Blueprints/UI/BP_BattleUI.ShowRegularAttack` (`/Game/TurnBasedJRPGTemplate/Blueprints/Battle/BP_BattleController.battleUI` _battlecontroller))
    (`/Game/TurnBasedJRPGTemplate/Blueprints/Battle/BP_BattleController.Attack` _battlecontroller (`self.currentTarget`))
    (else
      (`parent.StartTurn`))))

(event `self.ReceiveBeginPlay`
  (`parent.ReceiveBeginPlay`))

(fn `GetProjectileSpawnTransform`
  (returns (projectileSpawnTransform :type "Transform Structure") (projectileSpawnTransform2 :type "Transform Structure"))
  (bind _returnvalue (`SceneComponent.GetSocketTransform` (`self.Pixel2D`) "None" "RTS_World"))
  (`parent.GetProjectileSpawnTransform`)
  (return _returnvalue _returnvalue))

(fn `UserConstructionScript`
  (`parent.UserConstructionScript`))