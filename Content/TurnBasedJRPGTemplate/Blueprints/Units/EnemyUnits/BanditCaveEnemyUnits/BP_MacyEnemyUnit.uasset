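; Enemy battle unit for Macy, from the Bandit Cave set, with custom turn logic for self-curing and Overdrive.
; On turn start it checks in priority order: Inoculate on itself under DOT, Refresh on itself when blind, its Overdrive skill if entered, otherwise parent behavior.
; Skills run through the BattleController, with self-casts preselecting the target.
; It destroys its Box component on BeginPlay and spawns projectiles from the Pixel2D component's transform.
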(event `self.StartTurn`
  (bind _battlecontroller (`self.battleController`))
  (if (`self.Is DOT`)
    (set `/Game/TurnBasedJRPGTemplate/Blueprints/Battle/BP_BattleController.currentTargetUnit` self (`self.battleController`))
    (`/Game/TurnBasedJRPGTemplate/Blueprints/Battle/BP_BattleController.EnemyPrepareForSkill` _battlecontroller "/Game/TurnBasedJRPGTemplate/Blueprints/Skills/HealingSkills/BP_Inoculate.BP_Inoculate_C" false true)
    (elif (`self.Is Blind?`)
      (set `/Game/TurnBasedJRPGTemplate/Blueprints/Battle/BP_BattleController.currentTargetUnit` self (`self.battleController`))
      (`/Game/TurnBasedJRPGTemplate/Blueprints/Battle/BP_BattleController.EnemyPrepareForSkill` _battlecontroller "/Game/TurnBasedJRPGTemplate/Blueprints/Skills/HealingSkills/BP_Refresh.BP_Refresh_C" false true)
      (elif (`self.OverdriveEntered`)
        (`/Game/TurnBasedJRPGTemplate/Blueprints/Battle/BP_BattleController.EnemyPrepareForSkill` _battlecontroller "/Game/TurnBasedJRPGTemplate/Blueprints/Skills/Overdrives/BP_MacyOverdrive.BP_MacyOverdrive_C" false false)
        (else
          (`parent.StartTurn`))))))

(event `self.ReceiveBeginPlay`
  (`ActorComponent.K2_DestroyComponent` (`self.Box`))
  (`parent.ReceiveBeginPlay`))

(event `self.Is Target Player Unit Defending`)

(event `self.Block/Parry Input`)

(event `self.Box.OnComponentBeginOverlap`
  (params (OverlappedComponent :type "PrimitiveComponent Object Reference") (OtherActor :type "Actor Object Reference") (OtherComp :type "PrimitiveComponent Object Reference") (OtherBodyIndex :type Integer) (bFromSweep :type Boolean) (SweepResult :type "HitResult Structure (by ref)")))

(fn `GetProjectileSpawnTransform`
  (returns (projectileSpawnTransform :type "Transform Structure") (projectileSpawnTransform2 :type "Transform Structure"))
  (bind _returnvalue (`SceneComponent.GetSocketTransform` (`self.Pixel2D`) "None" "RTS_World"))
  (`parent.GetProjectileSpawnTransform`)
  (return _returnvalue _returnvalue))

(fn `UserConstructionScript`
  (`parent.UserConstructionScript`))