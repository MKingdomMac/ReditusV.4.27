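; Cerebus enemy unit for the Bandit Cave battles in the turn-based JRPG template.
; On StartTurn, it uses BP_Lick on the first enemy-side unit when that unit is valid and unprotected, preselecting the target through BattleController and printing its name.
; Otherwise it falls back to the parent turn logic.
; Projectiles spawn from the Pixel2D component's transform, and an older player-targeting attack chain is left unconnected.
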(event `self.StartTurn`
  (bind _battlecontroller (`self.battleController`))
  (bind _output (`|GetArrayItem` (`/Game/TurnBasedJRPGTemplate/Blueprints/Battle/BP_BattleBase.enemyUnits` (`/Game/TurnBasedJRPGTemplate/Blueprints/Battle/BP_BattleController.currentBattle` (`self.battleController`)))))
  (`/Engine/EditorBlueprintResources/StandardMacros.IsValid` _output
    (:`Is Valid`
      (if (`/Game/TurnBasedJRPGTemplate/Blueprints/Units/BP_UnitBase.IsProtected` _output)
        (`parent.StartTurn` :!label _label)
        (else
          (bind _output_get (set `/Game/TurnBasedJRPGTemplate/Blueprints/Battle/BP_BattleController.currentTargetUnit` _output _battlecontroller))
          (`KismetSystemLibrary.PrintString` (`KismetSystemLibrary.GetDisplayName` _output_get) true true (struct :`R` 1.0 :`G` 0.071004 :`B` 0.041157 :`A` 1.0) 10.0)
          (`/Game/TurnBasedJRPGTemplate/Blueprints/Battle/BP_BattleController.EnemyPrepareForSkill` _battlecontroller "/Game/TurnBasedJRPGTemplate/Blueprints/Skills/EnemySkills/BanditCave/BP_Lick.BP_Lick_C" false true))))
    (:`Is Not Valid`
      (goto _label))))

(event `self.ReceiveBeginPlay`
  (`parent.ReceiveBeginPlay`))

(fn `GetProjectileSpawnTransform`
  (returns (projectileSpawnTransform :type "Transform Structure") (projectileSpawnTransform2 :type "Transform Structure"))
  (bind _returnvalue (`SceneComponent.GetSocketTransform` (`self.Pixel2D`) "None" "RTS_World"))
  (`parent.GetProjectileSpawnTransform`)
  (return _returnvalue _returnvalue))

(fn `UserConstructionScript`
  (`parent.UserConstructionScript`))