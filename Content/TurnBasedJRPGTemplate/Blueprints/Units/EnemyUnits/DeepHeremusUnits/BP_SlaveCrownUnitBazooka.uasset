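; Bazooka variant of the Slave Crown enemy unit for turn-based JRPG battles.
; When berserk, it overrides its turn to pick a target from its status effects, focus on it, adjust the camera and attack through the battle controller after a short delay.
; Otherwise it runs the parent turn logic.
; Both projectile spawn transforms come from the Rocket socket on its Pixel2D component.
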(event `self.StartTurn`
  (if (`self.IsBerserk??`)
    (`self.OnTurnStarted`)
    (bind _targetunit (`self.GetTargetUnit` true (`self.Is Confused`) (`self.IsBerserk??`) (`self.IsCharmed??`) false (`self.IsTaunted`)))
    (set `self.currentTarget` _targetunit)
    (`self.FocusOnTarget` (struct))
    (`self.AdjustAttackerStandLocation` (`self.currentTarget`) self)
    (`/Game/TurnBasedJRPGTemplate/Blueprints/Battle/BP_BattleController.AdjustCamera` (`self.battleController`) (cast `/Game/TurnBasedJRPGTemplate/Blueprints/Units/PlayerUnits/BP_PlayerUnitBase` (`self.currentTarget`) :!pure true) self false)
    (`KismetSystemLibrary.Delay` 0.5)
    (`/Game/TurnBasedJRPGTemplate/Blueprints/Battle/BP_BattleController.Attack` (`self.battleController`) (`self.currentTarget`))
    (else
      (`parent.StartTurn`))))

(event `self.ReceiveBeginPlay`
  (`parent.ReceiveBeginPlay`))

(fn `GetProjectileSpawnTransform`
  (returns (projectileSpawnTransform :type "Transform Structure") (projectileSpawnTransform2 :type "Transform Structure"))
  (bind _returnvalue (`SceneComponent.GetSocketTransform` (`self.Pixel2D`) "Rocket" "RTS_World"))
  (`parent.GetProjectileSpawnTransform`)
  (return _returnvalue _returnvalue))

(fn `UserConstructionScript`
  (`parent.UserConstructionScript`))