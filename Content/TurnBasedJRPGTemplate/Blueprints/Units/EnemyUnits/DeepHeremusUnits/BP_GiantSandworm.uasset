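; Giant Sandworm enemy unit for the turn-based battle system, overriding turn logic and projectile origin.
; While protected, it picks a random skill but swaps Stir Up, or no skill, for a basic attack on a status-aware target, framing the camera first.
; Other skills go to the BattleController, and unprotected turns use the parent logic.
; Both projectile spawn transforms come from the Pixel2D "Rocket" socket.
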(event `self.StartTurn`
  (bind _is_confused (`self.Is Confused`))
  (if (`self.IsProtected`)
    (`self.OnTurnStarted`)
    (bind _skill (`self.GetRandomSkill`))
    (if (!= _skill null)
      (if (== _skill "/Game/TurnBasedJRPGTemplate/Blueprints/Skills/EnemySkills/DeepHeremus/BP_StirUp.BP_StirUp_C")
        (bind _targetunit (`self.GetTargetUnit` true _is_confused (`self.IsBerserk??`) (`self.IsCharmed??`) false (`self.IsTaunted`) :!label _label))
        (set `self.currentTarget` _targetunit)
        (`self.FocusOnTarget` (struct))
        (`self.AdjustAttackerStandLocation` (`self.currentTarget`) self)
        (`/Game/TurnBasedJRPGTemplate/Blueprints/Battle/BP_BattleController.AdjustCamera` (`self.battleController`) (cast `/Game/TurnBasedJRPGTemplate/Blueprints/Units/PlayerUnits/BP_PlayerUnitBase` (`self.currentTarget`) :!pure true) self false)
        (`KismetSystemLibrary.Delay` 0.5)
        (`/Game/TurnBasedJRPGTemplate/Blueprints/Battle/BP_BattleController.Attack` (`self.battleController`) (`self.currentTarget`))
        (else
          (`/Game/TurnBasedJRPGTemplate/Blueprints/Battle/BP_BattleController.EnemyPrepareForSkill` (`self.battleController`) _skill _is_confused false)))
      (else
        (goto _label)))
    (else
      (`parent.StartTurn`))))

(event `self.ReceiveBeginPlay`
  (`parent.ReceiveBeginPlay`))

(fn `GetProjectileSpawnTransform`
  (returns (projectileSpawnTransform :type "Transform Structure") (projectileSpawnTransform2 :type "Transform Structure"))
  (bind _returnvalue (`SceneComponent.GetSocketTransform` (`self.Pixel2D`) "Rocket" "RTS_World"))
  (`parent.GetProjectileSpawnTransform`)
  (return _returnvalue _returnvalue))

(fn `UserConstructionScript`
  (`parent.UserConstructionScript`))