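; Odin's player unit Blueprint for turn-based battles, which adds tutorial gating to the inherited turn logic.
; On turn start, battle controller flags select an amp or stamina-stagger tutorial widget, holding back the parent turn start until its dialogue is removed.
; The removal callback clears that tutorial's flag and resumes the turn.
; Projectiles spawn from the Shotgun socket on the Pixel2D component.
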(event `self.InitUnit`
  (params (battleController :type "/Game/TurnBasedJRPGTemplate/Blueprints/Battle/BP_BattleController Object Reference"))
  (`parent.InitUnit` battleController))

(event `self.StartTurn`
  (bind _battlecontroller (`self.battleController`))
  (bind _jrpgplayercontroller (`/Game/TurnBasedJRPGTemplate/Blueprints/Battle/BP_BattleController.jRPGPlayerController` _battlecontroller))
  (if (`/Game/TurnBasedJRPGTemplate/Blueprints/Battle/BP_BattleController.BattleTutorial_2` _battlecontroller)
    (bind _returnvalue (`|CreateWidget` "/Game/TurnBasedJRPGTemplate/Blueprints/UI/BP_AmpTut.BP_AmpTut_C" null _jrpgplayercontroller null))
    (`UserWidget.AddToViewport` _returnvalue 0)
    (add `/Game/TurnBasedJRPGTemplate/Blueprints/UI/BP_AmpTut.DialogueRemoved` _returnvalue (delegate `Removed2`))
    (elif (`/Game/TurnBasedJRPGTemplate/Blueprints/Battle/BP_BattleController.BattleTutorial 3` _battlecontroller)
      (bind _returnvalue_2 (`|CreateWidget` "/Game/TurnBasedJRPGTemplate/Blueprints/UI/BP_StaminaStaggerTut.BP_StaminaStaggerTut_C" null _jrpgplayercontroller self))
      (`UserWidget.AddToViewport` _returnvalue_2 0)
      (add `/Game/TurnBasedJRPGTemplate/Blueprints/UI/BP_StaminaStaggerTut.DialogueRemoved` _returnvalue_2 (delegate `finito`))
      (else
        (`parent.StartTurn`)))))

(event `Removed2`
  (set `/Game/TurnBasedJRPGTemplate/Blueprints/Battle/BP_BattleController.BattleTutorial_2` false (`self.battleController`))
  (`parent.StartTurn`))

(event `finito`
  (set `/Game/TurnBasedJRPGTemplate/Blueprints/Battle/BP_BattleController.BattleTutorial 3` false (`self.battleController`))
  (`parent.StartTurn`))

(fn `GetProjectileSpawnTransform`
  (returns (projectileSpawnTransform :type "Transform Structure") (projectileSpawnTransform2 :type "Transform Structure"))
  (`parent.GetProjectileSpawnTransform`)
  (return (`SceneComponent.GetSocketTransform` (`self.Pixel2D`) "Shotgun" "RTS_World")))

(fn `UserConstructionScript`
  (`parent.UserConstructionScript`))