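; Player unit Blueprint for Caeser in the turn-based JRPG battle system, adding a timed bonus attack to the parent unit's behaviour.
; During the battle tutorial, turn start waits until a double-attack dialogue widget is removed.
; A brief exclamation-marked window lets TimedAttack input add a reduced-damage hit to regular attacks, with a DoN limiting presses until window or turn end.
; Projectiles spawn from the sprite's Shotgun socket.
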(event `self.InitUnit`
  (params (battleController :type "/Game/TurnBasedJRPGTemplate/Blueprints/Battle/BP_BattleController Object Reference"))
  (`parent.InitUnit` battleController))

(event `self.StartTurn`
  (bind _battlecontroller (`self.battleController`))
  (set `self.CanBlock/Parry?` false)
  (if (`/Game/TurnBasedJRPGTemplate/Blueprints/Battle/BP_BattleController.BattleTutorial_1` _battlecontroller)
    (bind _returnvalue (`|CreateWidget` "/Game/TurnBasedJRPGTemplate/Blueprints/UI/BP_CaeserTutDoubleAttack.BP_CaeserTutDoubleAttack_C" null (`/Game/TurnBasedJRPGTemplate/Blueprints/Battle/BP_BattleController.jRPGPlayerController` _battlecontroller)))
    (`UserWidget.AddToViewport` _returnvalue 0)
    (add `/Game/TurnBasedJRPGTemplate/Blueprints/UI/BP_CaeserTutDoubleAttack.DialogueRemoved` _returnvalue (delegate `Remove`))
    (else
      (`parent.StartTurn`))))

(event `Remove`
  (set `/Game/TurnBasedJRPGTemplate/Blueprints/Battle/BP_BattleController.BattleTutorial_1` false (`self.battleController`))
  (`parent.StartTurn`))

(event `self.EndTurn`
  (`self.DoAgain`)
  (`parent.EndTurn`))

(event `InputAction|TimedAttack`
  (params (Key :type "Key Structure"))
  (:`Pressed`
    (switch `/Game/TurnBasedJRPGTemplate/Blueprints/Enums/E_SelectType` (`self.SelectType`)
      (:`NewEnumerator5`
        (`/Engine/EditorBlueprintResources/StandardMacros.Do N` 2 :!label _label
          (:`Exit`
            (`KismetSystemLibrary.PrintString` "you can do")
            (if (`self.TimedAttackOpportunity`)
              (`KismetSystemLibrary.PrintString` "Hello")
              (set `self.BonusAttack` true)
              (`KismetSystemLibrary.Delay` 0.8)
              (`GameplayStatics.SpawnSound2D` "/Game/Sounds/JrpgBlueprintSounds/WAV_Sword2.WAV_Sword2" 1.0 1.0 0.0 null)
              (`/Game/TurnBasedJRPGTemplate/Blueprints/Battle/BP_BattleController.DealDamage` (`self.battleController`) 0 0.6 (`self.Critical`))
              (`NiagaraFunctionLibrary.SpawnSystemAttached` "/Game/Particles/sA_Megapack_v1/sA_StylizedAttacksPack/FX/NiagaraSystems/NS_BasicHit.NS_BasicHit" (`/Game/TurnBasedJRPGTemplate/Blueprints/Units/BP_UnitBase.Pixel2D` (`/Game/TurnBasedJRPGTemplate/Blueprints/Battle/BP_BattleController.currentTargetUnit` (`self.battleController`))) "None" (0.0 0.0 0.0) (struct) "KeepRelativeOffset")
              (set `self.BonusAttack` false))))))))

(event `DoAgain`
  (goto _label :!via `Reset`))

(event `TimedAttackWindowIndicator`
  (set `self.TimedAttackOpportunity` true)
  (`GameplayStatics.SpawnEmitterAttached` "/Game/Particles/GoodParticleStatus/Particles/Head_Status/PS_GPS_ExclamationMark.PS_GPS_ExclamationMark" (`self.TargetIconWidget`) "StatusSocket" (0.0 0.0 0.0) (struct) (2.0 2.0 2.0))
  (`KismetSystemLibrary.Delay` 0.3)
  (set `self.TimedAttackOpportunity` false)
  (`self.DoAgain`)
  (if (`/Game/TurnBasedJRPGTemplate/Blueprints/Controllers/BP_JRPGPlayerController.IsFastSpeed` (`self.As BP JRPGPlayer Controller`))
    (set `self.CustomTimeDilation` 1.5)
    (else
      (set `self.CustomTimeDilation` 1.0))))

(fn `GetProjectileSpawnTransform`
  (returns (projectileSpawnTransform :type "Transform Structure") (projectileSpawnTransform2 :type "Transform Structure"))
  (`parent.GetProjectileSpawnTransform`)
  (return (`SceneComponent.GetSocketTransform` (`self.Pixel2D`) "Shotgun" "RTS_World")))

(fn `UserConstructionScript`
  (`parent.UserConstructionScript`))