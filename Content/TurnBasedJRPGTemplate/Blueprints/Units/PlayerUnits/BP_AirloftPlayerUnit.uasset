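; Player unit Blueprint for Airloft in the turn-based JRPG battle system, extending the parent unit's damage, turn and projectile socket logic.
; While the hit counter is active, damage taken builds charges up to a cap.
; At full charge, turn start applies a defense buff, fires an AoE fire overdrive using delayed amp points, then clears the counter.
; Turns also toggle the Hack action, and tutorial battles defer turn start until dialogue closes.
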(event `self.TakeDamage`
  (params (damage :type Integer))
  (if (and (`self.SkillHitCounterActivated`) (> damage 0))
    (set `self.SkillHitCounter` (`KismetMathLibrary.Clamp` (+ (`self.SkillHitCounter`) 1) 0 5))
    (`parent.TakeDamage` damage)
    (else
      (`parent.TakeDamage` damage))))

(event `self.StartTurn`
  (bind _battlecontroller (`self.battleController`))
  (bind _currentattackingunit (`/Game/TurnBasedJRPGTemplate/Blueprints/Battle/BP_BattleController.currentAttackingUnit` _battlecontroller))
  (`/Game/TurnBasedJRPGTemplate/Blueprints/UI/BP_ActionsUI.Add Hack` (`self.actionsUI`))
  (if (== (`self.SkillHitCounter`) 5)
    (`/Game/TurnBasedJRPGTemplate/Blueprints/Battle/BP_BattleController.ApplyBuff` _battlecontroller (`|MakeArray` _currentattackingunit) "/Game/TurnBasedJRPGTemplate/Blueprints/Skills/Buffs/BP_DefenseIncrease.BP_DefenseIncrease_C")
    (`KismetSystemLibrary.Delay` 1.0)
    (bind _returnvalue (`|SpawnActorFromClass` "/Game/TurnBasedJRPGTemplate/Blueprints/Skills/Overdrives/BP_AirloftAoeFireOverdrive.BP_AirloftAoeFireOverdrive_C" (`KismetMathLibrary.MakeTransform` (999999.0 999999.0 999999.0)) "Undefined" "OverrideRootScale" null (`/Game/TurnBasedJRPGTemplate/Blueprints/Units/BP_UnitBase.DelayedSkillAmpCounter` _currentattackingunit) "NewEnumerator2" "NewEnumerator0" true _battlecontroller false "Phys" false "None" 1.0 (`self.As BP JRPGPlayer Controller`) null))
    (bind _output_get (set `/Game/TurnBasedJRPGTemplate/Blueprints/Battle/BP_BattleController.currentSkill` _returnvalue _battlecontroller))
    (set `/Game/TurnBasedJRPGTemplate/Blueprints/Skills/Overdrives/BP_AirloftAoeFireOverdrive.Damage Multiplier_0` 1.0 _returnvalue)
    (`/Game/TurnBasedJRPGTemplate/Blueprints/Skills/BP_SkillBase.UseOverdrive` _output_get)
    (set `self.SkillHitCounter` 0)
    (`self.K2_DestroyActor` (`BlueprintMapLibrary.Map_Find` (`self.activeBuffs`) "/Game/TurnBasedJRPGTemplate/Blueprints/Skills/Buffs/BP_HitCounterActivate.BP_HitCounterActivate_C"))
    (set `self.SkillHitCounterActivated` false)
    (set `/Game/TurnBasedJRPGTemplate/Blueprints/Units/BP_UnitBase.DelayedSkillAmpCounter` 0 _currentattackingunit))
  (if (`/Game/TurnBasedJRPGTemplate/Blueprints/Battle/BP_BattleController.BattleTutorial` _battlecontroller)
    (bind _returnvalue_2 (`|CreateWidget` "/Game/TurnBasedJRPGTemplate/Blueprints/UI/BP_StaminaStaggerTut2.BP_StaminaStaggerTut2_C" null (`self.As BP JRPGPlayer Controller`)))
    (`UserWidget.AddToViewport` _returnvalue_2 0)
    (add `/Game/TurnBasedJRPGTemplate/Blueprints/UI/BP_StaminaStaggerTut2.DialogueRemoved` _returnvalue_2 (delegate `Remove`))
    (else
      (`parent.StartTurn`))))

(event `Remove`
  (set `/Game/TurnBasedJRPGTemplate/Blueprints/Battle/BP_BattleController.BattleTutorial` false (`self.battleController`))
  (set `/Game/TurnBasedJRPGTemplate/Blueprints/Controllers/BP_JRPGPlayerController.IsSequence` false (`self.As BP JRPGPlayer Controller`))
  (`parent.StartTurn`))

(event `self.EndTurn`
  (`/Game/TurnBasedJRPGTemplate/Blueprints/UI/BP_ActionsUI.Remove Hack` (`self.actionsUI`))
  (`parent.EndTurn`))

(fn `GetProjectileSpawnTransform`
  (returns (projectileSpawnTransform :type "Transform Structure") (projectileSpawnTransform2 :type "Transform Structure"))
  (bind _returnvalue (`SceneComponent.GetSocketTransform` (`self.Pixel2D`) "ProjectileSocket" "RTS_World"))
  (return _returnvalue _returnvalue))

(fn `UserConstructionScript`
  (`parent.UserConstructionScript`))