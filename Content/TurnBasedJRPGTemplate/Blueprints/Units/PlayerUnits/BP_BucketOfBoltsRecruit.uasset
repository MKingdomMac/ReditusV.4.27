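; Player-unit Blueprint for the Bucket of Bolts Recruit in the turn-based JRPG battle system.
; StartTurn, BeginPlay and construction simply defer to the parent class.
; GetProjectileSpawnTransform returns two world-space transforms from the HeremusHarrier1 and HeremusHarrier2 sockets on the Pixel2D component.
; A disconnected branch would show the Caeser parry tutorial widget when BattleTutorial1 is set; its removed handler clears that flag.
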(event `self.StartTurn`
  (`parent.StartTurn`))

(event `removed`
  (set `/Game/TurnBasedJRPGTemplate/Blueprints/Battle/BP_BattleController.BattleTutorial_1` false (`self.battleController`)))

(event `self.ReceiveBeginPlay`
  (`parent.ReceiveBeginPlay`))

(fn `GetProjectileSpawnTransform`
  (returns (projectileSpawnTransform :type "Transform Structure") (projectileSpawnTransform2 :type "Transform Structure"))
  (return (`SceneComponent.GetSocketTransform` (`self.Pixel2D`) "HeremusHarrier1" "RTS_World") (`SceneComponent.GetSocketTransform` (`self.Pixel2D`) "HeremusHarrier2" "RTS_World")))

(fn `UserConstructionScript`
  (`parent.UserConstructionScript`))