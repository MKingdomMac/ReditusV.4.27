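; BP_DoorSpawnFacingBack is an overworld door trigger that moves the player to another map with a preset spawn facing, back by its name.
; When a BP_JRPGCharacterBase overlaps its Box, it writes its DoorID and a fixed direction enum to the JRPG game instance.
; It then calls the game instance's ChangeMap with WhereTo, so the door and facing data persist across the map change.
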(event `self.Box.OnComponentBeginOverlap`
  (params (OverlappedComponent :type "PrimitiveComponent Object Reference") (OtherActor :type "Actor Object Reference") (OtherComp :type "PrimitiveComponent Object Reference") (OtherBodyIndex :type Integer) (bFromSweep :type Boolean) (SweepResult :type "HitResult Structure (by ref)"))
  (bind _asbp_jrpgcharacter_base (cast `/Game/TurnBasedJRPGTemplate/Blueprints/PlayerPawns/BP_JRPGCharacterBase` OtherActor))
  (set `self.CharacterBase` _asbp_jrpgcharacter_base)
  (bind _asbp_jrpggame_instance (cast `/Game/TurnBasedJRPGTemplate/Blueprints/Controllers/BP_JRPGGameInstance` (`GameplayStatics.GetGameInstance`)))
  (set `self.OurGameInstance` _asbp_jrpggame_instance)
  (set `/Game/TurnBasedJRPGTemplate/Blueprints/Controllers/BP_JRPGGameInstance. Door ID` (`self.door ID`) (`self.OurGameInstance`))
  (bind _output_get (set `self.PlayerSpawnDirection` "NewEnumerator0"))
  (set `/Game/TurnBasedJRPGTemplate/Blueprints/Controllers/BP_JRPGGameInstance.E_PlayerDirection` _output_get (`self.OurGameInstance`))
  (`/Game/TurnBasedJRPGTemplate/Blueprints/Controllers/BP_JRPGGameInstance.ChangeMap` _asbp_jrpggame_instance (`self.WhereTo?`)))

(fn `UserConstructionScript`)