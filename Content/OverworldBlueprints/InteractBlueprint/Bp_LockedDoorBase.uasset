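; Base Blueprint for an overworld flipbook door that the player opens once through interaction, with no key check in this graph.
; A child BP_InteractionDetector fires Interacted, which passes through a DoOnce to Open, and has its interaction enabled on its loaded event.
; Open plays a sound, swaps the flipbook, disables box collision and destroys the billboard.
; Until then, player overlap with the sphere toggles the billboard's visibility.
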(event `self.ReceiveBeginPlay`
  (bind _asbp_interaction_detector (cast `/Game/TurnBasedJRPGTemplate/Blueprints/Interactables/BP_InteractionDetector` (`ChildActorComponent.ChildActor` (`self.InteractionActor`))))
  (bind _output_get (set `self.interactionDetector` _asbp_interaction_detector))
  (add `/Game/TurnBasedJRPGTemplate/Blueprints/Interactables/BP_InteractionDetector.OnInteracted` _output_get (delegate `Interacted`))
  (add `/Game/TurnBasedJRPGTemplate/Blueprints/Interactables/BP_InteractionDetector.OnLoaded` (`self.interactionDetector`) (delegate `OnLoadedHandler`)))

(event `Interacted`
  (`/Engine/EditorBlueprintResources/StandardMacros.DoOnce` false
    (:`Completed`
      (`self.Open`))))

(event `OnLoadedHandler`
  (params (shouldLoadEnemyPawns :type Boolean))
  (`/Game/TurnBasedJRPGTemplate/Blueprints/Interactables/BP_InteractionDetector.EnableInteraction` (`self.interactionDetector`)))

(event `self.Sphere.OnComponentBeginOverlap`
  (params (OverlappedComponent :type "PrimitiveComponent Object Reference") (OtherActor :type "Actor Object Reference") (OtherComp :type "PrimitiveComponent Object Reference") (OtherBodyIndex :type Integer) (bFromSweep :type Boolean) (SweepResult :type "HitResult Structure (by ref)"))
  (bind _billboard_0 (`self.Billboard_0`))
  (if (== OtherActor (`GameplayStatics.GetPlayerCharacter` 0))
    (`/Engine/EditorBlueprintResources/StandardMacros.IsValid` _billboard_0
      (:`Is Valid`
        (`SceneComponent.ToggleVisibility` _billboard_0 false)))))

(event `self.Sphere.OnComponentEndOverlap`
  (params (OverlappedComponent :type "PrimitiveComponent Object Reference") (OtherActor :type "Actor Object Reference") (OtherComp :type "PrimitiveComponent Object Reference") (OtherBodyIndex :type Integer))
  (bind _billboard_0 (`self.Billboard_0`))
  (if (== OtherActor (`GameplayStatics.GetPlayerCharacter` 0))
    (`/Engine/EditorBlueprintResources/StandardMacros.IsValid` _billboard_0
      (:`Is Valid`
        (`SceneComponent.ToggleVisibility` _billboard_0 false)))))

(event `Open`
  (`GameplayStatics.PlaySoundAtLocation` (`self.Sound`) (0.0 0.0 0.0) (struct) 1.0 1.0 0.0 null null null)
  (`PaperFlipbookComponent.SetFlipbook` (`self.DoorIdle2`) "/Game/MapSpriteAssets/Doors/DoorIdle.DoorIdle")
  (`PrimitiveComponent.SetCollisionProfileName` (`self.Box`) "NoCollision" true)
  (`ActorComponent.K2_DestroyComponent` (`self.Billboard_0`)))

(fn `UserConstructionScript`)