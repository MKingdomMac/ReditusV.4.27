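; Overworld door trigger that moves a JRPG character within the map or to another map, setting the character to face front on a map change.
; When the character overlaps the Box, the Teleport flag selects between teleporting it to DestLocation with zeroed rotation and changing maps.
; For a map change, it stores DoorID on the game instance, sets PlayerDirection to 0, then calls ChangeMap with WhereTo.
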(event `self.Box.OnComponentBeginOverlap`
  (params (OverlappedComponent :type "PrimitiveComponent Object Reference") (OtherActor :type "Actor Object Reference") (OtherComp :type "PrimitiveComponent Object Reference") (OtherBodyIndex :type Integer) (bFromSweep :type Boolean) (SweepResult :type "HitResult Structure (by ref)"))
  (bind _asbp_jrpgcharacter_base (cast `/Game/TurnBasedJRPGTemplate/Blueprints/PlayerPawns/BP_JRPGCharacterBase` OtherActor))
  (bind _output_get (set `self.CharacterBase` _asbp_jrpgcharacter_base))
  (if (`self.Teleport`)
    (`self.K2_TeleportTo` :`self` (`self.CharacterBase`) :`DestLocation` (`self.Dest Location`))
    (else
      (bind _asbp_jrpggame_instance (cast `/Game/TurnBasedJRPGTemplate/Blueprints/Controllers/BP_JRPGGameInstance` (`GameplayStatics.GetGameInstance`)))
      (set `self.OurGameInstance` _asbp_jrpggame_instance)
      (set `/Game/TurnBasedJRPGTemplate/Blueprints/Controllers/BP_JRPGGameInstance. Door ID` (`self.door ID`) (`self.OurGameInstance`))
      (set `/Game/TurnBasedJRPGTemplate/Blueprints/PlayerPawns/BP_JRPGCharacterBase.PlayerDirection` 0 _output_get)
      (`/Game/TurnBasedJRPGTemplate/Blueprints/Controllers/BP_JRPGGameInstance.ChangeMap` _asbp_jrpggame_instance (`self.WhereTo?`)))))

(fn `UserConstructionScript`)