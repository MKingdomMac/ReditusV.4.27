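; Interactable overworld door that starts the last boss battle, tied to the DealWithBandits quest.
; On interaction, it checks the quest status through the JRPG player controller and, if it matches, calls the boss battle on MyGameState and destroys its map icon.
; BeginPlay removes the icon when the quest is at another specific status, and Refresh removes it unconditionally after calling the parent.
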(event `self.Refresh`
  (params (shouldLoadEnemyPawns :type Boolean))
  (`parent.Refresh` false)
  (`ActorComponent.K2_DestroyComponent` (`self.MapIcon`)))

(event `self.OnInteractedHandler`
  (`parent.OnInteractedHandler`)
  (bind _asbp_jrpgplayer_controller (cast `/Game/TurnBasedJRPGTemplate/Blueprints/Controllers/BP_JRPGPlayerController` (`GameplayStatics.GetPlayerController` 0)))
  (bind _queststatus (`/Game/TurnBasedJRPGTemplate/Blueprints/Controllers/BP_JRPGPlayerController.GetQuestStatus` _asbp_jrpgplayer_controller "/Game/TurnBasedJRPGTemplate/Blueprints/Quests/MainQuests/DealWithBandits.DealWithBandits_C"))
  (if (`|EnumEquality` _queststatus "NewEnumerator1")
    (bind _asmy_game_state (cast `/Game/OverworldBlueprints/SaveAndPersistentData/MyGameState` (`GameplayStatics.GetGameState`)))
    (`/Game/OverworldBlueprints/SaveAndPersistentData/MyGameState.LastBossBattle` _asmy_game_state)
    (`ActorComponent.K2_DestroyComponent` (`self.MapIcon`))))

(event `self.ReceiveBeginPlay`
  (`parent.ReceiveBeginPlay`)
  (bind _asbp_jrpgplayer_controller (cast `/Game/TurnBasedJRPGTemplate/Blueprints/Controllers/BP_JRPGPlayerController` (`GameplayStatics.GetPlayerController` 0)))
  (bind _queststatus (`/Game/TurnBasedJRPGTemplate/Blueprints/Controllers/BP_JRPGPlayerController.GetQuestStatus` _asbp_jrpgplayer_controller "/Game/TurnBasedJRPGTemplate/Blueprints/Quests/MainQuests/DealWithBandits.DealWithBandits_C"))
  (if (`|EnumEquality` _queststatus "NewEnumerator3")
    (`ActorComponent.K2_DestroyComponent` (`self.MapIcon`))))

(fn `UserConstructionScript`
  (`parent.UserConstructionScript`))