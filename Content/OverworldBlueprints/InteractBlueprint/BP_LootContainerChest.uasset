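; BP_LootContainerChest is an overworld loot chest with a Paper2D flipbook, opened through the Interact event.
; The first interaction plays the use sound at the chest's location, switches to the open flipbook and sets the Open flag.
; Later interactions only reapply the open flipbook.
; A comment says it spawns stored items, but the graph ends at a MyGameState cast with no spawning logic.
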(event `/Game/OverworldBlueprints/Interfaces/BP_ItemInteraction.Interact`
  (params (Interactor :type "Actor Object Reference"))
  (bind _paperflipbook (`self.PaperFlipbook`))
  ;[1 1 1] Spawns all stored items
  (if (`self.Open?`)
    (`PaperFlipbookComponent.SetFlipbook` _paperflipbook "/Game/Flipbooks/MiscAssets/treasures/open.open")
    (else
      (`GameplayStatics.PlaySoundAtLocation` (`self.OnUseSound`) (`self.K2_GetActorLocation`) (struct) 1.0 1.0 0.0 null null null)
      (`PaperFlipbookComponent.SetFlipbook` _paperflipbook "/Game/Flipbooks/MiscAssets/treasures/open.open")
      (set `self.Open?` true)
      (cast `/Game/OverworldBlueprints/SaveAndPersistentData/MyGameState` (`GameplayStatics.GetGameState`)))))

(fn `UserConstructionScript`)