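; Base overworld door Blueprint that moves the player's explore character into and out of what appears to be a home interior.
; Interaction, gated by DisableInput and IsInteracted, plays a sound, sets the door flipbook and uses a FlipFlop to alternate between two locations.
; Each side adjusts camera arm length and tilt and calls home hide or show.
; The interaction sphere toggles a prompt billboard and disables jumping while overlapped.
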(event `self.ReceiveBeginPlay`
  (set `self.As BP JRPGPlayer Controller` (cast `/Game/TurnBasedJRPGTemplate/Blueprints/Controllers/BP_JRPGPlayerController` (`GameplayStatics.GetPlayerController` 0) :!pure true)))

(event `self.OnInteractedHandler`
  (bind _explorecharacter (`/Game/TurnBasedJRPGTemplate/Blueprints/Controllers/BP_JRPGPlayerController.exploreCharacter` (cast `/Game/TurnBasedJRPGTemplate/Blueprints/Controllers/BP_JRPGPlayerController` (`GameplayStatics.GetPlayerController` 0) :!pure true)))
  (if (`self.Disable input`)
    _
    (elif (not (`self.IsInteracted`))
      (`GameplayStatics.PlaySoundAtLocation` (`self.Sound`) (0.0 0.0 0.0) (struct) 1.0 1.0 0.0 null null null)
      (`PaperFlipbookComponent.SetFlipbook` (`self.DoorIdle2`) "/Game/MapSpriteAssets/Doors/DoorIdle.DoorIdle")
      (`/Engine/EditorBlueprintResources/StandardMacros.FlipFlop`
        (:`A`
          (`self.K2_SetActorLocation` _explorecharacter (`self.New Location`) false false)
          (set `SpringArmComponent.TargetArmLength` 500.0 (`/Game/TurnBasedJRPGTemplate/Blueprints/PlayerPawns/BP_JRPGCharacterBase.SpringArm` _explorecharacter))
          (`/Game/TurnBasedJRPGTemplate/Blueprints/PlayerPawns/BP_JRPGCharacterBase.RemoveTilt` _explorecharacter)
          (`self.HomeHidden`))
        (:`B`
          (`self.K2_SetActorLocation` (`/Game/TurnBasedJRPGTemplate/Blueprints/Controllers/BP_JRPGPlayerController.exploreCharacter` (cast `/Game/TurnBasedJRPGTemplate/Blueprints/Controllers/BP_JRPGPlayerController` (`GameplayStatics.GetPlayerController` 0) :!pure true)) (`self.OldLocation`) false false)
          (set `SpringArmComponent.TargetArmLength` 800.0 (`/Game/TurnBasedJRPGTemplate/Blueprints/PlayerPawns/BP_JRPGCharacterBase.SpringArm` _explorecharacter))
          (`/Game/TurnBasedJRPGTemplate/Blueprints/PlayerPawns/BP_JRPGCharacterBase.AddTilt` _explorecharacter)
          (`self.HomeVisible`))))))

(event `self.InteractionSphere.OnComponentBeginOverlap`
  (params (OverlappedComponent :type "PrimitiveComponent Object Reference") (OtherActor :type "Actor Object Reference") (OtherComp :type "PrimitiveComponent Object Reference") (OtherBodyIndex :type Integer) (bFromSweep :type Boolean) (SweepResult :type "HitResult Structure (by ref)"))
  (bind _billboard_0 (`self.Billboard_0`))
  (cast `/Game/TurnBasedJRPGTemplate/Blueprints/PlayerPawns/BP_JRPGCharacterBase` OtherActor)
  (set `/Game/TurnBasedJRPGTemplate/Blueprints/Controllers/BP_JRPGPlayerController.CanJump` false (`self.As BP JRPGPlayer Controller`))
  (`/Engine/EditorBlueprintResources/StandardMacros.IsValid` _billboard_0
    (:`Is Valid`
      (`SceneComponent.SetVisibility` _billboard_0 true false))))

(event `self.InteractionSphere.OnComponentEndOverlap`
  (params (OverlappedComponent :type "PrimitiveComponent Object Reference") (OtherActor :type "Actor Object Reference") (OtherComp :type "PrimitiveComponent Object Reference") (OtherBodyIndex :type Integer))
  (bind _billboard_0 (`self.Billboard_0`))
  (cast `/Game/TurnBasedJRPGTemplate/Blueprints/PlayerPawns/BP_JRPGCharacterBase` OtherActor)
  (set `/Game/TurnBasedJRPGTemplate/Blueprints/Controllers/BP_JRPGPlayerController.CanJump` true (`self.As BP JRPGPlayer Controller`))
  (`/Engine/EditorBlueprintResources/StandardMacros.IsValid` _billboard_0
    (:`Is Valid`
      (`SceneComponent.SetVisibility` _billboard_0 false false))))

(fn `UserConstructionScript`)