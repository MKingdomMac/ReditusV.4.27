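; Training dummy overworld NPC that opens a dialogue when interacted with and shows its state through a Paper2D flipbook.
; The interaction handler creates a DemoDialogueWidget from its Dialogue, then compares player and NPC positions for facing, though all four directions set the same idle flipbook.
; Box overlap begin and end events toggle a Billboard's visibility for the player, likely as an interaction prompt.
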(event `self.OnInteractedHandler`
  (bind (_returnvalue_x _returnvalue_y) (`KismetMathLibrary.BreakVector` (`self.K2_GetActorLocation`)))
  (bind _returnvalue_x_2 (`KismetMathLibrary.BreakVector` (`self.K2_GetActorLocation`)))
  (bind _returnvalue_x_3 (`KismetMathLibrary.BreakVector` (`self.K2_GetActorLocation`)))
  (bind (_returnvalue_x_4 _returnvalue_y_2) (`KismetMathLibrary.BreakVector` (`self.K2_GetActorLocation`)))
  (bind _paperflipbook (`self.PaperFlipbook`))
  (bind _paperflipbook_2 (`self.PaperFlipbook`))
  (bind (_returnvalue_x_5 _returnvalue_y_3) (`KismetMathLibrary.BreakVector` (`self.K2_GetActorLocation` (`GameplayStatics.GetPlayerCharacter` 0))))
  (bind _returnvalue_x_6 (`KismetMathLibrary.BreakVector` (`self.K2_GetActorLocation` (`GameplayStatics.GetPlayerCharacter` 0))))
  (bind _returnvalue_x_7 (`KismetMathLibrary.BreakVector` (`self.K2_GetActorLocation` (`GameplayStatics.GetPlayerCharacter` 0))))
  (bind (_returnvalue_x_8 _returnvalue_y_4) (`KismetMathLibrary.BreakVector` (`self.K2_GetActorLocation` (`GameplayStatics.GetPlayerCharacter` 0))))
  (bind _returnvalue (`|CreateWidget` "/DialoguePlugin/UI/DemoDialogueWidget.DemoDialogueWidget_C" null (`self.Dialogue`) false false null null))
  (`UserWidget.AddToViewport` _returnvalue 0)
  ;[1 1 1] Npc Turns Toward Character
  ;;[1 1 1] True = x direction player is closer to npc
  (if (>= (`KismetMathLibrary.Abs` (- _returnvalue_y_3 _returnvalue_y)) (`KismetMathLibrary.Abs` (- _returnvalue_x_6 _returnvalue_x_2)))
    (if (>= _returnvalue_y_4 _returnvalue_y_2)
      (`PaperFlipbookComponent.SetFlipbook` _paperflipbook "/Game/Flipbooks/EnemyNpcFlipbooks/SideViewBattler/RediitCamp/DummyBattler/F_Overworld_Training_Dummy_Idlet_Flipbook.F_Overworld_Training_Dummy_Idlet_Flipbook")
      (else
        (`PaperFlipbookComponent.SetFlipbook` _paperflipbook "/Game/Flipbooks/EnemyNpcFlipbooks/SideViewBattler/RediitCamp/DummyBattler/F_Overworld_Training_Dummy_Idlet_Flipbook.F_Overworld_Training_Dummy_Idlet_Flipbook")))
    (elif (>= _returnvalue_x_7 _returnvalue_x_3)
      (`PaperFlipbookComponent.SetFlipbook` _paperflipbook_2 "/Game/Flipbooks/EnemyNpcFlipbooks/SideViewBattler/RediitCamp/DummyBattler/F_Overworld_Training_Dummy_Idlet_Flipbook.F_Overworld_Training_Dummy_Idlet_Flipbook")
      (else
        (`PaperFlipbookComponent.SetFlipbook` _paperflipbook_2 "/Game/Flipbooks/EnemyNpcFlipbooks/SideViewBattler/RediitCamp/DummyBattler/F_Overworld_Training_Dummy_Idlet_Flipbook.F_Overworld_Training_Dummy_Idlet_Flipbook")))))

(event `self.Box.OnComponentBeginOverlap`
  (params (OverlappedComponent :type "PrimitiveComponent Object Reference") (OtherActor :type "Actor Object Reference") (OtherComp :type "PrimitiveComponent Object Reference") (OtherBodyIndex :type Integer) (bFromSweep :type Boolean) (SweepResult :type "HitResult Structure (by ref)"))
  (bind _billboard (`self.Billboard`))
  (if (and (== OtherActor (`GameplayStatics.GetPlayerCharacter` 0)) (`KismetSystemLibrary.IsValid` _billboard))
    (`SceneComponent.ToggleVisibility` _billboard false)))

(event `self.Box.OnComponentEndOverlap`
  (params (OverlappedComponent :type "PrimitiveComponent Object Reference") (OtherActor :type "Actor Object Reference") (OtherComp :type "PrimitiveComponent Object Reference") (OtherBodyIndex :type Integer))
  (bind _billboard (`self.Billboard`))
  (if (and (`KismetSystemLibrary.IsValid` _billboard) (== OtherActor (`GameplayStatics.GetPlayerCharacter` 0)))
    (`SceneComponent.ToggleVisibility` _billboard false)))

(fn `UserConstructionScript`)