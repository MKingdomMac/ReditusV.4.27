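; Camp quest NPC, a flipbook child character, that completes the IveBeenSavingQuest step when the player talks to it.
; On interaction, a quest status check picks the dialogue; at the matching status it also delivers that quest, hides its map icon and progresses BP_QuestMountUp.
; The NPC then swaps idle flipbooks to face the player along the dominant X/Y axis.
; Box overlaps toggle a billboard, and delayed BeginPlay sets icon visibility from quest status.
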(event `self.ReceiveBeginPlay`
  (bind _asbp_jrpgplayer_controller (cast `/Game/TurnBasedJRPGTemplate/Blueprints/Controllers/BP_JRPGPlayerController` (`GameplayStatics.GetPlayerController` 0)))
  (bind _output_get (set `self.JrpgController` _asbp_jrpgplayer_controller))
  (`KismetSystemLibrary.Delay` 0.6)
  (`/Game/TurnBasedJRPGTemplate/Blueprints/Controllers/BP_JRPGPlayerController.GetQuestStatus` (`self.JrpgController`) "/Game/TurnBasedJRPGTemplate/Blueprints/Quests/CampSideQuests/IveBeenSavingQuest.IveBeenSavingQuest_C")
  (bind _queststatus (`/Game/TurnBasedJRPGTemplate/Blueprints/Controllers/BP_JRPGPlayerController.GetQuestStatus` _output_get "/Game/TurnBasedJRPGTemplate/Blueprints/Quests/CampSideQuests/IveBeenSavingQuest.IveBeenSavingQuest_C"))
  (if (`|EnumEquality` _queststatus "NewEnumerator1")
    (`MapIconComponent.SetIconVisible` (`self.MapIcon`) true)
    (else
      (`MapIconComponent.SetIconVisible` (`self.MapIcon`) false))))

(event `self.OnInteractedHandler`
  (bind (_returnvalue_x _returnvalue_y) (`KismetMathLibrary.BreakVector` (`self.K2_GetActorLocation`)))
  (bind _returnvalue_x_2 (`KismetMathLibrary.BreakVector` (`self.K2_GetActorLocation`)))
  (bind _returnvalue_x_3 (`KismetMathLibrary.BreakVector` (`self.K2_GetActorLocation`)))
  (bind (_returnvalue_x_4 _returnvalue_y_2) (`KismetMathLibrary.BreakVector` (`self.K2_GetActorLocation`)))
  (bind _jrpgcontroller (`self.JrpgController`))
  (bind _paperflipbook (`self.PaperFlipbook`))
  (bind _paperflipbook_2 (`self.PaperFlipbook`))
  (bind (_returnvalue_x_5 _returnvalue_y_3) (`KismetMathLibrary.BreakVector` (`self.K2_GetActorLocation` (`GameplayStatics.GetPlayerCharacter` 0))))
  (bind _returnvalue_x_6 (`KismetMathLibrary.BreakVector` (`self.K2_GetActorLocation` (`GameplayStatics.GetPlayerCharacter` 0))))
  (bind _returnvalue_x_7 (`KismetMathLibrary.BreakVector` (`self.K2_GetActorLocation` (`GameplayStatics.GetPlayerCharacter` 0))))
  (bind (_returnvalue_x_8 _returnvalue_y_4) (`KismetMathLibrary.BreakVector` (`self.K2_GetActorLocation` (`GameplayStatics.GetPlayerCharacter` 0))))
  ;[1 1 1] Spawns all stored items
  (bind _queststatus (`/Game/TurnBasedJRPGTemplate/Blueprints/Controllers/BP_JRPGPlayerController.GetQuestStatus` (`self.JrpgController`) "/Game/TurnBasedJRPGTemplate/Blueprints/Quests/CampSideQuests/IveBeenSavingQuest.IveBeenSavingQuest_C"))
  (if (`|EnumEquality` _queststatus "NewEnumerator1")
    (bind _returnvalue (`|CreateWidget` "/DialoguePlugin/UI/DemoDialogueWidget.DemoDialogueWidget_C" null (`self.Dialogue`) false false null null))
    (`UserWidget.AddToViewport` _returnvalue 0)
    (`/Game/TurnBasedJRPGTemplate/Blueprints/Controllers/BP_JRPGPlayerController.UpdateQuest` _jrpgcontroller "/Game/TurnBasedJRPGTemplate/Blueprints/Quests/CampSideQuests/IveBeenSavingQuest.IveBeenSavingQuest_C" 1 false false false)
    (`/Game/TurnBasedJRPGTemplate/Blueprints/Controllers/BP_JRPGPlayerController.DeliverQuest` _jrpgcontroller "/Game/TurnBasedJRPGTemplate/Blueprints/Quests/CampSideQuests/IveBeenSavingQuest.IveBeenSavingQuest_C" false)
    (`MapIconComponent.SetIconVisible` (`self.MapIcon`) false)
    (`/Game/TurnBasedJRPGTemplate/Blueprints/Controllers/BP_JRPGPlayerController.UpdateQuest` (`self.JrpgController`) "/Game/TurnBasedJRPGTemplate/Blueprints/Quests/SideQuests/RediitCamp/BP_QuestMountUp.BP_QuestMountUp_C" 1 false false true)
    (else
      (bind _returnvalue_2 (`|CreateWidget` "/DialoguePlugin/UI/DemoDialogueWidget.DemoDialogueWidget_C" null (`self.Dialogue_1`) false false null null))
      (`UserWidget.AddToViewport` _returnvalue_2 0)))
  ;[1 1 1] Npc Turns Toward Character
  ;;[1 1 1] True = x direction player is closer to npc
  (if (>= (`KismetMathLibrary.Abs` (- _returnvalue_y_3 _returnvalue_y)) (`KismetMathLibrary.Abs` (- _returnvalue_x_6 _returnvalue_x_2)))
    (if (>= _returnvalue_y_4 _returnvalue_y_2)
      (`PaperFlipbookComponent.SetFlipbook` _paperflipbook "/Game/Flipbooks/OverWorldNpcs/Children/BoyChild1/Front/BoyChildFrontIdle1.BoyChildFrontIdle1")
      (else
        (`PaperFlipbookComponent.SetFlipbook` _paperflipbook "/Game/Flipbooks/OverWorldNpcs/Children/BoyChild1/Back/BoyChildBackIdle1.BoyChildBackIdle1")))
    (elif (>= _returnvalue_x_7 _returnvalue_x_3)
      (`PaperFlipbookComponent.SetFlipbook` _paperflipbook_2 "/Game/Flipbooks/OverWorldNpcs/Children/BoyChild1/Right/BoyChildRightIdle1.BoyChildRightIdle1")
      (else
        (`PaperFlipbookComponent.SetFlipbook` _paperflipbook_2 "/Game/Flipbooks/OverWorldNpcs/Children/BoyChild1/Left/BoyChildLeftIdle1.BoyChildLeftIdle1")))))

(event `CustomEvent_1`
  (params (OverlappedComponent :type "PrimitiveComponent Object Reference") (OtherActor :type "Actor Object Reference") (OtherComp :type "PrimitiveComponent Object Reference") (OtherBodyIndex :type Integer) (bFromSweep :type Boolean) (SweepResult :type "HitResult Structure (by ref)"))
  (if (== OtherActor (`GameplayStatics.GetPlayerCharacter` 0))
    (`SceneComponent.ToggleVisibility` (`self.Billboard_0`) false)))

(event `CustomEvent_2`
  (params (OverlappedComponent :type "PrimitiveComponent Object Reference") (OtherActor :type "Actor Object Reference") (OtherComp :type "PrimitiveComponent Object Reference") (OtherBodyIndex :type Integer))
  (if (== OtherActor (`GameplayStatics.GetPlayerCharacter` 0))
    (`SceneComponent.ToggleVisibility` (`self.Billboard_0`) false)))

(event `self.Box.OnComponentBeginOverlap`
  (params (OverlappedComponent :type "PrimitiveComponent Object Reference") (OtherActor :type "Actor Object Reference") (OtherComp :type "PrimitiveComponent Object Reference") (OtherBodyIndex :type Integer) (bFromSweep :type Boolean) (SweepResult :type "HitResult Structure (by ref)"))
  (if (== OtherActor (`GameplayStatics.GetPlayerCharacter` 0))
    (`SceneComponent.ToggleVisibility` (`self.Billboard_0`) false)))

(event `self.Box.OnComponentEndOverlap`
  (params (OverlappedComponent :type "PrimitiveComponent Object Reference") (OtherActor :type "Actor Object Reference") (OtherComp :type "PrimitiveComponent Object Reference") (OtherBodyIndex :type Integer))
  (if (== OtherActor (`GameplayStatics.GetPlayerCharacter` 0))
    (`SceneComponent.ToggleVisibility` (`self.Billboard_0`) false)))

(fn `UserConstructionScript`)